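; BP_WoodStockPile is a placeable wood stockpile that reflects how full it is through four BP_StockPileStack child actors.
; On each inventory update it calls the parent handler, then passes StockPilePercentage to SetPercentage, which also prints the value.
; SetPercentage maps each quarter of the range to one stack and sends it a rescaled percentage via OnPercentChange.
; Only the stack for the current quarter is updated; the others are left untouched.
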(event EventOnInventoryUpdate
  (|CallParentFunction)
  (CallFunction|SetPercentage (Variables|Default|GetStock%20Pile%20Percentage)))

(fn ConstructionScript
  (|CallParentFunction))

(fn SetPercentage
  (params (Percentage :type Float%20%28single-precision%29))
  (Development|PrintString (Utilities|String|ToString(Float) Percentage))
  (if (<= Percentage 0.25)
    (bind _asbp_stock_pile_stack (Utilities|Casting|CastToBP_StockPileStack (Variables|/Script/Engine.ChildActorComponent|GetChildActor (Variables|Default|GetStack1))))
    (Default|OnPercentChange _asbp_stock_pile_stack (/ Percentage 0.25))
    (elif (<= Percentage 0.5)
      (bind _asbp_stock_pile_stack_2 (Utilities|Casting|CastToBP_StockPileStack (Variables|/Script/Engine.ChildActorComponent|GetChildActor (Variables|Default|GetStack2))))
      (Default|OnPercentChange _asbp_stock_pile_stack_2 (/ (- Percentage 0.25) 0.25))
      (elif (<= Percentage 0.75)
        (bind _asbp_stock_pile_stack_3 (Utilities|Casting|CastToBP_StockPileStack (Variables|/Script/Engine.ChildActorComponent|GetChildActor (Variables|Default|GetStack3))))
        (Default|OnPercentChange _asbp_stock_pile_stack_3 (/ (- Percentage 0.5) 0.25))
        (else
          (bind _asbp_stock_pile_stack_4 (Utilities|Casting|CastToBP_StockPileStack (Variables|/Script/Engine.ChildActorComponent|GetChildActor (Variables|Default|GetStack4))))
          (Default|OnPercentChange _asbp_stock_pile_stack_4 (/ (- Percentage 0.75) 0.25)))))))