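; BP_StockPileStack is a stockpile placeable that displays a fill percentage as a stack of up to 25 static meshes, starting empty on BeginPlay.
; OnPercentChange clamps the 0–1 value and converts it to a count of meshes to show.
; Meshes are found by numeric component tags; those within the count become visible with collision, the rest hidden without collision.
; A missing tag prints a debug message.
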(event Custom|Set%20Visibiltiy
  (params (New%20Percent :type Float%20%28single-precision%29))
  (for _index (range 1 25)
    (if (<= _index (CallFunction|GetIndexesfromPercent New%20Percent))
      (bind _mesh_component (CallFunction|GetMeshbyTag _index))
      (Development|SetHiddeninGame _mesh_component false false)
      (Collision|SetCollisionEnabled _mesh_component "QueryAndPhysics")
      (else
        (bind _mesh_component_2 (CallFunction|GetMeshbyTag _index))
        (Development|SetHiddeninGame _mesh_component_2 true false)
        (Collision|SetCollisionEnabled _mesh_component_2 "NoCollision")))))

(event Custom|On%20Percent%20Change
  (params (New%20Percent :type Float%20%28single-precision%29))
  (CallFunction|SetVisibiltiy New%20Percent))

(event EventBeginPlay
  (CallFunction|OnPercentChange 0.0))

(fn ConstructionScript)

(fn GetMeshbyTag
  (params (Index :type Integer))
  (bind _returnvalue (Utilities|String|ToString(Integer) Index))
  (bind _returnvalue_2 (Utilities|String|StringToName _returnvalue))
  (bind _returnvalue_3 (Actor|GetComponentsbyTag "/Script/Engine.StaticMeshComponent" _returnvalue_2))
  (bind _output (Utilities|Array|Get(acopy) _returnvalue_3))
  (Utilities|IsValid _output
    (:Is%20Valid
      (return _output))
    (:Is%20Not%20Valid
      (Development|PrintString (Utilities|String|Append "Could not find mesh tag for index: " _returnvalue)))))

(fn GetIndexesfromPercent
  (params (New%20Percent :type Float%20%28single-precision%29))
  (return (/ (Math|Float|Round (* 100 (Math|Float|Clamp(Float) New%20Percent))) 4)))