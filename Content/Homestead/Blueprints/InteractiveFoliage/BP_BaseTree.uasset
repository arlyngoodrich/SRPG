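; BP_BaseTree is the base Blueprint for interactive foliage trees that drop log pickups when depleted.
; It extends the parent's fully depleted event, acting only when depletion does not come from an interaction.
; On authority, it waits a set delay, deactivates the actor and spawns a log pickup at each component tagged "Log Spawner".
; A leftover debug print fires for each spawned log.
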(event EventOnFullyDepleated
  (params (From%20Interaction :type Boolean))
  (|CallParentFunction From%20Interaction)
  (if (not From%20Interaction)
    (Networking|SwitchHasAuthority
      (:Authority
        (Utilities|FlowControl|Delay (Variables|TreeSettings|GetDelay%20to%20Spawn))
        (CallFunction|DeactivateActor)
        (for _array_element (Actor|GetComponentsbyTag "/Script/Engine.SceneComponent" "Log Spawner")
          (Game|SpawnActorfromClass (Variables|TreeSettings|GetLogPickupToSpawn) (Transformation|GetWorldTransform _array_element) "Undefined" 0 0)
          (Development|PrintString "Hello"))))))

(fn ConstructionScript
  (|CallParentFunction))