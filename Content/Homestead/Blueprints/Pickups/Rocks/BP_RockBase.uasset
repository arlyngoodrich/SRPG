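; Base Blueprint for rock pickups that gives each rock a random visual variant.
; The construction script and BeginPlay each call their parent, then independently set StaticMesh to a random pick from the first three RockMeshes entries.
; Because BeginPlay re-rolls, the mesh in play can differ from the one placed in the editor.
; The index range is hardcoded rather than derived from the array length.
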(event EventBeginPlay
  (Components|StaticMesh|SetStaticMesh (Variables|Default|GetStaticMesh) (Utilities|Array|Get(acopy) (Variables|Default|GetRock%20Meshes) (Math|Random|RandomIntegerinRange 0 2)))
  (|CallParentFunction))

(fn ConstructionScript
  (|CallParentFunction)
  (Components|StaticMesh|SetStaticMesh (Variables|Default|GetStaticMesh) (Utilities|Array|Get(acopy) (Variables|Default|GetRock%20Meshes) (Math|Random|RandomIntegerinRange 0 2))))