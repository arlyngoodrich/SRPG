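; Snap point actor for the build system that detects building pieces it can accept and is destroyed along with its parent.
; When a piece is set, it waits briefly, scans sphere overlaps for non-spawning pieces of an accepted type and calls OnSnap, which only checks validity.
; A RepNotify on IsSnapped toggles sphere collision and visibility, but the logic that sets that flag is disconnected.
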(event Custom|On%20Snap
  (params (My%20Piece :type BP%20Building%20Piece%20Base%20Object%20Reference))
  (Utilities|IsValid My%20Piece))

(event Custom|On%20Piece%20Destroyed
  (params (DestroyedActor :type Actor%20Object%20Reference)))

(event Custom|On%20Destroyed
  (params (Actor :type Actor%20Object%20Reference) (EndPlayReason :type EEndPlayReason%20Enum :default "Destroyed"))
  (if (== Actor (Variables|References|GetMy%20Parent))
    (Actor|DestroyActor)))

(event EventBeginPlay
  (bind _my_parent (Variables|References|GetMy%20Parent))
  (Utilities|IsValid _my_parent
    (:Is%20Valid
      (Game|BindEventtoOnEndPlay _my_parent (delegate Custom|On%20Destroyed)))))

(event EventOnBuildingPieceSet
  (Utilities|FlowControl|Delay 0.2)
  (for _array_element (Collision|GetOverlappingActors (Variables|Default|GetSphere) "/Game/SRPG/Blueprints/BuildSystem/BP_BuildingPieceBase.BP_BuildingPieceBase_C" :!class /Script/Engine.PrimitiveComponent)
    (bind _asbp_building_piece_base (Utilities|Casting|CastToBP_BuildingPieceBase _array_element))
    (if (not (Utilities|Enum|Equal(Enum) (Variables|/Script/SRPG.BuildingPiece|GetBuildStatus _asbp_building_piece_base) "BPSE_Spawning"))
      (bind _ok (CallFunction|AmIEligible _asbp_building_piece_base))
      (if _ok
        (CallFunction|OnSnap _asbp_building_piece_base)))))

(fn ConstructionScript)

(fn AmIEligible
  (params (Piece%20to%20check :type Building%20Piece%20Object%20Reference))
  (if (not (Variables|References|GetIs%20Snapped))
    (return (Utilities|Array|ContainsItem (Variables|Configuration|GetAcceptable%20Types) (Variables|/Script/SRPG.BuildingPiece|GetBuildingType Piece%20to%20check)))))

(fn OnRepIsSnapped
  (if (Variables|References|GetIs%20Snapped)
    (Collision|SetCollisionEnabled (Variables|Default|GetSphere) "NoCollision")
    (Development|SetHiddeninGame (Variables|Default|GetSphere) true false)
    (else
      (Collision|SetCollisionEnabled (Variables|Default|GetSphere) "QueryOnly")
      (Development|SetHiddeninGame (Variables|Default|GetSphere) false false))))