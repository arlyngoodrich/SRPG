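; BP_BuildingRoot is the manager actor for one player-built structure in the build system, tracking its pieces and persisting them through saves.
; Pieces check in and out, triggering delayed connection-level updates and snap-point rechecks, and the root destroys itself when the last piece leaves.
; Save-system events store each piece's class, build status and transform in parallel arrays, then respawn the pieces on load with the root reassigned.
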(event Custom|Call%20update%20Pieces
  (Utilities|FlowControl|Delay 0.01)
  (for _array_element (Variables|Default|GetMy%20Building%20Pieces)
    (Utilities|IsValid _array_element
      (:Is%20Valid
        (Default|UpdateConnectionLevel _array_element))))
  (CallFunction|UpdateSnaps)
  (Default|CallOnPieceCheckOut))

(event EventActorLoaded
  (CallFunction|LoadSavedBuildings))

(event EventActorPreSave
  (CallFunction|SaveBuildingData))

(event EventDestroyed
  (Default|CallOnDestroy)
  (Development|PrintString "destroyed"))

(fn ConstructionScript)

(fn CheckinPiece
  (params (Piece%20to%20add :type BP%20Building%20Piece%20Base%20Object%20Reference%20%28by%20ref%29))
  (Utilities|Array|AddUnique (Variables|Default|GetMy%20Building%20Pieces) Piece%20to%20add)
  (CallFunction|CallUpdatePieces))

(fn CheckOutPiece
  (params (Item%20to%20Remove :type BP%20Building%20Piece%20Base%20Object%20Reference%20%28by%20ref%29))
  (bind _print_to_screen (Variables|Default|GetPrint%20to%20Screen))
  (bind _returnvalue (Utilities|Array|RemoveItem (Variables|Default|GetMy%20Building%20Pieces) Item%20to%20Remove))
  (if _returnvalue
    (Development|PrintString "Item Removed" _print_to_screen false)
    (if (== (Utilities|Array|Length (Variables|Default|GetMy%20Building%20Pieces)) 0)
      (Actor|DestroyActor)
      (else
        (CallFunction|CallUpdatePieces)))
    (else
      (Development|PrintString "Failed to remvoe item" _print_to_screen false))))

(fn UpdateSnaps
  (for _array_element (Variables|Default|GetMy%20Building%20Pieces)
    (Utilities|IsValid _array_element
      (:Is%20Valid
        (for _array_element_2 (Actor|GetComponentsByClass _array_element "/Game/SRPG/Blueprints/BuildSystem/BPC_SnapPointSpawn.BPC_SnapPointSpawn_C")
          (Utilities|IsValid (Variables|/Game/SRPG/Blueprints/BuildSystem/BPC_SnapPointSpawn.BPC_SnapPointSpawn_C|GetAttached%20Snap%20Point _array_element_2)
            (:Is%20Valid
              (Default|CheckforSnaps (Variables|/Game/SRPG/Blueprints/BuildSystem/BPC_SnapPointSpawn.BPC_SnapPointSpawn_C|GetAttached%20Snap%20Point _array_element_2)))))))))

(fn SaveBuildingData
  (CallFunction|ClearSavedData)
  (for _array_element (Variables|Default|GetMy%20Building%20Pieces)
    (Utilities|Array|Add (Variables|Default|GetSaved%20Building%20Pieces) (Utilities|GetClass _array_element))
    (Utilities|Array|Add (Variables|Default|GetSaved%20Building%20States) (Variables|/Script/SRPG.BuildingPiece|GetBuildStatus _array_element))
    (Utilities|Array|Add (Variables|Default|GetSaved%20Building%20Transforms) (Transformation|GetActorTransform _array_element))))

(fn LoadSavedBuildings
  (for (_array_element _array_index) (Variables|Default|GetSaved%20Building%20Pieces)
    (LocalVariables|SetCurrent%20Index _array_index)
    (bind _returnvalue (Game|SpawnActorfromClass _array_element (Utilities|Array|Get(acopy) (Variables|Default|GetSaved%20Building%20Transforms) (LocalVariables|GetCurrent%20Index)) "Undefined" 0 false 0))
    (Variables|/Game/SRPG/Blueprints/BuildSystem/BP_BuildingPieceBase.BP_BuildingPieceBase_C|SetBuilding%20Root _returnvalue self)
    (Default|OnSpawnStart _returnvalue)
    (Default|PerformSpawnLoop _returnvalue (Utilities|Array|Get(acopy) (Variables|Default|GetSaved%20Building%20Transforms) (LocalVariables|GetCurrent%20Index)))
    (Default|OnSpawnFinished _returnvalue)
    (Class|BuildingPiece|SetBuildStatusfromLoad _returnvalue (Utilities|Array|Get(acopy) (Variables|Default|GetSaved%20Building%20States) (LocalVariables|GetCurrent%20Index))))
  (CallFunction|ClearSavedData))

(fn ClearSavedData
  (Utilities|Array|Clear (Variables|Default|GetSaved%20Building%20Pieces))
  (Utilities|Array|Clear (Variables|Default|GetSaved%20Building%20States))
  (Utilities|Array|Clear (Variables|Default|GetSaved%20Building%20Transforms)))

(fn ComponentstoSave
  (return 0))