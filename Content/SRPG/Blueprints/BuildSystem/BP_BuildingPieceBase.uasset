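; Base actor for placeable build-system pieces, handling preview placement and an interact-to-build, then interact-to-destroy lifecycle.
; During spawning it snaps to the nearest eligible snap point and tints by overlap and snap validity.
; Once set, it registers with a shared or new BuildingRoot and derives a connection level from built neighbours, destroying itself if unsupported.
; Built pieces restore their materials and can hide grass foliage instances, re-adding them on destruction.
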(event InteractionTriggered(BPC_InteractableObjectComponent)
  (params (Player%20Interaction%20Sensor :type BPC%20Player%20Interaction%20Sensor%20Object%20Reference) (Interaction%20Index :type Integer))
  (Utilities|IsValid (Variables|Default|GetBPC_InteractableObjectComponent)
    (:Is%20Valid
      (switch Utilities|FlowControl|Switch|SwitchonEBuildingPieceStatus (Variables|Default|GetBuildStatus)
        (:BPSE_Set
          (Class|BuildingPiece|UpdateBuildStatus "BPSE_FullyBuilt"))
        (:BPSE_FullyBuilt
          (Actor|DestroyActor))))))

(event Custom|Remove%20Foliage%20Multicast
  (FoliageControl|RemoveFoliage))

(event Custom|Update%20Materials
  (params (Array :type Array%20of%20Material%20Interface%20Object%20References))
  (Utility|SetMaterials Array))

(event Custom|Set%20Material%20to%20Color
  (params (Value :type Linear%20Color%20Structure))
  (Utility|SetMaterialColor Value))

(event EventBeginPlay
  (Utility|Initalize))

(event EventDestroyed
  (bind _building_root (Variables|BuildingInformation|GetBuilding%20Root))
  (if (Utilities|Enum|NotEqual(Enum) (Variables|Default|GetBuildStatus) "BPSE_Spawning")
    (Default|CallDestroyed)
    (Utilities|IsValid _building_root
      (:Is%20Valid
        (Default|CheckOutPiece _building_root self)
        (if (Variables|SpawnConfig|GetRemove%20Grass)
          (FoliageControl|ReturnFoliage))))))

(event EventOnBuildStatusChangetoBuilt
  (Development|PrintString "Changed to fully built")
  (CallFunction|UpdateMaterials (Variables|Utility|GetDefault%20Materials))
  (Variables|/Game/SRPG/Blueprints/InteractionSystem/BPC_InteractableObjectComponent.BPC_InteractableObjectComponent_C|SetInteraction%20Prompt (Variables|Default|GetBPC_InteractableObjectComponent) (Utilities|Array|MakeArray "destroy"))
  (if (Variables|SpawnConfig|GetRemove%20Grass)
    (CallFunction|RemoveFoliageMulticast)))

(event EventOnBuildStatusChangetoSet
  (bind _bpc_interactableobjectcomponent (Variables|Default|GetBPC_InteractableObjectComponent))
  (CallFunction|SetMaterialtoColor (Variables|SpawnConfig|GetSpawn%20OK%20Color))
  (Default|CallSpawnFinished)
  (Collision|SetCollisionObjectType (Variables|Default|GetStaticMesh) "ECC_WorldDynamic")
  (bind _outactors (Actor|GetAllActorswithInterface "/Game/SRPG/Blueprints/BuildSystem/BPI_BuildSystem.BPI_BuildSystem_C"))
  (Class|BPIBuildSystem|OnBuildingPieceSet(Message) _outactors)
  (ConnectionSystem|UpdateConnectionLevel)
  (Utilities|IsValid _bpc_interactableobjectcomponent
    (:Is%20Valid
      (Variables|/Game/SRPG/Blueprints/InteractionSystem/BPC_InteractableObjectComponent.BPC_InteractableObjectComponent_C|SetInteraction%20Prompt _bpc_interactableobjectcomponent (Utilities|Array|MakeArray "build")))
    (:Is%20Not%20Valid
      _))
  (ConnectionSystem|UpdateConnectionLevel)
  (CallFunction|SetMaterialtoColor (Utilities|Select :Index (Variables|Default|GetConnectionLevel) :BCLE_Foundation (Variables|ConnectionSystem|GetFoundation) :BCLE_First (Variables|ConnectionSystem|GetFirst) :BCLE_Second (Variables|ConnectionSystem|GetSecond) :BCLE_Third (Variables|ConnectionSystem|GetThird) :BCLE_Fourth (Variables|ConnectionSystem|GetToo%20Far) :BCLE_TooFar (Variables|ConnectionSystem|GetToo%20Far) :BCLE_None "(R=1.000000,G=1.000000,B=1.000000,A=1.000000)")))

(fn ConstructionScript)

(fn PerformSpawnLoop
  (params (Input%20Location :type Transform))
  (LocalVariables|SetView%20Location Input%20Location)
  (bind (_new_location _ok_to_spawn) (SpawnLoop|PerformSnapCheck (LocalVariables|GetView%20Location)))
  (bind _output_get (LocalVariables|SetFinal%20Locaiton _new_location))
  (Transformation|SetActorTransform _output_get)
  (bind _spawn_ok (SpawnLoop|PerformOverlapCheck))
  (Utility|SetMaterialColor (select (select (Variables|SpawnConfig|GetClippingOK) _ok_to_spawn (and _spawn_ok _ok_to_spawn)) (Variables|SpawnConfig|GetSpawn%20OK%20Color) (Variables|SpawnConfig|GetSpawn%20Not%20OK%20Color)))
  (return (LocalVariables|GetFinal%20Locaiton) (select (Variables|SpawnConfig|GetClippingOK) _ok_to_spawn (and _spawn_ok _ok_to_spawn))))

(fn PerformOverlapCheck
  (bind _brequiresterrain (Variables|Default|GetbRequiresTerrain))
  (bind _overlappingbuildingpieces (Utility|GetAllOverlappingPieces))
  (LocalVariables|SetOverlapped%20BuildingPieces _overlappingbuildingpieces)
  (for _array_element (LocalVariables|GetOverlapped%20BuildingPieces)
    (bind _asbp_building_piece_base (Utilities|Casting|CastToBP_BuildingPieceBase _array_element))
    (if (Utilities|Enum|Equal(Enum) (Variables|/Script/SRPG.BuildingPiece|GetBuildStatus _asbp_building_piece_base) "BPSE_FullyBuilt")
      (Math|Integer|IncrementInt (LocalVariables|GetCount%20of%20Overlapped%20Built%20Actors))))
  (LocalVariables|SetOverlapping%20Actors (Collision|GetOverlappingActors (Variables|Default|GetStaticMesh) 0 :!class /Script/Engine.PrimitiveComponent))
  (Utilities|Array|RemoveItem (LocalVariables|GetOverlapping%20Actors) self)
  (for _array_element_2 (LocalVariables|GetOverlapping%20Actors)
    (Utilities|Casting|CastToBuildingPiece _array_element_2
      (:CastFailed
        (Utilities|Casting|CastToBP_SnapPointActor _array_element_2
          (:CastFailed
            (Utilities|Casting|CastToLandscape _array_element_2
              (:then
                (LocalVariables|SetLandscape%20Overlapped true))
              (:CastFailed
                (Math|Integer|IncrementInt (LocalVariables|GetCount%20of%20Overlapped%20Non%20Building%20Actors)))))))))
  (if (== (LocalVariables|GetCount%20of%20Overlapped%20Non%20Building%20Actors) 0)
    (if _brequiresterrain
      (return (Math|Boolean|Equal(Boolean) _brequiresterrain (LocalVariables|GetLandscape%20Overlapped)))
      (elif (Variables|Default|GetbRequiresBuildingPiece)
        (return (> (LocalVariables|GetCount%20of%20Overlapped%20Built%20Actors) 0))
        (else
          (return true))))
    (else
      (return false))))

(fn PerformSnapCheck
  (params (Current%20Location :type Transform))
  (bind (_new_location _snapped) (SpawnLoop|SnaptoLocation Current%20Location))
  (bind _output_get (Variables|BuildingInformation|SetIs%20Snapped _snapped))
  (if _output_get
    (return _new_location true)
    (else
      (return _new_location (not (Variables|Default|GetbRequiresSnap))))))

(fn SetMaterialColor
  (params (Value :type Linear%20Color%20Structure))
  (Utilities|IsValid (Variables|Default|GetStaticMesh)
    (:Is%20Valid
      (for _index (range 0 (- (Rendering|Material|GetNumMaterials (Variables|Default|GetStaticMesh)) 1))
        (bind _returnvalue (Rendering|Material|CreateDynamicMaterialInstance (Variables|Default|GetStaticMesh) _index "/Game/SRPG/Blueprints/BuildSystem/MI_SpawnMaterial.MI_SpawnMaterial" "None" :!class /Script/Engine.PrimitiveComponent))
        (Rendering|Material|SetVectorParameterValue _returnvalue "Base Color" Value :!class /Script/Engine.MaterialInstanceDynamic)
        (Rendering|Material|SetScalarParameterValue _returnvalue "Opacity" (Variables|SpawnConfig|GetOpacity) :!class /Script/Engine.MaterialInstanceDynamic)))))

(fn SnaptoLocation
  (params (View%20Location :type Transform))
  (bind _snappedpoints (LocalVariables|GetSnappedPoints))
  (bind _distances (LocalVariables|GetDistances))
  (bind _indexofminvalue (Math|Float|MinOfFloatArray _distances))
  (bind _output (Utilities|Array|Get(acopy) _snappedpoints _indexofminvalue))
  (Transformation|SetActorTransform View%20Location)
  (Utilities|Array|Clear (LocalVariables|GetSnappedPoints))
  (Variables|BuildingInformation|SetIs%20Snapped false)
  (for _array_element (Collision|GetOverlappingActors (Variables|Default|GetSnapPointcheck) "/Game/SRPG/Blueprints/BuildSystem/BP_SnapPointActor.BP_SnapPointActor_C" :!class /Script/Engine.PrimitiveComponent)
    (bind _asbp_snap_point_actor (Utilities|Casting|CastToBP_SnapPointActor _array_element))
    (bind _ok (Default|AmIEligible _asbp_snap_point_actor self))
    (if _ok
      (Utilities|Array|Add (LocalVariables|GetDistances) (Math|Vector|Distance(Vector) (Transformation|GetActorLocation _asbp_snap_point_actor) (Transformation|GetActorLocation)))
      (Utilities|Array|Add (LocalVariables|GetSnappedPoints) _asbp_snap_point_actor)))
  (if (> (Utilities|Array|Length (LocalVariables|GetSnappedPoints)) 0)
    (Variables|BuildingInformation|SetSnap%20Point _output)
    (return (Transformation|GetActorTransform _output) true)
    (else
      (Variables|BuildingInformation|SetSnap%20Point 0)
      (return View%20Location false))))

(fn OnSpawnFinished
  (bind _snap_point (Variables|BuildingInformation|GetSnap%20Point))
  (bind _my_parent (Variables|/Game/SRPG/Blueprints/BuildSystem/BP_SnapPointActor.BP_SnapPointActor_C|GetMy%20Parent _snap_point))
  (Class|BuildingPiece|UpdateBuildStatus "BPSE_Set")
  (bind _snappointcheck (Variables|Default|GetSnapPointcheck)
    (:then
      (Components|DestroyComponent _snappointcheck))
    (:else
      _))
  (if (Variables|SpawnConfig|GetbPartofBuilding)
    (if (Variables|BuildingInformation|GetIs%20Snapped)
      (Utilities|IsValid _my_parent
        (:Is%20Valid
          (bind _asbp_building_piece_base (Utilities|Casting|CastToBP_BuildingPieceBase _my_parent))
          (bind _output_get (Variables|BuildingInformation|SetBuilding%20Root (Variables|BP_BuildingPieceBase_C|GetBuilding%20Root _asbp_building_piece_base)))
          (Default|CheckinPiece _output_get self))
        (:Is%20Not%20Valid
          (Development|PrintString "No Valid Root")))
      (else
        (bind _returnvalue (Game|SpawnActorfromClass "/Game/SRPG/Blueprints/BuildSystem/BP_BuildingRoot.BP_BuildingRoot_C" (Math|Transform|MakeTransform "0, 0, 0" "0, 0, 0" "1,1,1") "AlwaysSpawn" 0 0))
        (bind _output_get_2 (Variables|BuildingInformation|SetBuilding%20Root _returnvalue))
        (Default|CheckinPiece _output_get_2 self)))))

(fn OnSpawnStart
  (Collision|SetCollisionObjectType (Variables|Default|GetStaticMesh) "ECC_GameTraceChannel1")
  (Networking|SwitchHasAuthority
    (:Authority
      (Networking|SetReplicates false)
      (if (Utilities|Enum|Equal(Enum) (Networking|GetLocalRole) "ROLE_AutonomousProxy")
        (Actor|DestroyActor)))))

(fn SetMaterials
  (params (Array :type Array%20of%20Material%20Interface%20Object%20References))
  (for (_array_element _array_index) Array
    (Rendering|Material|SetMaterial (Variables|Default|GetStaticMesh) _array_index _array_element)))

(fn Initalize
  (Variables|Utility|SetDefault%20Materials (Rendering|Material|GetMaterials (Variables|Default|GetStaticMesh)))
  (for _array_element (Actor|GetComponentsbyTag "/Script/Engine.BoxComponent" "OverlappCheckVolume")
    (Collision|SetCollisionEnabled _array_element "NoCollision")))

(fn UpdateConnectionLevel
  (bind _overlappingbuildingpieces (Utility|GetAllOverlappingPieces))
  (for _array_element _overlappingbuildingpieces
    (if (Utilities|Enum|Equal(Enum) (Variables|/Script/SRPG.BuildingPiece|GetBuildStatus _array_element) "BPSE_FullyBuilt")
      (Utilities|Array|AddUnique (LocalVariables|GetConnect%20Connection%20Levels) (Variables|/Script/SRPG.BuildingPiece|GetConnectionLevel _array_element))))
  (for _array_element_2 (LocalVariables|GetConnect%20Connection%20Levels)
    (if (< _array_element_2 (LocalVariables|GetMin%20Connection%20Level))
      (LocalVariables|SetMin%20Connection%20Level _array_element_2)))
  (if (> (Utilities|Array|Length (LocalVariables|GetConnect%20Connection%20Levels)) 0)
    (if (Variables|ConnectionSystem|GetbConnectionsDecrease)
      (if (> (LocalVariables|GetMin%20Connection%20Level) (Variables|Default|GetConnectionLevel))
        (Actor|DestroyActor)
        (else
          (bind _outconnecitonlevel (Class|BuildingPiece|IncreaseConnectionLevel (LocalVariables|GetMin%20Connection%20Level)))
          (if (Utilities|Enum|Equal(Enum) _outconnecitonlevel "BCLE_TooFar")
            (Actor|DestroyActor)
            (else
              (Class|BuildingPiece|SetConnectionLevel _outconnecitonlevel))))))
    (elif (Variables|ConnectionSystem|GetbConnectionsDecrease)
      (if (or (Variables|Default|GetbRequiresBuildingPiece) (Variables|Default|GetbRequiresSnap))
        (Actor|DestroyActor)
        (else
          (Class|BuildingPiece|SetConnectionLevel (LocalVariables|GetMin%20Connection%20Level)))))))

(fn GetAllOverlappingPieces
  (Utilities|IsValid (Variables|Default|GetBoxVolume)
    (:Is%20Valid
      (for _array_element (Actor|GetComponentsbyTag "/Script/Engine.BoxComponent" "OverlappCheckVolume")
        (Collision|SetCollisionEnabled _array_element "QueryOnly")
        (for _array_element_2 (Collision|GetOverlappingActors _array_element "BP_BuildingPieceBase_C" :!class /Script/Engine.PrimitiveComponent)
          (bind _asbp_building_piece_base (Utilities|Casting|CastToBP_BuildingPieceBase _array_element_2))
          (Utilities|Array|AddUnique (LocalVariables|GetConnected%20pieces) _asbp_building_piece_base)))
      (for _array_element_3 (Actor|GetComponentsbyTag "/Script/Engine.BoxComponent" "OverlappCheckVolume")
        (Collision|SetCollisionEnabled _array_element_3 "NoCollision"))
      (Utilities|Array|RemoveItem (LocalVariables|GetConnected%20pieces) self)
      (return (LocalVariables|GetConnected%20pieces)))))

(fn RemoveFoliage
  (bind _returnvalue (Transformation|GetActorRotation))
  (bind _foliage_remove_x_max (Variables|Default|GetFoliage%20Remove%20X%20Max))
  (bind _returnvalue_2 (Math|Trig|Cos(Degrees) (.yaw _returnvalue)))
  (bind _returnvalue_3 (Math|Trig|Sin(Degrees) (.yaw _returnvalue)))
  (bind _returnvalue_4 (Transformation|GetWorldLocation _foliage_remove_x_max))
  (bind _outactors (Actor|GetAllActorsOfClass "/Script/Foliage.InstancedFoliageActor"))
  (Variables|FoliageControl|SetFoliage%20Actor (Utilities|Array|Get(acopy) _outactors))
  (bind _poly_center (Utilities|2DGridExecutionMacro :Sector%20Size 1e+02 :X (Math|Float|Truncate (/ (Math|Vector|Distance(Vector) (Transformation|GetWorldLocation (Variables|Default|GetFoliage%20Remove%20X%20Min)) _returnvalue_4) 1e+02)) :Y (Math|Float|Truncate (/ (Math|Vector|Distance(Vector) _returnvalue_4 (Transformation|GetWorldLocation (Variables|Default|GetFoliage%20Remove%20Y%20Max))) 1e+02)))
    (:Per%20Poly%20Execution
      (bind _outhit (Collision|LineTraceForObjects (+ (+ (Math|Vector|MakeVector (- (* (.X (Math|Vector|BreakVector _poly_center)) _returnvalue_2) (* (.Y (Math|Vector|BreakVector _poly_center)) _returnvalue_3)) (+ (* (.Y (Math|Vector|BreakVector _poly_center)) _returnvalue_2) (* (.X (Math|Vector|BreakVector _poly_center)) _returnvalue_3)) 0.0) (Transformation|GetActorLocation)) (Math|Vector|MakeVector 0.0 0.0 5e+02)) (+ (+ (Math|Vector|MakeVector (- (* (.X (Math|Vector|BreakVector _poly_center)) _returnvalue_2) (* (.Y (Math|Vector|BreakVector _poly_center)) _returnvalue_3)) (+ (* (.Y (Math|Vector|BreakVector _poly_center)) _returnvalue_2) (* (.X (Math|Vector|BreakVector _poly_center)) _returnvalue_3)) 0.0) (Transformation|GetActorLocation)) (Math|Vector|MakeVector 0.0 0.0 -5e+02)) (Utilities|Array|MakeArray "ObjectTypeQuery1") false 0 "ForDuration" true "(R=1.000000,G=0.000000,B=0.000000,A=1.000000)" "(R=0.000000,G=1.000000,B=0.000000,A=1.000000)" 2e+01))
      (for _array_element (Actor|GetComponentsByClass (Variables|FoliageControl|GetFoliage%20Actor) "/Game/Homestead/Blueprints/FoliageSpawners/TemperateGrass/BPC_GrassFoliage.BPC_GrassFoliage_C")
        (LocalVariables|SetOverlapped%20Instances (Class|InstancedStaticMeshComponent|GetInstancesOverlappingSphere _array_element (.location _outhit) 1e+02 true))
        (for _array_element_2 (Class|InstancedStaticMeshComponent|GetInstancesOverlappingSphere _array_element (.location _outhit) 1e+02 true)
          (Utilities|Array|Add (Variables|FoliageControl|GetFoliage%20Components) _array_element)
          (Utilities|Array|Add (Variables|FoliageControl|GetFoliage%20Transforms) (.OutInstanceTransform (Components|InstancedStaticMesh|GetInstanceTransform _array_element _array_element_2 true))))
        (for _array_element_3 (LocalVariables|GetOverlapped%20Instances)
          (Components|InstancedStaticMesh|UpdateInstanceTransform _array_element _array_element_3 (Math|Transform|MakeTransform "0, 0,-7000.000000" "0, 0, 0" "0.000000,0.000000,0.000000") false false false))))))

(fn ReturnFoliage
  (for (_array_element _array_index) (Variables|FoliageControl|GetFoliage%20Components)
    (Class|InstancedStaticMeshComponent|AddInstanceWorldSpace _array_element (Utilities|Array|Get(acopy) (Variables|FoliageControl|GetFoliage%20Transforms) _array_index))))