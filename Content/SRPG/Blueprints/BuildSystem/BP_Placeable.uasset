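; Placeable build-system piece that depends on overlapping building pieces and destroys itself when none remain.
; When set or built, it takes the first overlapping piece's BuildingRoot and binds to that root's destroy and piece-check-out events.
; Either event triggers a briefly delayed overlap recheck.
; Save hooks store the build status and restore it on load with authority, while remote copies destroy themselves.
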(event Custom|Check%20if%20still%20connected
  (Utilities|FlowControl|Delay 0.01)
  (bind _overlappingbuildingpieces (CallFunction|GetAllOverlappingPieces))
  (if (== (Utilities|Array|Length _overlappingbuildingpieces) 0)
    (Actor|DestroyActor)))

(event Custom|On%20Building%20Root%20Destroyed
  (params (DestroyedActor :type Actor%20Object%20Reference))
  (CallFunction|CheckifStillConnected))

(event EventOnBuildStatusChangetoSet
  (|CallParentFunction)
  (bind _overlappingbuildingpieces (CallFunction|GetAllOverlappingPieces))
  (Utilities|IsValid (Utilities|Array|Get(acopy) _overlappingbuildingpieces)
    (:Is%20Valid
      (Utilities|IsValid (Variables|/Game/SRPG/Blueprints/BuildSystem/BP_BuildingPieceBase.BP_BuildingPieceBase_C|GetBuilding%20Root (Utilities|Array|Get(acopy) _overlappingbuildingpieces))
        (:Is%20Valid
          (bind _output_get (Variables|Default|SetBuilding%20Root (Variables|/Game/SRPG/Blueprints/BuildSystem/BP_BuildingPieceBase.BP_BuildingPieceBase_C|GetBuilding%20Root (Utilities|Array|Get(acopy) _overlappingbuildingpieces))))
          (Game|BindEventtoOnDestroyed _output_get (delegate Custom|On%20Building%20Root%20Destroyed))
          (EventDispatchers|BindEventtoOnPieceCheckOut _output_get (delegate Custom|Check%20if%20still%20connected)))))))

(event EventActorPreSave
  (Variables|Default|SetSave%20Build%20State (Variables|Default|GetBuildStatus)))

(event EventActorLoaded
  (Networking|SwitchHasAuthority
    (:Authority
      (Class|BuildingPiece|SetBuildStatusfromLoad (Variables|Default|GetSave%20Build%20State)))
    (:Remote
      (Actor|DestroyActor))))

(event EventOnBuildStatusChangetoBuilt
  (|CallParentFunction)
  (bind _overlappingbuildingpieces (CallFunction|GetAllOverlappingPieces))
  (Utilities|IsValid (Utilities|Array|Get(acopy) _overlappingbuildingpieces)
    (:Is%20Valid
      (Utilities|IsValid (Variables|/Game/SRPG/Blueprints/BuildSystem/BP_BuildingPieceBase.BP_BuildingPieceBase_C|GetBuilding%20Root (Utilities|Array|Get(acopy) _overlappingbuildingpieces))
        (:Is%20Valid
          (bind _output_get (Variables|Default|SetBuilding%20Root (Variables|/Game/SRPG/Blueprints/BuildSystem/BP_BuildingPieceBase.BP_BuildingPieceBase_C|GetBuilding%20Root (Utilities|Array|Get(acopy) _overlappingbuildingpieces))))
          (Game|BindEventtoOnDestroyed _output_get (delegate Custom|On%20Building%20Root%20Destroyed))
          (EventDispatchers|BindEventtoOnPieceCheckOut _output_get (delegate Custom|Check%20if%20still%20connected)))))))

(fn ConstructionScript
  (|CallParentFunction))

(fn ComponentstoSave
  (return 0))