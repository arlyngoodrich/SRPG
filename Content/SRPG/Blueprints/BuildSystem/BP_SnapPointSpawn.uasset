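; BP_SnapPointSpawn is a component on building pieces that spawns a snap point actor for the build system.
; On BeginPlay it casts its owner to BP_BuildingPieceBase and binds to that piece's spawn-finished event.
; When the event fires, it spawns a BP_SnapPointActor at its own world transform, passing the parent piece and acceptable types, and keeps a reference to it.
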(event Custom|On%20Spawn%20Finished
  (bind _returnvalue (Game|SpawnActorfromClass "/Game/SRPG/Blueprints/BuildSystem/BP_SnapPointActor.BP_SnapPointActor_C" (Transformation|GetWorldTransform self) "Undefined" 0 (Variables|References|GetMy%20Owner) (Variables|Configuration|GetAceeptable%20Types) 0))
  (Variables|References|SetAttached%20Snap%20Point _returnvalue))

(event EventBeginPlay
  (bind _asbp_building_piece_base (Utilities|Casting|CastToBP_BuildingPieceBase (Components|GetOwner)))
  (bind _output_get (Variables|References|SetMy%20Owner _asbp_building_piece_base))
  (EventDispatchers|BindEventtoSpawnFinished _output_get (delegate Custom|On%20Spawn%20Finished)))