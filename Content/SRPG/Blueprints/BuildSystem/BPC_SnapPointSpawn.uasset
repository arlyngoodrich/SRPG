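; BPC_SnapPointSpawn is a build-system scene component that adds a snap point to a building piece once it is built.
; On BeginPlay it binds to the OnBuilt event of its BP_BuildingPieceBase owner.
; When that fires, it spawns a BP_SnapPointActor at its own world location and rotation, passing the owner as parent along with its accepted types, snap limit and debug flag.
; It stores the spawned actor as AttachedSnapPoint.
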(event Custom|On%20Built%20Finished
  (bind _self self)
  (bind _returnvalue (Transformation|GetWorldTransform _self))
  (bind _returnvalue_2 (Game|SpawnActorfromClass "/Game/SRPG/Blueprints/BuildSystem/BP_SnapPointActor.BP_SnapPointActor_C" (Math|Transform|MakeTransform (.location _returnvalue) (.rotation _returnvalue) "1,1,1") "Undefined" 0 (Variables|References|GetMy%20Owner) (Variables|Configuration|GetAceeptable%20Types) (Variables|Configuration|GetMaxNumberOfSnaps) (Variables|Configuration|GetDebug) 0))
  (Variables|References|SetAttached%20Snap%20Point _returnvalue_2))

(event EventBeginPlay
  (bind _output_get (Variables|References|SetMy%20Owner (Components|GetOwner)))
  (bind _asbp_building_piece_base (Utilities|Casting|CastToBP_BuildingPieceBase _output_get))
  (EventDispatchers|BindEventtoOnBuilt _asbp_building_piece_base (delegate Custom|On%20Built%20Finished)))