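; Player component that runs building placement, previewing a piece where the camera looks and placing it on confirm.
; A looping timer line-traces from the camera and passes a rotation-adjusted transform to the preview piece, which returns a location and validity.
; Stopping either cancels or, if valid, destroys the preview and spawns the final piece at the last transform via ClientSetBuilding.
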(event Custom|Start%20Build%20Loop
  (params (Building%20Piece :type BP%20Building%20Piece%20Base%20Class%20Reference))
  (bind _output_get (Variables|BuildLoop|SetBuilding%20Piece%20Class Building%20Piece))
  (if (Utilities|IsValidClass _output_get)
    (Variables|BuildLoop|SetRotation "0, 0, 0")
    (bind _returnvalue (Utilities|Time|SetTimerbyEvent (delegate Custom|Build%20Loop) (Variables|Config|GetCheck%20Frequency) true))
    (Variables|References|SetBuild%20Loop%20Timer _returnvalue)))

(event Custom|Build%20Loop
  (Utilities|IsValid (Variables|BuildLoop|GetActive%20Piece)
    (:Is%20Valid
      _)
    (:Is%20Not%20Valid
      (bind _returnvalue (Game|SpawnActorfromClass (Variables|BuildLoop|GetBuilding%20Piece%20Class) (Math|Transform|MakeTransform "0, 0, 0" "0, 0, 0" "1,1,1") "Undefined" 0 0))
      (bind _output_get (Variables|BuildLoop|SetActive%20Piece _returnvalue))
      (Default|OnSpawnStart _output_get)))
  (bind _hit_locaiton (CallFunction|GetLocationfromView))
  (bind _returnvalue_2 (CallFunction|MakeTransform _hit_locaiton "0, 0, 0"))
  (bind (_outputlocation _spawn_ok) (Default|PerformSpawnLoop (Variables|BuildLoop|GetActive%20Piece) _returnvalue_2))
  (Variables|BuildLoop|SetLast%20Valid%20Transform _outputlocation)
  (Variables|BuildLoop|SetSpawn%20OK _spawn_ok))

(event Custom|Stop%20Build%20Loop
  (params (Clear%20Build :type Boolean))
  (bind _active_piece (Variables|BuildLoop|GetActive%20Piece))
  (bind _last_valid_transform (Variables|BuildLoop|GetLast%20Valid%20Transform))
  (bind (_location _rotation) (Math|Transform|BreakTransform _last_valid_transform))
  (Utilities|IsValid _active_piece
    (:Is%20Valid
      (if Clear%20Build
        (Actor|DestroyActor _active_piece)
        (Utilities|Time|ClearandInvalidateTimerbyHandle (Variables|References|GetBuild%20Loop%20Timer))
        (Default|CallBuildLoopFinished)
        (elif (Variables|BuildLoop|GetSpawn%20OK)
          (Utilities|Time|ClearandInvalidateTimerbyHandle (Variables|References|GetBuild%20Loop%20Timer))
          (Default|CallBuildLoopFinished)
          (Actor|DestroyActor (Variables|BuildLoop|GetActive%20Piece))
          (CallFunction|ClientSetBuilding (Variables|BuildLoop|GetBuilding%20Piece%20Class) _location _rotation (Variables|BuildLoop|GetSpawn%20OK)))))))

(event Custom|Client%20Set%20Building
  (params (Building%20Piece :type BP%20Building%20Piece%20Base%20Class%20Reference) (Location :type Vector) (Rotation :type Rotator) (Spawn%20OK :type Boolean))
  (bind _returnvalue (Math|Transform|MakeTransform Location Rotation))
  (bind _returnvalue_2 (Game|SpawnActorfromClass Building%20Piece _returnvalue "Undefined" 0 0))
  (Default|PerformSpawnLoop _returnvalue_2 _returnvalue)
  (if Spawn%20OK
    (Default|OnSpawnFinished _returnvalue_2)
    (else
      (Actor|DestroyActor _returnvalue_2)
      (Development|PrintString "byeee"))))

(event EventBeginPlay
  (CallFunction|Initalize))

(fn Initalize
  (Variables|References|SetPlayerCameraManager (Game|GetPlayerCameraManager 0)))

(fn GetLocationfromView
  (bind _playercameramanager (Variables|References|GetPlayerCameraManager))
  (bind _view_distance (Variables|Config|GetView%20Distance))
  (bind _returnvalue (Camera|GetCameraLocation _playercameramanager))
  (bind _returnvalue_2 (Transformation|GetActorForwardVector _playercameramanager))
  (bind _returnvalue_3 (* _returnvalue_2 _view_distance))
  (bind _returnvalue_4 (+ _returnvalue _returnvalue_3))
  (Utilities|IsValid _playercameramanager
    (:Is%20Valid
      (bind _outhit (Collision|LineTraceForObjects _returnvalue _returnvalue_4 (Variables|Config|GetTraceTargets) false (Utilities|Array|MakeArray (Components|GetOwner)) (select (Variables|Config|GetDebug) "ForDuration" "None") true "(R=0.000000,G=0.061501,B=1.000000,A=1.000000)" "(R=0.000000,G=1.000000,B=0.000000,A=1.000000)" (Variables|Config|GetCheck%20Frequency)))
      (return (select (.bblockinghit _outhit) (.location _outhit) _returnvalue_4) (Math|Rotator|MakeRotfromZ (.normal _outhit))))))

(fn AddRotation
  (params (Active%20Building%20Piece :type BP%20Building%20Piece%20Base%20Class%20Reference))
  (Variables|BuildLoop|SetRotation (Math|Rotator|MakeRotator (.Roll (Math|Rotator|BreakRotator (Variables|BuildLoop|GetRotation))) (.Pitch (Math|Rotator|BreakRotator (Variables|BuildLoop|GetRotation))) (+ (.Default%20Rotation (Utilities|GetClassDefaults Active%20Building%20Piece)) (.Yaw (Math|Rotator|BreakRotator (Variables|BuildLoop|GetRotation)))))))

(fn MakeTransform
  (params (Location :type Vector) (Terrain%20Allignment :type Rotator))
  (bind (_roll _pitch) (Math|Rotator|BreakRotator Terrain%20Allignment))
  (bind _active_piece (Variables|BuildLoop|GetActive%20Piece))
  (bind _rotation (Variables|BuildLoop|GetRotation))
  (bind _can_rotate_x (Variables|/Game/SRPG/Blueprints/BuildSystem/BP_BuildingPieceBase.BP_BuildingPieceBase_C|GetCan%20Rotate%20X _active_piece))
  (bind _returnvalue (Math|Rotator|SelectRotator _rotation "0, 0, 0" _can_rotate_x))
  (return (Math|Transform|MakeTransform Location (select (Variables|/Game/SRPG/Blueprints/BuildSystem/BP_BuildingPieceBase.BP_BuildingPieceBase_C|GetAlignToTerrain (Variables|BuildLoop|GetActive%20Piece)) (Math|Rotator|MakeRotator _roll _pitch (.Yaw (Math|Rotator|BreakRotator _returnvalue))) _returnvalue))))