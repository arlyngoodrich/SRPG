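; Crafting component that supplies recipes and input/output inventories for its owning actor.
; On BeginPlay, with authority only, it loads every row of the recipe data table as the crafting recipes and registers all of the owner's inventory container components as both inputs and outputs.
; For SRPG character owners, it binds to the equipment manager's UI update event to refresh those inventories, printing a debug message on each refresh.
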(event Custom|Update%20From%20Equpment%20Manager
  (CallFunction|RefreshInventories))

(event EventBeginPlay
  (CallFunction|Initalize)
  (CallFunction|RefreshInventories)
  (bind _asbp_srpgcharacter (Utilities|Casting|CastToBP_SRPGCharacter (Components|GetOwner)))
  (EventDispatchers|BindEventtoUpdateUI (Variables|/Game/SRPG/Blueprints/CharacterAssets/BP_SRPGCharacter.BP_SRPGCharacter_C|GetBPC_PlayerEquipmentManager _asbp_srpgcharacter) (delegate Custom|Update%20From%20Equpment%20Manager)))

(fn Initalize
  (if (Ability|HasAuthority (Components|GetOwner))
    (bind _outrownames (DataTable|GetDataTableRowNames (Variables|Default|GetRecipe%20Data%20Table)))
    (for _array_element _outrownames
      (bind _returnvalue (Utilities|GetDataTableRow (Variables|Default|GetRecipe%20Data%20Table) _array_element)
        (:then
          (Utilities|Array|Add (LocalVariables|GetRecepies) _returnvalue))))
    (Class|CraftingComponent|SetCraftingRecipes (LocalVariables|GetRecepies))))

(fn RefreshInventories
  (bind _returnvalue (Components|GetOwner))
  (bind _returnvalue_2 (Actor|GetComponentsByClass _returnvalue "/Game/SRPG/Blueprints/InventorySystem/BPC_InventoryContainer.BPC_InventoryContainer_C"))
  (Development|PrintString "Refreshed")
  (if (Ability|HasAuthority _returnvalue)
    (Class|CraftingComponent|SetAssociatedInputInventories _returnvalue_2)
    (Class|CraftingComponent|SetAssociatedOutputInventories _returnvalue_2)))