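; Player crafting component that supplies the recipes and inventories used for crafting on an SRPG character.
; On BeginPlay, it reads every row of the recipe data table and registers them as its crafting recipes.
; RefreshInventories assigns all of the owning character's inventory container components as both crafting inputs and outputs.
; Both setup steps run only when the owner has authority.
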(event EventBeginPlay
  (CallFunction|Initalize))

(fn Initalize
  (if (Ability|HasAuthority (Components|GetOwner))
    (bind _outrownames (DataTable|GetDataTableRowNames (Variables|Default|GetRecipe%20Data%20Table)))
    (for _array_element _outrownames
      (bind _returnvalue (Utilities|GetDataTableRow (Variables|Default|GetRecipe%20Data%20Table) _array_element)
        (:then
          (Utilities|Array|Add (LocalVariables|GetRecepies) _returnvalue))))
    (Class|CraftingComponent|SetCraftingRecipes (LocalVariables|GetRecepies))))

(fn RefreshInventories
  (bind _returnvalue (Components|GetOwner))
  (if (Ability|HasAuthority _returnvalue)
    (bind _asbp_srpgcharacter (Utilities|Casting|CastToBP_SRPGCharacter _returnvalue))
    (Class|CraftingComponent|SetAssociatedInputInventories (Actor|GetComponentsByClass _asbp_srpgcharacter "/Game/SRPG/Blueprints/InventorySystem/BPC_InventoryContainer.BPC_InventoryContainer_C"))
    (Class|CraftingComponent|SetAssociatedOutputInventories (Actor|GetComponentsByClass _asbp_srpgcharacter "/Game/SRPG/Blueprints/InventorySystem/BPC_InventoryContainer.BPC_InventoryContainer_C"))))