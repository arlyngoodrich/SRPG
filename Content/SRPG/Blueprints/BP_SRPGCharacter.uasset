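; Player character Blueprint for the SRPG game that hosts the inventory UI and routes player input to its components.
; On BeginPlay it caches the player controller and creates an inventory container widget bound to its InventoryContainer.
; The Toggle Inventory input and ToggleStorage event share one toggle that shows or hides the widget, switches input mode and cursor, and signals menu open or close.
; Interact and item-rotate inputs forward to the interaction sensor and inventory manager components.
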(event Custom|Toggle%20Storage
  (bind _player_controller (Variables|Components|GetPlayer%20Controller))
  (if (UserInterface|Viewport|IsinViewport (Variables|Default|GetInventoy%20Container%20Widget))
    (Widget|RemovefromParent (Variables|Default|GetInventoy%20Container%20Widget))
    (Input|SetInputModeGameOnly _player_controller)
    (Variables|/Script/Engine.PlayerController|SetbShowMouseCursor _player_controller false)
    (Default|CallMenuClosed)
    (else
      (UserInterface|Viewport|AddtoViewport (Variables|Default|GetInventoy%20Container%20Widget) 0)
      (Input|SetInputModeGameandUI _player_controller 0 "LockInFullscreen" true)
      (Variables|/Script/Engine.PlayerController|SetbShowMouseCursor _player_controller true)
      (Default|CallMenuOpen))))

(event EventBeginPlay
  (CallFunction|Initalize))

(event Input|ActionEvents|InputActionToggleInventory
  (params (Key :type Key%20Structure :default "None"))
  (bind _player_controller (Variables|Components|GetPlayer%20Controller))
  (:Pressed
    (if (UserInterface|Viewport|IsinViewport (Variables|Default|GetInventoy%20Container%20Widget))
      (Widget|RemovefromParent (Variables|Default|GetInventoy%20Container%20Widget))
      (Input|SetInputModeGameOnly _player_controller)
      (Variables|/Script/Engine.PlayerController|SetbShowMouseCursor _player_controller false)
      (Default|CallMenuClosed)
      (else
        (UserInterface|Viewport|AddtoViewport (Variables|Default|GetInventoy%20Container%20Widget) 0)
        (Input|SetInputModeGameandUI _player_controller 0 "LockInFullscreen" true)
        (Variables|/Script/Engine.PlayerController|SetbShowMouseCursor _player_controller true)
        (Default|CallMenuOpen)))))

(event Input|ActionEvents|InputActionRotateInventoryItem
  (params (Key :type Key%20Structure :default "None"))
  (:Pressed
    (Default|PlayerPressedRotate (Variables|Default|GetBPC_PlayerInventoryManager))))

(event Input|ActionEvents|InputActionInteract
  (params (Key :type Key%20Structure :default "None"))
  (:Pressed
    (Default|Interact (Variables|Default|GetBPC_PlayerInteractionSensor))))

(fn ConstructionScript)

(fn Initalize
  (bind _asplayer_controller (Utilities|Casting|CastToPlayerController (Pawn|GetController)))
  (bind _output_get (Variables|Components|SetPlayer%20Controller _asplayer_controller))
  (bind _returnvalue (UserInterface|CreateWidget "/Game/SRPG/Blueprints/InventorySystem/WBP_InventoryContainer.WBP_InventoryContainer_C" _output_get (Variables|Default|GetInventoryContainer)))
  (Variables|Default|SetInventoy%20Container%20Widget _returnvalue))