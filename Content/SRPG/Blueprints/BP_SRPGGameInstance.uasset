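; Game instance for the SRPG game that starts new or saved worlds, solo or hosted, and joins multiplayer sessions.
; NewWorld and LoadWorld store the world name as the current save game name and flag whether it is new, with LoadWorld first checking that the slot exists.
; Hosting creates an Advanced Session tagged with the world name, then opens the starting level as a listen server.
; ComponentsToSave is an empty stub.
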(event Custom|Join%20Session
  (params (PlayerController :type Player%20Controller%20Object%20Reference) (Session :type Blueprint%20Session%20Result%20Structure))
  (|JoinSession PlayerController Session))

(event Custom|New%20World
  (params (World%20Name :type String) (Host :type Boolean) (Player%20Controller :type Player%20Controller%20Object%20Reference))
  (bind _output_get (Variables|WorldInfo|SetWorldName World%20Name))
  (Class|EMSFunctionLibrary|SetCurrentSaveGameName _output_get)
  (Variables|References|SetPlayer%20Controller Player%20Controller)
  (Variables|WorldInfo|SetIs%20New true)
  (if Host
    (|AdvancedSession (Utilities|Array|MakeArray (Class|AdvancedSessionsLibrary|MakeLiteralSessionPropertyString "SNAME" (Variables|WorldInfo|GetWorldName))) (Variables|References|GetPlayer%20Controller) 100 0 false true false true true false false false true
      (:OnSuccess
        (Development|PrintString "Hosting")
        (Game|OpenLevel(byName) (Variables|References|GetStarting%20Level%20Name) true "?Listen"))
      (:OnFailure
        (Development|PrintString "Hosting Failed")))
    (else
      (Game|OpenLevel(byName) (Variables|References|GetStarting%20Level%20Name)))))

(event Custom|Load%20World
  (params (WorldName :type String) (Host :type Boolean) (Player%20Controller :type Player%20Controller%20Object%20Reference))
  (bind _output_get (Variables|WorldInfo|SetWorldName WorldName))
  (if (Class|EMSFunctionLibrary|DoesSaveSlotExist _output_get)
    (Class|EMSFunctionLibrary|SetCurrentSaveGameName _output_get)
    (Variables|References|SetPlayer%20Controller Player%20Controller)
    (Variables|WorldInfo|SetIs%20New false)
    (if Host
      (|AdvancedSession (Utilities|Array|MakeArray (Class|AdvancedSessionsLibrary|MakeLiteralSessionPropertyString "SNAME" (Variables|WorldInfo|GetWorldName))) (Variables|References|GetPlayer%20Controller) 100 0 false true false true true false false false true
        (:OnSuccess
          (Development|PrintString "Hosting")
          (Game|OpenLevel(byName) (Variables|References|GetStarting%20Level%20Name) true "?Listen"))
        (:OnFailure
          (Development|PrintString "Hosting Failed")))
      (else
        (Game|OpenLevel(byName) (Variables|References|GetStarting%20Level%20Name))))
    (else
      (Development|PrintString "Tried to load save slot that does not exist"))))

(fn ComponentstoSave
  (return 0))