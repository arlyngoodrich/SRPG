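; Player foliage manager on BP_SRPGCharacter that swaps nearby instanced foliage for interactive actors and adds harvested resources to the inventory.
; A server timer hides in-range instances by sinking and zero-scaling them via multicast, then spawns data-table-defined actors through a mesh-to-row map.
; Parallel arrays link actors to source components, so actors the player leaves can become instances again.
; Hidden instances are never removed; returning actors add new ones.
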(event Custom|FoliageInteractionLoop
  (for _array_element (Variables|References|GetFoliageComponents)
    (CallFunction|MulticastRemoveInstances _array_element))
  (for _array_element_2 (Variables|References|GetSpawnedFoliageActors)
    (CallFunction|ReturntoInstance _array_element_2)))

(event Custom|Multicast_AddInstances
  (params (Target :type Instanced%20Static%20Mesh%20Component%20Object%20Reference) (Target%20Foliage%20Actor :type BP%20Base%20Custom%20Foliage%20Object%20Reference) (World%20Location :type Vector) (World%20Rotation :type Rotator) (World%20Scale :type Vector))
  (Class|InstancedStaticMeshComponent|AddInstanceWorldSpace Target (Math|Transform|MakeTransform World%20Location World%20Rotation World%20Scale))
  (if (Variables|References|GetHas%20Authoirty)
    (Actor|SetLifeSpan Target%20Foliage%20Actor 0.01)))

(event Custom|Multicast%20Remove%20Instances
  (params (Foliage%20Components :type BP%20Custom%20Foliage%20Component%20Object%20Reference))
  (bind _transforms (CallFunction|RemoveInstances Foliage%20Components))
  (if (Variables|References|GetHas%20Authoirty)
    (CallFunction|SpawnActorcs _transforms Foliage%20Components)))

(event EventBeginPlay
  (bind _asbp_srpgcharacter (Utilities|Casting|CastToBP_SRPGCharacter (Components|GetOwner)))
  (bind _output_get (Variables|References|SetHas%20Authoirty (Ability|HasAuthority _asbp_srpgcharacter)))
  (if _output_get
    (bind _has_valid_foliage_ (CallFunction|Initalize))
    (if _has_valid_foliage_
      (bind _returnvalue (Utilities|Time|SetTimerbyEvent (delegate Custom|FoliageInteractionLoop) (Variables|Configuration|GetInteractionTestFrequency) true))
      (Variables|References|SetInteractionTimer _returnvalue))))

(fn CheckforFoliage)

(fn Initalize
  (bind _asbp_srpgcharacter (Utilities|Casting|CastToBP_SRPGCharacter (Components|GetOwner)))
  (Variables|References|SetMy%20Player _asbp_srpgcharacter)
  (bind _outactors (Actor|GetAllActorsOfClass "/Script/Foliage.InstancedFoliageActor"))
  (Utilities|IsValid (Utilities|Array|Get(acopy) _outactors)
    (:Is%20Valid
      (Networking|SetReplicates (Utilities|Array|Get(acopy) _outactors) true)
      (bind _output_get (Variables|References|SetFoliageComponents (Actor|GetComponentsByClass (Utilities|Array|Get(acopy) _outactors) "/Game/SRPG/Blueprints/EnviornmentSystem/BP_CustomFoliageComponent.BP_CustomFoliageComponent_C")))
      (for _array_element _output_get
        (Class|ActorComponent|SetIsReplicated _array_element true))
      (CallFunction|RefreshMeshMap)
      (return true))
    (:Is%20Not%20Valid
      (return false))))

(fn RemoveInstances
  (params (Foliage%20Component :type BP%20Custom%20Foliage%20Component%20Object%20Reference))
  (bind _output_get (LocalVariables|SetActive%20Component Foliage%20Component))
  (bind (_outinstanceindexies _outinstancetransforms) (Class|CustomFoliageISMComponent|GetInstancesinRange _output_get (Transformation|GetActorLocation (Variables|References|GetMy%20Player)) (Variables|Configuration|GetInteractionRange)))
  (LocalVariables|SetInstancesToConvert _outinstanceindexies)
  (LocalVariables|SetInstances%20Transforms _outinstancetransforms)
  (for _array_element (LocalVariables|GetInstancesToConvert)
    (Components|InstancedStaticMesh|UpdateInstanceTransform (LocalVariables|GetActive%20Component) _array_element (Math|Transform|MakeTransform "0, 0,-7000.000000" "0, 0, 0" "0.000000,0.000000,0.000000") false false false))
  (return (LocalVariables|GetInstances%20Transforms)))

(fn RefreshMeshMap
  (bind _foliage_data_table (Variables|References|GetFoliage%20Data%20Table))
  (bind _outrownames (DataTable|GetDataTableRowNames _foliage_data_table))
  (for _array_element _outrownames
    (bind _returnvalue (Utilities|GetDataTableRow _foliage_data_table _array_element)
      (:then
        (for _array_element_2 (.FolliageMeshes (Utilities|Struct|BreakFoliageInformation _returnvalue))
          (Utilities|Map|Add (Variables|References|GetMeshMap) _array_element_2 _array_element))))))

(fn ReturntoInstance
  (params (FoliageActor :type BP%20Base%20Custom%20Foliage%20Object%20Reference))
  (bind _spawnedfoliageactors (Variables|References|GetSpawnedFoliageActors))
  (bind _my_player (Variables|References|GetMy%20Player))
  (bind _owningfoliagecomponents (Variables|References|GetOwningFoliageComponents))
  (bind _owningfoliagecomponents_2 (Variables|References|GetOwningFoliageComponents))
  (bind _spawnedfoliageactors_2 (Variables|References|GetSpawnedFoliageActors))
  (Utilities|IsValid FoliageActor
    (:Is%20Valid
      (LocalVariables|SetActive%20Foliage%20Actor FoliageActor)
      (if (>= (Math|Vector|Distance(Vector) (Transformation|GetActorLocation (LocalVariables|GetActive%20Foliage%20Actor)) (Transformation|GetActorLocation (Variables|References|GetMy%20Player))) (Variables|Configuration|GetInteractionRange))
        (bind _ok_to_remove (Default|OnPlayerLeaveArea (LocalVariables|GetActive%20Foliage%20Actor) _my_player))
        (if _ok_to_remove
          (if (Utilities|Array|IsValidIndex _owningfoliagecomponents_2 (Utilities|Array|FindItem (Variables|References|GetSpawnedFoliageActors) (LocalVariables|GetActive%20Foliage%20Actor)))
            (LocalVariables|SetTraget%20Index (Utilities|Array|FindItem (Variables|References|GetSpawnedFoliageActors) (LocalVariables|GetActive%20Foliage%20Actor)))
            (CallFunction|MulticastAddInstances (Utilities|Array|Get(acopy) _owningfoliagecomponents_2 (Utilities|Array|FindItem (Variables|References|GetSpawnedFoliageActors) (LocalVariables|GetActive%20Foliage%20Actor))) (LocalVariables|GetActive%20Foliage%20Actor) (.Location (Math|Transform|BreakTransform (Transformation|GetActorTransform (LocalVariables|GetActive%20Foliage%20Actor)))) (.Rotation (Math|Transform|BreakTransform (Transformation|GetActorTransform (LocalVariables|GetActive%20Foliage%20Actor)))) (.Scale (Math|Transform|BreakTransform (Transformation|GetActorTransform (LocalVariables|GetActive%20Foliage%20Actor)))))
            (if (Utilities|Array|IsValidIndex _spawnedfoliageactors (LocalVariables|GetTraget%20Index))
              (Utilities|Array|RemoveIndex _spawnedfoliageactors (LocalVariables|GetTraget%20Index)))
            (if true
              (if (Utilities|Array|IsValidIndex _owningfoliagecomponents (LocalVariables|GetTraget%20Index))
                (Utilities|Array|RemoveIndex _owningfoliagecomponents (LocalVariables|GetTraget%20Index))))
            (else
              (Development|PrintString "In valid foliage index"))))
        (else
          (Default|OnOverlappedbyPlayer (LocalVariables|GetActive%20Foliage%20Actor) _my_player))))
    (:Is%20Not%20Valid
      ;[1 1 1] If no longer valid -- may happen if already harvested
      (if (Utilities|Array|IsValidIndex _spawnedfoliageactors_2 (Utilities|Array|FindItem (Variables|References|GetSpawnedFoliageActors) (LocalVariables|GetActive%20Foliage%20Actor)))
        (Utilities|Array|RemoveIndex _spawnedfoliageactors_2 (Utilities|Array|FindItem (Variables|References|GetSpawnedFoliageActors) (LocalVariables|GetActive%20Foliage%20Actor)))
        (Utilities|Array|RemoveIndex (Variables|References|GetOwningFoliageComponents) (Utilities|Array|FindItem (Variables|References|GetSpawnedFoliageActors) (LocalVariables|GetActive%20Foliage%20Actor)))))))

(fn SpawnActorcs
  (params (Instances%20Transforms1 :type Array%20of%20Transforms) (Foliage%20Component :type BP%20Custom%20Foliage%20Component%20Object%20Reference))
  (LocalVariables|SetActive%20Component Foliage%20Component)
  (LocalVariables|SetMesh (Variables|/Script/Engine.StaticMeshComponent|GetStaticMesh (LocalVariables|GetActive%20Component)))
  (LocalVariables|SetInstances%20Transforms Instances%20Transforms1)
  (LocalVariables|SetRow%20Name (.Value (Utilities|Map|Find (Variables|References|GetMeshMap) (Variables|/Script/Engine.StaticMeshComponent|GetStaticMesh (LocalVariables|GetActive%20Component)))))
  (bind _returnvalue (Utilities|GetDataTableRow (Variables|References|GetFoliage%20Data%20Table) (.Value (Utilities|Map|Find (Variables|References|GetMeshMap) (Variables|/Script/Engine.StaticMeshComponent|GetStaticMesh (LocalVariables|GetActive%20Component)))))
    (:then
      (bind _output_get (LocalVariables|SetFoliageInfo _returnvalue))
      (bind _asbp_base_custom_foliage (Utilities|Casting|CastToBP_BaseCustomFoliageClass (.FoliageActor (Utilities|Struct|BreakFoliageInformation _output_get))))
      (LocalVariables|SetClass%20to%20Spawn _asbp_base_custom_foliage)
      (for _array_element (LocalVariables|GetInstances%20Transforms)
        (bind _returnvalue_2 (Game|SpawnActorfromClass (LocalVariables|GetClass%20to%20Spawn) _array_element "AlwaysSpawn" 0 (LocalVariables|GetFoliageInfo) (LocalVariables|GetMesh) 0 (LocalVariables|GetRow%20Name) false 0))
        (Utilities|Array|Add (Variables|References|GetSpawnedFoliageActors) _returnvalue_2)
        (Utilities|Array|Add (Variables|References|GetOwningFoliageComponents) (LocalVariables|GetActive%20Component))))))

(fn OnHarvest
  (params (Resource%20Item%20Data :type Item%20Data%20Structure) (Quantity :type Integer))
  (bind _structout (Utilities|Struct|SetmembersinItemData Resource%20Item%20Data Quantity))
  (Default|AutoAddItem (Variables|/Game/SRPG/Blueprints/CharacterAssets/BP_SRPGCharacter.BP_SRPGCharacter_C|GetBPC_PlayerInventoryManager (Variables|References|GetMy%20Player)) _structout))