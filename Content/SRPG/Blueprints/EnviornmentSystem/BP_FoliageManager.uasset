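; Server-side foliage manager that saves and restores the level's custom foliage instances and spawned foliage actors through save-system callbacks.
; On BeginPlay it caches the InstancedFoliageActor's custom foliage components.
; Before saving, it records instance meshes and transforms in parallel arrays, skipping zero-scale instances, plus each foliage actor's mesh, transform and row name.
; On load, it clears and rebuilds instances by mesh match, then respawns actors from FoliageDataTable rows.
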(event EventActorLoaded
  (CallFunction|ClearAllInstances)
  (for _array_element (Variables|Default|GetFoliage%20Components)
    (CallFunction|LoadInstances _array_element))
  (CallFunction|LoadFoliageActors))

(event EventActorPreSave
  (Utilities|Array|Clear (Variables|Default|GetMesh%20Components))
  (Utilities|Array|Clear (Variables|Default|GetInstances%20Transforms))
  (for _array_element (Variables|Default|GetFoliage%20Components)
    (CallFunction|SaveInstances _array_element))
  (CallFunction|SaveFoliageActors))

(event EventBeginPlay
  (Networking|SwitchHasAuthority
    (:Authority
      (bind _outactors (Actor|GetAllActorsOfClass "/Script/Foliage.InstancedFoliageActor"))
      (bind _output_get (Variables|References|SetFoliage%20Actor (Utilities|Array|Get(acopy) _outactors)))
      (Variables|Default|SetFoliage%20Components (Actor|GetComponentsByClass _output_get "/Game/SRPG/Blueprints/EnviornmentSystem/BP_CustomFoliageComponent.BP_CustomFoliageComponent_C"))
      (Utilities|IsValid (Variables|References|GetFoliage%20Data%20Table)
        (:Is%20Not%20Valid
          (Development|PrintString "Foliage Manager Data Table Not Set! "))))))

(fn ConstructionScript)

(fn LoadInstances
  (params (Foliage%20Component :type BP%20Custom%20Foliage%20Component%20Object%20Reference))
  (bind _output_get (LocalVariables|SetActice%20Mesh%20Component Foliage%20Component))
  (for (_array_element _array_index) (Variables|Default|GetMesh%20Components)
    (if (== _array_element (Variables|/Script/Engine.StaticMeshComponent|GetStaticMesh _output_get))
      (Class|InstancedStaticMeshComponent|AddInstanceWorldSpace (LocalVariables|GetActice%20Mesh%20Component) (Utilities|Array|Get(acopy) (Variables|Default|GetInstances%20Transforms) _array_index)))))

(fn SaveInstances
  (params (Foliage%20Component :type BP%20Custom%20Foliage%20Component%20Object%20Reference))
  (bind _outinstancetransforms (Class|CustomFoliageISMComponent|GetAllInstances Foliage%20Component))
  (for _array_element _outinstancetransforms
    (if (not (Math|Vector|Equal(Vector) (.Scale (Math|Transform|BreakTransform _array_element)) "0, 0, 0" 0.0001))
      (Utilities|Array|Add (Variables|Default|GetInstances%20Transforms) _array_element)
      (Utilities|Array|Add (Variables|Default|GetMesh%20Components) (Variables|/Script/Engine.StaticMeshComponent|GetStaticMesh Foliage%20Component)))))

(fn ClearAllInstances
  (for _array_element (Variables|Default|GetFoliage%20Components)
    (Components|InstancedStaticMesh|ClearInstances _array_element)))

(fn SaveFoliageActors
  (Utilities|Array|Clear (Variables|Default|GetActor%20Meshes))
  (Utilities|Array|Clear (Variables|Default|GetActor%20Transforms))
  (Utilities|Array|Clear (Variables|Default|GetActor%20Foliage%20Data%20Row))
  (bind _outactors (Actor|GetAllActorsOfClass "/Game/SRPG/Blueprints/EnviornmentSystem/BP_BaseCustomFoliage.BP_BaseCustomFoliage_C"))
  (for _array_element _outactors
    (Utilities|Array|Add (Variables|Default|GetActor%20Transforms) (Transformation|GetActorTransform _array_element))
    (Utilities|Array|Add (Variables|Default|GetActor%20Foliage%20Data%20Row) (Variables|/Game/SRPG/Blueprints/EnviornmentSystem/BP_BaseCustomFoliage.BP_BaseCustomFoliage_C|GetTable%20Row%20Name _array_element))
    (Utilities|Array|Add (Variables|Default|GetActor%20Meshes) (Variables|/Game/SRPG/Blueprints/EnviornmentSystem/BP_BaseCustomFoliage.BP_BaseCustomFoliage_C|GetMyNewStaticMesh _array_element))))

(fn LoadFoliageActors
  (bind _outactors (Actor|GetAllActorsOfClass "/Game/SRPG/Blueprints/EnviornmentSystem/BP_BaseCustomFoliage.BP_BaseCustomFoliage_C"))
  (for _array_element _outactors
    (Actor|DestroyActor _array_element))
  (for (_array_element_2 _array_index) (Variables|Default|GetActor%20Foliage%20Data%20Row)
    (LocalVariables|SetRow%20Name _array_element_2)
    (LocalVariables|SetFoliage%20Transform (Utilities|Array|Get(acopy) (Variables|Default|GetActor%20Transforms) _array_index))
    (LocalVariables|SetActor%20Mesh%20Object (Utilities|Array|Get(acopy) (Variables|Default|GetActor%20Meshes) _array_index))
    (bind _returnvalue (Utilities|GetDataTableRow (Variables|References|GetFoliage%20Data%20Table) (LocalVariables|GetRow%20Name))
      (:then
        (bind _output_get (LocalVariables|SetFoliage%20Info _returnvalue))
        (bind _asbp_base_custom_foliage (Utilities|Casting|CastToBP_BaseCustomFoliageClass (Utilities|Struct|BreakFoliageInformation _output_get)))
        (LocalVariables|SetClass%20to%20Spawn _asbp_base_custom_foliage)
        (Game|SpawnActorfromClass (LocalVariables|GetClass%20to%20Spawn) (LocalVariables|GetFoliage%20Transform) "AlwaysSpawn" 0 (LocalVariables|GetFoliage%20Info) (LocalVariables|GetActor%20Mesh%20Object) (LocalVariables|GetRow%20Name) 0)))))

(fn ComponentstoSave
  (return 0))