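; Base actor that stands in for a foliage instance and lets players harvest it by interaction or damage.
; FoliageInfo drives the static or destructible mesh, harvest limits, damage filters and random rewards sent to the player's BP_PlayerFoliageManager.
; Depletion can destroy the actor, apply a physics impulse, or start a respawn timer that re-adds it as an instance on the mesh-matched foliage component.
; Overlap tracking permits switching back only while unharvested and without players nearby.
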(event Custom|Interaction%20Triggered
  (params (Player%20Interaction%20Sensor :type BPC%20Player%20Interaction%20Sensor%20Object%20Reference) (Interaction%20Index :type Integer))
  (CallFunction|OnInteractHarvest Player%20Interaction%20Sensor))

(event Custom|On%20Fully%20Depleated
  (params (From%20Interaction :type Boolean))
  (bind _foliageinfo (Variables|Configuration|GetFoliageInfo))
  (bind _foliageinfo_2 (Variables|Configuration|GetFoliageInfo))
  (bind (_busedestructablemesh _foliagedestructiblemeshes _brespawnafterinteractdepletion _timetorespawnafterinteractharvest) (Utilities|Struct|BreakFoliageInformation _foliageinfo_2))
  (bind (_busedestructablemesh_2 _foliagedestructiblemeshes_2 _brespawnafterharvestdepletion _timetorespawnafterdamageharvest _presistanceafterdepletion) (Utilities|Struct|BreakFoliageInformation _foliageinfo))
  (if From%20Interaction
    (if _brespawnafterinteractdepletion
      (CallFunction|StartRespawnTimer _timetorespawnafterinteractharvest)
      (else
        (Actor|SetLifeSpan 0.01)))
    (elif _brespawnafterharvestdepletion
      (CallFunction|StartRespawnTimer _timetorespawnafterdamageharvest)
      (CallFunction|DeactivateActor)
      (else
        (Actor|SetLifeSpan _presistanceafterdepletion)))))

(event EventActorLoaded
  (CallFunction|SetMesh)
  (CallFunction|Initalize)
  (if (.bCanInteractForHarvest (Utilities|Struct|BreakFoliageInformation (Variables|Configuration|GetFoliageInfo)))
    (CallFunction|AddInteraction)
    (EventDispatchers|BindEventtoInteractionTriggered (Variables|Default|GetInteraction%20Component) (delegate Custom|Interaction%20Triggered))))

(event Game|Damage|EventPointDamage
  (params (Damage :type Float%20%28single-precision%29) (DamageType :type Damage%20Type%20Object%20Reference) (HitLocation :type Vector :default "0, 0, 0") (HitNormal :type Vector :default "0, 0, 0") (HitComponent :type Primitive%20Component%20Object%20Reference) (BoneName :type Name :default "None") (ShotFromDirection :type Vector :default "0, 0, 0") (InstigatedBy :type Controller%20Object%20Reference) (DamageCauser :type Actor%20Object%20Reference) (HitInfo :type Hit%20Result%20Structure%20%28by%20ref%29))
  (bind _activemeshcomponent (Variables|Default|GetActiveMeshComponent))
  (bind _fully_depleted (CallFunction|OnDamageHarvest Damage DamageType DamageCauser))
  (if (and _fully_depleted (Utilities|Struct|BreakFoliageInformation (Variables|Configuration|GetFoliageInfo)))
    (Collision|SetCollisionEnabled _activemeshcomponent "QueryAndPhysics")
    (Physics|SetSimulatePhysics _activemeshcomponent true)
    (Physics|AddImpulseatLocation (Variables|Default|GetActiveMeshComponent) (* ShotFromDirection (* (Physics|GetMass (Variables|Default|GetActiveMeshComponent)) (.ForceMultiplyer (Utilities|Struct|BreakFoliageInformation (Variables|Configuration|GetFoliageInfo))))) HitLocation "None")))

(event EventBeginPlay
  (CallFunction|SetMesh)
  (CallFunction|Initalize)
  (if (.bCanInteractForHarvest (Utilities|Struct|BreakFoliageInformation (Variables|Configuration|GetFoliageInfo)))
    (CallFunction|AddInteraction)
    (EventDispatchers|BindEventtoInteractionTriggered (Variables|Default|GetInteraction%20Component) (delegate Custom|Interaction%20Triggered))))

(fn ConstructionScript)

(fn OnOverlappedbyPlayer
  (params (OverlappingCharacter :type BP%20SRPG%20Character%20Object%20Reference))
  (Utilities|Array|AddUnique (Variables|References|GetOverlapping%20Characters) OverlappingCharacter))

(fn OnPlayerLeaveArea
  (params (LeavingCharacter :type BP%20SRPG%20Character%20Object%20Reference))
  (bind _overlapping_characters (Variables|References|GetOverlapping%20Characters))
  (Utilities|Array|RemoveItem _overlapping_characters LeavingCharacter)
  (return (and (== (Utilities|Array|Length _overlapping_characters) 0) (not (Variables|HarvestInfo|GetBlock%20Switch%20back%20to%20Instance)))))

(fn OnInteractHarvest
  (params (Interaction%20Sensor :type BPC%20Player%20Interaction%20Sensor%20Object%20Reference))
  (bind _foliageinfo (Variables|Configuration|GetFoliageInfo))
  (bind _foliageinfo_2 (Variables|Configuration|GetFoliageInfo))
  (bind (_busedestructablemesh _foliagedestructiblemeshes _brespawnafterinteractdepletion _timetorespawnafterinteractharvest) (Utilities|Struct|BreakFoliageInformation _foliageinfo))
  (bind _asbp_srpgcharacter (Utilities|Casting|CastToBP_SRPGCharacter (Components|GetOwner Interaction%20Sensor)))
  (LocalVariables|SetInteracting%20Foliage%20Component (Actor|GetComponentbyClass _asbp_srpgcharacter "/Game/SRPG/Blueprints/EnviornmentSystem/BP_PlayerFoliageManager.BP_PlayerFoliageManager_C"))
  (if (> (.MaxNumberOfInteractHarvests (Utilities|Struct|BreakFoliageInformation _foliageinfo_2)) (Variables|HarvestInfo|GetNumber%20of%20Interaction%20Harvests))
    (bind _output_get (LocalVariables|SetRewards%20on%20Harvest (.RewardsOnInteract (Utilities|Struct|BreakFoliageInformation _foliageinfo_2))))
    (CallFunction|ProcessHarvestRewards _output_get (LocalVariables|GetInteracting%20Foliage%20Component))
    (Math|Integer|IncrementInt (Variables|HarvestInfo|GetNumber%20of%20Interaction%20Harvests)
      (:%20%20
        (Variables|HarvestInfo|SetBlock%20Switch%20back%20to%20Instance true)
        (if _brespawnafterinteractdepletion
          (CallFunction|StartRespawnTimer _timetorespawnafterinteractharvest))))
    (else
      (CallFunction|OnFullyDepleated true))))

(fn ManualReturntoInstance
  (if (== (Variables|/Script/Engine.StaticMeshComponent|GetStaticMesh (Variables|References|GetPaired%20Foliage%20Component)) (Variables|Components|GetMyNewStaticMesh))
    (Class|InstancedStaticMeshComponent|AddInstanceWorldSpace (Variables|References|GetPaired%20Foliage%20Component) (Transformation|GetActorTransform))
    (Actor|SetLifeSpan 0.01)
    (else
      (Development|PrintString "Manual return to instance failed due to mismatch of meshes"))))

(fn Initalize
  (bind _outactors (Actor|GetAllActorsOfClass "/Game/SRPG/Blueprints/EnviornmentSystem/BP_FoliageManager.BP_FoliageManager_C"))
  (if (== (Utilities|Array|Length _outactors) 0)
    (Development|PrintString "NO FOLIAGE MANAGER")
    (Variables|References|SetFoliage%20Manager (Utilities|Array|Get(acopy) _outactors)))
  (bind _outactors_2 (Actor|GetAllActorsOfClass "/Script/Foliage.InstancedFoliageActor"))
  (for _array_element (Actor|GetComponentsByClass (Utilities|Array|Get(acopy) _outactors_2) "/Game/SRPG/Blueprints/EnviornmentSystem/BP_CustomFoliageComponent.BP_CustomFoliageComponent_C")
    (if (== (Variables|/Script/Engine.StaticMeshComponent|GetStaticMesh _array_element) (Variables|Components|GetMyNewStaticMesh))
      (Variables|References|SetPaired%20Foliage%20Component _array_element))))

(fn ProcessHarvestRewards
  (params (Harvest%20Rewards :type Array%20of%20Resource%20Reward%20Data%20Structures) (Target :type BP%20Player%20Foliage%20Manager%20Object%20Reference))
  (for _array_element Harvest%20Rewards
    (Default|OnHarvest Target (.ResourceName (Utilities|Struct|BreakResourceRewardData _array_element)) (Math|Random|RandomIntegerinRange (.MinAmount (Utilities|Struct|BreakResourceRewardData _array_element)) (.MaxAmount (Utilities|Struct|BreakResourceRewardData _array_element))))))

(fn OnDamageHarvest
  (params (Damage :type Float%20%28single-precision%29) (Damage%20type :type Damage%20Type%20Object%20Reference) (Damage%20Causer :type Actor%20Object%20Reference))
  (bind _foliageinfo (Variables|Configuration|GetFoliageInfo))
  (bind (_busedestructablemesh _foliagedestructiblemeshes _validdamangetypes _rewardsondamage _mindamageamountforharvest _maxnumberofdamageharvests) (Utilities|Struct|BreakFoliageInformation _foliageinfo))
  (LocalVariables|SetDamage%20Amount Damage)
  (LocalVariables|SetDamageType Damage%20type)
  (LocalVariables|SetDamageCauser Damage%20Causer)
  (bind _asbp_srpgcharacter (Utilities|Casting|CastToBP_SRPGCharacter (LocalVariables|GetDamageCauser))
    (:then
      (LocalVariables|SetEnviornment%20Manager (Actor|GetComponentbyClass _asbp_srpgcharacter "/Game/SRPG/Blueprints/EnviornmentSystem/BP_PlayerFoliageManager.BP_PlayerFoliageManager_C"))
      (if (Utilities|Array|ContainsItem _validdamangetypes (Utilities|GetClass (LocalVariables|GetDamageType)))
        (if (>= (LocalVariables|GetDamage%20Amount) _mindamageamountforharvest)
          (LocalVariables|SetResources%20on%20Harvest _rewardsondamage)
          (if (> _maxnumberofdamageharvests (Variables|HarvestInfo|GetNumber%20of%20Damage%20Harvests))
            (CallFunction|ProcessHarvestRewards (LocalVariables|GetResources%20on%20Harvest) (LocalVariables|GetEnviornment%20Manager))
            (Math|Integer|IncrementInt (Variables|HarvestInfo|GetNumber%20of%20Damage%20Harvests)
              (:%20%20
                (Variables|HarvestInfo|SetBlock%20Switch%20back%20to%20Instance true)
                (return false)))
            (else
              (CallFunction|OnFullyDepleated false)
              (return true)))
          (else
            (Development|PrintString "Not enough damage")))
        (else
          (Development|PrintString "Damage not right type"))))
    (:CastFailed
      (Development|PrintString "Damage Causer Not SRPG")))
  (return false))

(fn AddInteraction
  (bind _foliageinfo (Variables|Configuration|GetFoliageInfo))
  (bind (_busedestructablemesh _foliagedestructiblemeshes _interactionprompt _bshouldoutline) (Utilities|Struct|BreakFoliageInformation _foliageinfo))
  (Utilities|IsValid (Variables|Default|GetInteraction%20Component)
    (:Is%20Not%20Valid
      (bind _returnvalue (Game|AddComponentbyClass "/Game/SRPG/Blueprints/InteractionSystem/BPC_InteractableObjectComponent.BPC_InteractableObjectComponent_C" _bshouldoutline (Utilities|Array|MakeArray _interactionprompt)))
      (Variables|Default|SetInteraction%20Component _returnvalue)
      (return))))

(fn StartRespawnTimer
  (params (Time :type Float%20%28single-precision%29))
  (if (Utilities|Time|IsValidTimerHandle (Variables|HarvestInfo|GetRespawnTimer))
    (Utilities|Time|ClearandInvalidateTimerbyHandle (Variables|HarvestInfo|GetRespawnTimer)))
  (bind _returnvalue (Utilities|Time|SetTimerbyFunctionName self "Manual Return to Instance" Time))
  (Variables|HarvestInfo|SetRespawnTimer _returnvalue)
  (Development|PrintString "Respawn Timer Started"))

(fn DeactivateActor
  (bind _activemeshcomponent (Variables|Default|GetActiveMeshComponent))
  (Physics|SetSimulatePhysics _activemeshcomponent false)
  (Rendering|SetVisibility _activemeshcomponent false false)
  (Collision|SetCollisionEnabled _activemeshcomponent "NoCollision"))

(fn SetMesh
  (bind _foliageinfo (Variables|Configuration|GetFoliageInfo))
  (bind (_folliagemeshes _foliagedestructiblemeshes) (Utilities|Struct|BreakFoliageInformation _foliageinfo))
  (if (Utilities|Struct|BreakFoliageInformation (Variables|Configuration|GetFoliageInfo))
    (bind _returnvalue (Game|AddComponentbyClass "/Script/ApexDestruction.DestructibleComponent" false))
    (bind _output_get (Variables|Default|SetDestructableMesh _returnvalue))
    (Class|DestructibleComponent|SetDestructibleMesh _output_get (Utilities|Array|Get(acopy) _foliagedestructiblemeshes (Utilities|Array|FindItem _folliagemeshes (Variables|Components|GetMyNewStaticMesh))))
    (bind _output_get_2 (Variables|Default|SetActiveMeshComponent (Variables|Default|GetDestructableMesh)))
    (Physics|SetSimulatePhysics _output_get_2 false)
    (Collision|SetCollisionEnabled _output_get_2 "QueryAndPhysics")
    (Components|StaticMesh|SetStaticMesh (Variables|Default|GetStaticMesh) 0)
    (else
      (Components|StaticMesh|SetStaticMesh (Variables|Default|GetStaticMesh) (Variables|Components|GetMyNewStaticMesh))
      (Variables|Default|SetActiveMeshComponent (Variables|Default|GetStaticMesh)))))

(fn ComponentstoSave
  (return 0))