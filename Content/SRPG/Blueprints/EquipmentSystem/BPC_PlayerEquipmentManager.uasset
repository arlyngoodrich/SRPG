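; Player character component that manages equipped armor, attached gear and the active weapon.
; Equipping swaps tagged skeletal meshes or spawns socket-attached actors, and adds inventory containers for items that have one.
; Slot inputs toggle shoulder or hip weapons by spawning a proxy copy at its active socket.
; Attacks route through the server to multicast montages, whose notifies open and close melee damage windows on authority only.
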(event Custom|Client%20Update%20UI
  (Default|CallUpdateUI))

(event Custom|Remove%20Skeletal%20Mesh
  (params (Slot :type EEquipmentSlots%20Enum%20%28by%20ref%29 :default "ESE_None"))
  (bind _meshcomponentmap (Variables|Default|GetMeshComponentMap))
  (bind (_value _returnvalue) (Utilities|Map|Find _meshcomponentmap Slot))
  (if _returnvalue
    (Class|SkinnedMeshComponent|SetSkeletalMesh _value 0 true)))

(event Custom|Multicast%20On%20Primary%20Pressed
  (bind _active_proxy_weapon (Variables|Default|GetActive%20Proxy%20Weapon))
  (bind _primary_animation_montoge (Variables|/Game/SRPG/Blueprints/EquipmentSystem/BP_WeaponBase.BP_WeaponBase_C|GetPrimary%20Animation%20Montoge _active_proxy_weapon))
  (Utilities|IsValid _active_proxy_weapon
    (:Is%20Valid
      (Utilities|IsValid _primary_animation_montoge
        (:Is%20Valid
          (bind _notifyname (Animation|Montage|PlayMontage (Variables|/Script/Engine.Character|GetMesh (Variables|Default|GetOwner)) _primary_animation_montoge)
            (:OnNotifyBegin
              (if (Ability|HasAuthority (Variables|Default|GetOwner))
                (if (Utilities|Name|Equal(Name) _notifyname "StartDamage")
                  (bind _asbp_melee_weapon (Utilities|Casting|CastToBP_MeleeWeapon (Variables|Default|GetActive%20Proxy%20Weapon)))
                  (Default|StartDamage _asbp_melee_weapon)
                  (elif (Utilities|Name|Equal(Name) _notifyname "EndDamage")
                    (bind _asbp_melee_weapon_2 (Utilities|Casting|CastToBP_MeleeWeapon (Variables|Default|GetActive%20Proxy%20Weapon)))
                    (Default|EndDamage _asbp_melee_weapon_2)))))))
        (:Is%20Not%20Valid
          (Development|PrintString "Not valid animation"))))
    (:Is%20Not%20Valid
      (Development|PrintString "Not valid proxy"))))

(event Custom|Multicast%20On%20Secondary%20Pressed
  (bind _active_proxy_weapon (Variables|Default|GetActive%20Proxy%20Weapon))
  (bind _secondary_animation_montoge (Variables|/Game/SRPG/Blueprints/EquipmentSystem/BP_WeaponBase.BP_WeaponBase_C|GetSecondary%20Animation%20Montoge _active_proxy_weapon))
  (Utilities|IsValid _active_proxy_weapon
    (:Is%20Valid
      (Utilities|IsValid _secondary_animation_montoge
        (:Is%20Valid
          (bind _notifyname (Animation|Montage|PlayMontage (Variables|/Script/Engine.Character|GetMesh (Variables|Default|GetOwner)) _secondary_animation_montoge)
            (:OnNotifyBegin
              (if (Ability|HasAuthority (Variables|Default|GetOwner))
                (if (Utilities|Name|Equal(Name) _notifyname "StartDamage")
                  (bind _asbp_melee_weapon (Utilities|Casting|CastToBP_MeleeWeapon (Variables|Default|GetActive%20Proxy%20Weapon)))
                  (Default|StartDamage _asbp_melee_weapon)
                  (elif (Utilities|Name|Equal(Name) _notifyname "EndDamage")
                    (bind _asbp_melee_weapon_2 (Utilities|Casting|CastToBP_MeleeWeapon (Variables|Default|GetActive%20Proxy%20Weapon)))
                    (Default|EndDamage _asbp_melee_weapon_2)))))))
        (:Is%20Not%20Valid
          (Development|PrintString "Not valid animation"))))
    (:Is%20Not%20Valid
      (Development|PrintString "Not valid proxy"))))

(event Custom|On%20Secondary%20Pressed
  (if (Ability|HasAuthority (Variables|Default|GetOwner))
    (CallFunction|MulticastonSecondaryPressed)
    (else
      (CallFunction|ServeronSecondaryPressed))))

(event Custom|Server_OnSecondary%20Pressed
  (if (and (not (Variables|Default|GetbIsAnimationPlayer)) (Variables|Default|GetbIsWeaponEquipped))
    (CallFunction|MulticastonSecondaryPressed)))

(event Custom|Slot%201
  (CallFunction|ActivateSlot "ESE_Shoulder"))

(event Custom|Slot%202
  (CallFunction|ActivateSlot "ESE_LeftHip"))

(event Custom|Slot%203
  (CallFunction|ActivateSlot "ESE_RightHip"))

(event Custom|Activate%20Slot
  (params (Active%20Slot :type EEquipmentSlots%20Enum :default "ESE_None"))
  (CallFunction|SpawnActiveWeapon Active%20Slot))

(event Custom|Primary%20Pressed
  (if (and (not (Variables|Default|GetbIsAnimationPlayer)) (Variables|Default|GetbIsWeaponEquipped))
    (CallFunction|OnPrimaryPressed)))

(event Custom|Secondary%20Pressed
  (if (and (not (Variables|Default|GetbIsAnimationPlayer)) (Variables|Default|GetbIsWeaponEquipped))
    (CallFunction|OnSecondaryPressed)))

(event Custom|On%20Primary%20Pressed
  (if (Ability|HasAuthority (Variables|Default|GetOwner))
    (CallFunction|MulticastonPrimaryPressed)
    (else
      (CallFunction|ServeronPrimaryPressed))))

(event Custom|Server_On%20Primary%20Pressed
  (if (and (not (Variables|Default|GetbIsAnimationPlayer)) (Variables|Default|GetbIsWeaponEquipped))
    (CallFunction|MulticastonPrimaryPressed)))

(event EventOnRepEquipmentSlots
  (Default|CallUpdateUI))

(event EventOnEquipItem
  (params (Slot :type EEquipmentSlots%20Enum :default "ESE_None") (ItemData :type Item%20Data%20Structure))
  (CallFunction|EquipItem Slot ItemData)
  (CallFunction|AddInventory ItemData Slot)
  (CallFunction|ClientUpdateUI)
  (Default|CallUpdateUI))

(event EventOnUnequipItem
  (params (Slot :type EEquipmentSlots%20Enum :default "ESE_None"))
  (CallFunction|UnequipItem Slot)
  (CallFunction|RemoveInventory Slot)
  (CallFunction|ClientUpdateUI)
  (Default|CallUpdateUI))

(event EventBeginPlay
  (bind _owner (Variables|Default|GetOwner))
  (CallFunction|SetMeshMap)
  (EventDispatchers|BindEventtoSlot1 _owner (delegate Custom|Slot%201))
  (EventDispatchers|BindEventtoSlot2 _owner (delegate Custom|Slot%202))
  (EventDispatchers|BindEventtoSlot3 _owner (delegate Custom|Slot%203))
  (EventDispatchers|BindEventtoPrimaryPressed _owner (delegate Custom|Primary%20Pressed))
  (EventDispatchers|BindEventtoSecondaryPressed _owner (delegate Custom|Secondary%20Pressed)))

(event EventSetSkeletalMesh
  (params (TargetSlot :type EEquipmentSlots%20Enum :default "ESE_None") (ItemData :type Item%20Data%20Structure))
  (CallFunction|EquipMesh TargetSlot ItemData))

(fn SetMeshMap
  (bind _meshcomponentmap (Variables|Default|GetMeshComponentMap))
  (Utilities|Map|Clear (Variables|Default|GetMeshComponentMap))
  (bind _asbp_srpgcharacter (Utilities|Casting|CastToBP_SRPGCharacter (Components|GetOwner)))
  (Variables|Default|SetOwner _asbp_srpgcharacter)
  (Utilities|Map|Add _meshcomponentmap "ESE_Head" (Utilities|Array|Get(acopy) (Actor|GetComponentsbyTag _asbp_srpgcharacter "/Script/Engine.SkeletalMeshComponent" "Head")))
  (Utilities|Map|Add _meshcomponentmap "ESE_Hands" (Utilities|Array|Get(acopy) (Actor|GetComponentsbyTag _asbp_srpgcharacter "/Script/Engine.SkeletalMeshComponent" "Hands")))
  (Utilities|Map|Add _meshcomponentmap "ESE_Legs" (Utilities|Array|Get(acopy) (Actor|GetComponentsbyTag _asbp_srpgcharacter "/Script/Engine.SkeletalMeshComponent" "Legs")))
  (Utilities|Map|Add _meshcomponentmap "ESE_Feet" (Utilities|Array|Get(acopy) (Actor|GetComponentsbyTag _asbp_srpgcharacter "/Script/Engine.SkeletalMeshComponent" "Feet")))
  (Utilities|Map|Add _meshcomponentmap "ESE_Torso" (Utilities|Array|Get(acopy) (Actor|GetComponentsbyTag _asbp_srpgcharacter "/Script/Engine.SkeletalMeshComponent" "Torso"))))

(fn EquipItem
  (params (Selection :type EEquipmentSlots%20Enum :default "ESE_None") (Data :type Item%20Data%20Structure))
  (LocalVariables|SetItem%20Data Data)
  (LocalVariables|SetSlot Selection)
  (switch Utilities|FlowControl|Switch|SwitchonEEquipmentSlots (LocalVariables|GetSlot)
    (:ESE_None
      (Development|PrintString "Cannon equip to slot none"))
    (:ESE_Torso
      (Class|PlayerEquipmentManager|CallSetSkeletalMesh (LocalVariables|GetSlot) (LocalVariables|GetItem%20Data) :!label _label))
    (:ESE_Head
      (goto _label))
    (:ESE_Hands
      (goto _label))
    (:ESE_Legs
      (goto _label))
    (:ESE_Feet
      (goto _label))
    (:ESE_Back
      (if (.bIsMesh (Utilities|Struct|BreakItemData (LocalVariables|GetItem%20Data))) :!label _label_2
        (Development|PrintString "Cannot equip mesh to these slots")
        (else
          (bind _returnvalue (Game|SpawnActorfromClass (.InWorldActorClass (Utilities|Struct|BreakItemData (LocalVariables|GetItem%20Data))) (Math|Transform|MakeTransform "0, 0, 0" "0, 0, 0" "1,1,1") "Undefined" (Variables|Default|GetOwner) (LocalVariables|GetItem%20Data) 0))
          (bind _asbp_equipment_base (Utilities|Casting|CastToBP_EquipmentBase _returnvalue)
            (:then
              (bind _output_get (LocalVariables|SetSpawned%20Equipment _asbp_equipment_base))
              (Default|OnEquip _output_get)
              (Transformation|AttachComponentToComponent (LocalVariables|GetSpawned%20Equipment) (Variables|/Script/Engine.Character|GetMesh (Variables|Default|GetOwner)) (Utilities|Select :Index (LocalVariables|GetSlot) :ESE_None "None" :ESE_Torso "None" :ESE_Head "None" :ESE_Hands "None" :ESE_Legs "None" :ESE_Feet "None" :ESE_Back "Back" :ESE_Shoulder "Shoulder" :ESE_LeftHip "LeftHip" :ESE_RightHip "RightHip") "SnapToTarget" "SnapToTarget" "SnapToTarget" true)
              (switch Utilities|FlowControl|Switch|SwitchonEEquipmentSlots (LocalVariables|GetSlot)
                (:ESE_None
                  (Development|PrintString "Unexpected outcome in equipment manager" :!label _label_3))
                (:ESE_Torso
                  (goto _label_3))
                (:ESE_Head
                  (goto _label_3))
                (:ESE_Hands
                  (goto _label_3))
                (:ESE_Legs
                  (goto _label_3))
                (:ESE_Feet
                  (goto _label_3))
                (:ESE_Back
                  (Variables|Default|SetItem%20Attached%20to%20Back (LocalVariables|GetSpawned%20Equipment)))
                (:ESE_Shoulder
                  (bind _asbp_weapon_base (Utilities|Casting|CastToBP_WeaponBase (LocalVariables|GetSpawned%20Equipment))
                    (:then
                      (Variables|Default|SetItem%20Attached%20to%20Shoulder _asbp_weapon_base))
                    (:CastFailed
                      (Development|PrintString "Cannot equip non-weapon to weapon only slots" :!label _label_4))))
                (:ESE_LeftHip
                  (bind _asbp_weapon_base_2 (Utilities|Casting|CastToBP_WeaponBase (LocalVariables|GetSpawned%20Equipment))
                    (:then
                      (Variables|Default|SetItem%20Attached%20to%20LeftHip _asbp_weapon_base_2))
                    (:CastFailed
                      (goto _label_4))))
                (:ESE_RightHip
                  (bind _asbp_weapon_base_3 (Utilities|Casting|CastToBP_WeaponBase (LocalVariables|GetSpawned%20Equipment))
                    (:then
                      (Variables|Default|SetItem%20Attached%20to%20RightHip _asbp_weapon_base_3))
                    (:CastFailed
                      (goto _label_4))))))
            (:CastFailed
              (Development|PrintString "Cannot equip non-equipment base class"))))))
    (:ESE_Shoulder
      (goto _label_2))
    (:ESE_LeftHip
      (goto _label_2))
    (:ESE_RightHip
      (goto _label_2))))

(fn UnequipItem
  (params (TargetSlot :type EEquipmentSlots%20Enum :default "ESE_None"))
  (bind _item_attached_to_back (Variables|Default|GetItem%20Attached%20to%20Back))
  (bind _item_attached_to_shoulder (Variables|Default|GetItem%20Attached%20to%20Shoulder))
  (bind _item_attached_to_lefthip (Variables|Default|GetItem%20Attached%20to%20LeftHip))
  (bind _item_attached_to_righthip (Variables|Default|GetItem%20Attached%20to%20RightHip))
  (bind _returnvalue (Utilities|Select :Index TargetSlot :ESE_None 0 :ESE_Torso 0 :ESE_Head 0 :ESE_Hands 0 :ESE_Legs 0 :ESE_Feet 0 :ESE_Back _item_attached_to_back :ESE_Shoulder _item_attached_to_shoulder :ESE_LeftHip _item_attached_to_lefthip :ESE_RightHip _item_attached_to_righthip))
  (switch Utilities|FlowControl|Switch|SwitchonEEquipmentSlots TargetSlot
    (:ESE_None
      (Development|PrintString "Canno unequip from slot \"none\""))
    (:ESE_Torso
      (CallFunction|RemoveSkeletalMesh TargetSlot :!label _label))
    (:ESE_Head
      (goto _label))
    (:ESE_Hands
      (goto _label))
    (:ESE_Legs
      (goto _label))
    (:ESE_Feet
      (goto _label))
    (:ESE_Back
      (Utilities|IsValid _returnvalue :!label _label_2
        (:Is%20Valid
          (LocalVariables|SetActor%20to%20Remove _returnvalue)
          (Actor|SetLifeSpan (LocalVariables|GetActor%20to%20Remove) 0.01))
        (:Is%20Not%20Valid
          (Development|PrintString "Cannot unequip, not valid actor reference"))))
    (:ESE_Shoulder
      (goto _label_2))
    (:ESE_LeftHip
      (goto _label_2))
    (:ESE_RightHip
      (goto _label_2))))

(fn EquipMesh
  (params (Key :type EEquipmentSlots%20Enum%20%28by%20ref%29 :default "ESE_None") (ItemData :type Item%20Data%20Structure%20%28by%20ref%29))
  (bind (_itemtype _bismesh _skeletalmesh) (Utilities|Struct|BreakItemData ItemData))
  (bind _meshcomponentmap (Variables|Default|GetMeshComponentMap))
  (bind (_value _returnvalue) (Utilities|Map|Find _meshcomponentmap Key))
  (if (Math|Boolean|ANDBoolean _returnvalue _bismesh (Utilities|IsValid _skeletalmesh))
    (Class|SkinnedMeshComponent|SetSkeletalMesh _value _skeletalmesh true)
    (else
      (Development|PrintString "Could not equipment mesh"))))

(fn AddInventory
  (params (Item%20Data :type Item%20Data%20Structure) (EquippedSlot :type EEquipmentSlots%20Enum :default "ESE_None"))
  (bind (_itemtype _bhasinventory _inventoryname _inventorysizex _inventorysizey _maxweight) (Utilities|Struct|BreakItemData Item%20Data))
  (bind _abstractinventory (Utilities|Struct|BreakItemData Item%20Data))
  (if _bhasinventory
    (bind _returnvalue (Game|AddComponentbyClass (Variables|Default|GetOwner) "/Game/SRPG/Blueprints/InventorySystem/BPC_InventoryContainer.BPC_InventoryContainer_C" EquippedSlot _inventoryname _inventorysizex _inventorysizey _maxweight))
    (bind _output_get (LocalVariables|SetAdded%20Inventory _returnvalue))
    (Default|CallInvetoryAdded _output_get)
    (Utilities|IsValid _abstractinventory
      (:Is%20Valid
        (bind (_outinventory _outabstractinventorypairid) (Class|AbstractInventoryContainer|GetInventory _abstractinventory))
        (Class|InventoryContainer|SetInventoryfromAbstract (LocalVariables|GetAdded%20Inventory) _outinventory _outabstractinventorypairid))
      (:Is%20Not%20Valid
        (Development|PrintString "No Valid Abstract Inventory")))))

(fn RemoveInventory
  (params (EquipmentSlot :type EEquipmentSlots%20Enum :default "ESE_None"))
  (bind (_outpairedinventory _returnvalue) (Class|PlayerEquipmentManager|FindPairedInventory EquipmentSlot))
  (if _returnvalue
    (bind _asbpc_inventory_container (Utilities|Casting|CastToBPC_InventoryContainer _outpairedinventory))
    (Default|CallInventoryRemoved _asbpc_inventory_container)
    (Default|ExternalDestroyComponent _asbpc_inventory_container)
    (else
      (Development|PrintString "No paired inventory found"))))

(fn SpawnActiveWeapon
  (params (Selection :type EEquipmentSlots%20Enum :default "ESE_None"))
  (bind _owner (Variables|Default|GetOwner))
  (bind _item_attached_to_lefthip (Variables|Default|GetItem%20Attached%20to%20LeftHip))
  (bind _item_attached_to_righthip (Variables|Default|GetItem%20Attached%20to%20RightHip))
  (bind _item_attached_to_shoulder (Variables|Default|GetItem%20Attached%20to%20Shoulder))
  (bind _returnvalue (Utilities|Select :Index Selection :ESE_None 0 :ESE_Torso 0 :ESE_Head 0 :ESE_Hands 0 :ESE_Legs 0 :ESE_Feet 0 :ESE_Back 0 :ESE_Shoulder _item_attached_to_shoulder :ESE_LeftHip _item_attached_to_lefthip :ESE_RightHip _item_attached_to_righthip))
  (if (Utilities|Enum|Equal(Enum) (Variables|Default|GetActive%20Slot) Selection)
    (CallFunction|DeactivateSpawnedWeapon)
    (Variables|Default|SetbIsWeaponEquipped false)
    (else
      (CallFunction|DeactivateSpawnedWeapon)
      (Variables|Default|SetActive%20Slot Selection)
      (Utilities|IsValid _returnvalue
        (:Is%20Valid
          (bind _output_get (Variables|Default|SetActive%20Equipped%20Weapon _returnvalue))
          (Default|OnActivatedasEquipped _output_get)
          (bind _asbp_weapon_base (Utilities|Casting|CastToBP_WeaponBaseClass (Utilities|GetClass (Variables|Default|GetActive%20Equipped%20Weapon))))
          (bind _returnvalue_2 (Game|SpawnActorfromClass _asbp_weapon_base (Math|Transform|MakeTransform "0, 0, 0" "0, 0, 0" "1,1,1") "Undefined" _owner false false (Variables|/Script/SRPG.ItemBase|GetItemData (Variables|Default|GetActive%20Equipped%20Weapon)) _owner))
          (Default|OnActivatedasWeapon _returnvalue_2)
          (bind _output_get_2 (Variables|Default|SetActive%20Proxy%20Weapon _returnvalue_2))
          (Actor|SetOwner _output_get_2 (Variables|Default|GetOwner))
          (Transformation|AttachComponentToComponent _returnvalue_2 (Variables|/Script/Engine.Character|GetMesh (Variables|Default|GetOwner)) (Variables|/Game/SRPG/Blueprints/EquipmentSystem/BP_WeaponBase.BP_WeaponBase_C|GetActivated%20Slot _returnvalue_2) "SnapToTarget" "SnapToTarget" "SnapToTarget" true)
          (Default|OnActivatedasEquipped (Variables|Default|GetActive%20Equipped%20Weapon))
          (Variables|Default|SetbIsWeaponEquipped true))
        (:Is%20Not%20Valid
          (Development|PrintString "No valid weapon in slot"))))))

(fn DeactivateSpawnedWeapon
  (Utilities|IsValid (Variables|Default|GetActive%20Equipped%20Weapon)
    (:Is%20Valid
      (Default|OnDeactivatedasEquipped (Variables|Default|GetActive%20Equipped%20Weapon))
      (Utilities|IsValid (Variables|Default|GetActive%20Proxy%20Weapon)
        (:Is%20Valid
          (Default|OnDeactivatedasWeapon (Variables|Default|GetActive%20Proxy%20Weapon)))
        (:Is%20Not%20Valid
          _)))
    (:Is%20Not%20Valid
      _))
  (Variables|Default|SetActive%20Equipped%20Weapon 0)
  (Variables|Default|SetActive%20Proxy%20Weapon 0)
  (Variables|Default|SetActive%20Slot "ESE_None"))