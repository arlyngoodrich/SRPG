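; BP_WeaponBase is a weapon base actor in the SRPG equipment system that responds to activation and deactivation in two roles, equipped and weapon.
; Activating as equipped hides its static mesh, and deactivating as equipped shows it again, without propagating to child components.
; Activating as weapon calls OnEquip, which is not defined in this graph, and deactivating as weapon destroys the actor.
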(event Custom|On%20Activated%20as%20Equipped
  (Rendering|SetVisibility (Variables|Default|GetStaticMesh) false false))

(event Custom|On%20Deactivated%20as%20Equipped
  (Rendering|SetVisibility (Variables|Default|GetStaticMesh) true false))

(event Custom|On%20Activated%20as%20Weapon
  (CallFunction|OnEquip))

(event Custom|On%20Deactivated%20as%20Weapon
  (Actor|DestroyActor))

(event EventBeginPlay
  (|CallParentFunction) ; This node is disabled and will not be called.\nDrag off pins to build functionality.
)

(fn ConstructionScript
  (|CallParentFunction))