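; BP_WearableBase is a base Blueprint for wearable equipment that can also act as an openable storage container.
; On BeginPlay, the authority adds an "Open Inventory" prompt to the interactable component when a valid InventoryContainer exists.
; The first interaction is passed to the parent class, while any other index toggles the container's storage for the owner of the interacting sensor.
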(event EventBeginPlay
  (|CallParentFunction)
  (Networking|SwitchHasAuthority
    (:Authority
      (Utilities|IsValid (Variables|Default|GetInventoryContainer)
        (:Is%20Valid
          (Utilities|Array|Add (Variables|/Game/SRPG/Blueprints/InteractionSystem/BPC_InteractableObjectComponent.BPC_InteractableObjectComponent_C|GetInteraction%20Prompt (Variables|Default|GetBPC_InteractableObjectComponent)) "Open Inventory"))))))

(event EventOnInteractionTriggered
  (params (Player%20Interaction%20Sensor :type BPC%20Player%20Interaction%20Sensor%20Object%20Reference) (Interaction%20Index :type Integer))
  (bind _inventorycontainer (Variables|Default|GetInventoryContainer))
  (if (== Interaction%20Index 0)
    (|CallParentFunction Player%20Interaction%20Sensor Interaction%20Index)
    (else
      (Utilities|IsValid _inventorycontainer
        (:Is%20Valid
          (Default|CallToggleStroage _inventorycontainer (Components|GetOwner Player%20Interaction%20Sensor)))))))

(fn ConstructionScript
  (|CallParentFunction))