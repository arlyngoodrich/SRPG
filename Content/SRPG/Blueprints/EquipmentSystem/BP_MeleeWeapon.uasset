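; Melee weapon base that deals point damage through traces during a toggled damage window.
; On BeginPlay it gathers its BP_MeleeDamageTrace child actors.
; While StartDamage has the window open, the server runs each trace on Tick, ignoring itself and its owner.
; The first valid hit closes the window and applies damage with the owner as causer.
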(event Custom|Start%20Damage
  (Variables|Default|SetbCheckforDamage true))

(event Custom|End%20Damage
  (Variables|Default|SetbCheckforDamage false))

(event Custom|On%20Valid%20Hit
  (params (Hit :type Hit%20Result%20Structure))
  (bind (_bblockinghit _binitialoverlap _time _distance _location _impactpoint _normal _impactnormal _physmat _hitactor) (Collision|BreakHitResult Hit))
  (CallFunction|EndDamage)
  (Development|PrintString "Hit" true true "(R=0.000000,G=0.660000,B=1.000000,A=1.000000)" 0.5)
  (Game|Damage|ApplyPointDamage _hitactor (Variables|DamageSettings|GetBase%20Damage) _normal Hit 0 (Components|GetOwner) (Variables|DamageSettings|GetDamage%20Type)))

(event EventTick
  (params (DeltaSeconds :type Float%20%28single-precision%29))
  (Networking|SwitchHasAuthority
    (:Authority
      (if (Variables|Default|GetbCheckforDamage)
        (CallFunction|CheckforDamage)))))

(event EventBeginPlay
  (|CallParentFunction)
  (for _array_element (Actor|GetAllChildActors true)
    (bind _asbp_melee_damage_trace (Utilities|Casting|CastToBP_MeleeDamageTrace _array_element))
    (Utilities|Array|Add (Variables|Internal|GetDamage%20Traces) _asbp_melee_damage_trace)))

(fn ConstructionScript)

(fn CheckforDamage
  (for _array_element (Variables|Internal|GetDamage%20Traces)
    (if (not (LocalVariables|GetValid%20Hit))
      (bind (_outhit _returnvalue) (Default|PerformTrace _array_element (Variables|TraceSettings|GetTrace%20Channel) (Variables|TraceSettings|GetTrace%20Complex) (Utilities|Array|MakeArray self (Components|GetOwner)) (Variables|TraceSettings|GetDraw%20Debug%20Type) (Variables|TraceSettings|GetDraw%20Time) (Variables|TraceSettings|GetTrace%20Color) (Variables|TraceSettings|GetTrace%20Hit%20Color)))
      (bind _output_get (LocalVariables|SetValid%20Hit _returnvalue))
      (if _output_get
        (CallFunction|OnValidHit _outhit)
        (return)))))