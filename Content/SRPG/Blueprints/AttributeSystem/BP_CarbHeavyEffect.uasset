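; BP_CarbHeavyEffect is an attribute effect that modifies the player's stamina regeneration while a metabolic balance state lasts.
; On trigger it casts its target to the stamina component and its spawner to the metabolism component, then applies the regen modifier.
; A one-second timer delays binding to metabolism balance changes.
; The next balance change of any type reverses the modifier, unbinds and checks the effect out of the attribute.
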(event Custom|On%20Metabolic%20Blanace%20Change
  (params (NewMetabolisimBalanceType :type EMetabolicBalanceType%20Enum :default "EMBT_None"))
  (Class|StaminaAttribute|ModifyStaminaReGen (Variables|References|GetStamina%20Attribute) (* -1 (Variables|Default|GetReGen%20Modify%20Amount)))
  (EventDispatchers|UnbindEventfromMetabolismonBalanceChange (Variables|References|GetMetabolism%20Attribute) (delegate Custom|On%20Metabolic%20Blanace%20Change))
  (Class|AttributeEffect|CheckOutEffectfromAttribute))

(event Custom|Bind%20to%20Metabolism%20Update
  (EventDispatchers|BindEventtoMetabolismonBalanceChange (Variables|References|GetMetabolism%20Attribute) (delegate Custom|On%20Metabolic%20Blanace%20Change)))

(event EventOnEffectTriggered
  (bind _asbpc_player_stamina_component (Utilities|Casting|CastToBPC_PlayerStaminaComponent (Variables|Default|GetTargetAttributeComponent)))
  (Variables|References|SetStamina%20Attribute _asbpc_player_stamina_component)
  (bind _asbpc_player_metabolism_component (Utilities|Casting|CastToBPC_PlayerMetabolismComponent (Variables|Default|GetSpawningAttributeComponent)))
  (Variables|References|SetMetabolism%20Attribute _asbpc_player_metabolism_component)
  (Class|StaminaAttribute|ModifyStaminaReGen (Variables|References|GetStamina%20Attribute) (Variables|Default|GetReGen%20Modify%20Amount))
  (Utilities|Time|SetTimerbyEvent (delegate Custom|Bind%20to%20Metabolism%20Update) 1.0))