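; Attribute effect for a vitamin-heavy metabolism state that modifies the player's health regeneration while it is active.
; On trigger it applies the regen modifier to the target health component and, after a one-second timer, binds to the spawning metabolism component's balance-change event.
; The next balance change, whatever the new type, reverses the modifier, unbinds and checks the effect out of the attribute.
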(event Custom|On%20Metabolic%20Blanace%20Change
  (params (NewMetabolisimBalanceType :type EMetabolicBalanceType%20Enum :default "EMBT_None"))
  (Class|HealthAttribute|ModifyHealthReGenAmount (Variables|Default|GetHealth%20Attribute) (* -1 (Variables|Default|GetRegen%20Modify%20Amount)))
  (EventDispatchers|UnbindEventfromMetabolismonBalanceChange (Variables|Default|GetMetabolism%20Attribute) (delegate Custom|On%20Metabolic%20Blanace%20Change))
  (Class|AttributeEffect|CheckOutEffectfromAttribute))

(event Custom|Bind%20to%20Metabolism%20Update
  (EventDispatchers|BindEventtoMetabolismonBalanceChange (Variables|Default|GetMetabolism%20Attribute) (delegate Custom|On%20Metabolic%20Blanace%20Change)))

(event EventOnEffectTriggered
  (bind _asbpc_player_health_component (Utilities|Casting|CastToBPC_PlayerHealthComponent (Variables|Default|GetTargetAttributeComponent)))
  (Variables|Default|SetHealth%20Attribute _asbpc_player_health_component)
  (bind _asbpc_player_metabolism_component (Utilities|Casting|CastToBPC_PlayerMetabolismComponent (Variables|Default|GetSpawningAttributeComponent)))
  (Variables|Default|SetMetabolism%20Attribute _asbpc_player_metabolism_component)
  (Class|HealthAttribute|ModifyHealthReGenAmount (Variables|Default|GetHealth%20Attribute) (Variables|Default|GetRegen%20Modify%20Amount))
  (Utilities|Time|SetTimerbyEvent (delegate Custom|Bind%20to%20Metabolism%20Update) 1.0))