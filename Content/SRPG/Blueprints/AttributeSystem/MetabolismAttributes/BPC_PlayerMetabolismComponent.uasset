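; Player metabolism component that turns changes in metabolic balance into attribute effects on the owning character.
; On BeginPlay it caches the owner's stamina and health components.
; On authority, a balance update constructs an effect object, with Carb Heavy and Protein Heavy targeting stamina and Vitamin Heavy targeting health.
; UI events add or remove effect icons on both the SRPG character's HUD and character menu.
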(event EventRemoveEffectfromUI
  (params (EffectName :type Name :default "None"))
  (bind _asbp_srpgcharacter (Utilities|Casting|CastToBP_SRPGCharacter (Components|GetOwner)))
  (Default|RemoveEffect (Variables|/Game/SRPG/Blueprints/CharacterAssets/BP_SRPGCharacter.BP_SRPGCharacter_C|GetPlayer%20HUD _asbp_srpgcharacter) EffectName)
  (Default|RemoveEffect (Variables|/Game/SRPG/Blueprints/MenuSystem/CharacterMenu/WBP_PlayerMenuContainer.WBP_PlayerMenuContainer_C|GetWBP_CharacterMenuContainer (Variables|/Game/SRPG/Blueprints/CharacterAssets/BP_SRPGCharacter.BP_SRPGCharacter_C|GetPlayer%20Menu%20Widget _asbp_srpgcharacter)) EffectName))

(event EventOnMetabolicBalanceUpdate
  (params (NewBalance :type EMetabolicBalanceType%20Enum :default "EMBT_None"))
  (bind _self self)
  (bind _self_2 self)
  (bind _self_3 self)
  (if (Ability|HasAuthority (Components|GetOwner))
    (switch Utilities|FlowControl|Switch|SwitchonEMetabolicBalanceType NewBalance
      (:EMBT_Carbs
        (bind _returnvalue (Game|ConstructObjectfromClass "/Game/SRPG/Blueprints/AttributeSystem/MetabolismAttributes/BP_CarbHeavyEffect.BP_CarbHeavyEffect_C" _self_2))
        (Class|AttributeEffect|InitalizeEffect _returnvalue _self_2 (Variables|Default|GetStamina%20Component)))
      (:EMBT_Protein
        (bind _returnvalue_2 (Game|ConstructObjectfromClass "/Game/SRPG/Blueprints/AttributeSystem/MetabolismAttributes/BP_ProteinHeavyEffect.BP_ProteinHeavyEffect_C" _self_3))
        (Class|AttributeEffect|InitalizeEffect _returnvalue_2 _self_3 (Variables|Default|GetStamina%20Component)))
      (:EMBT_Vitamins
        (bind _returnvalue_3 (Game|ConstructObjectfromClass "/Game/SRPG/Blueprints/AttributeSystem/MetabolismAttributes/BP_VitaminHeavyEffect.BP_VitaminHeavyEffect_C" _self))
        (Class|AttributeEffect|InitalizeEffect _returnvalue_3 _self (Variables|Default|GetHealth%20Component))))))

(event EventBeginPlay
  (bind _returnvalue (Components|GetOwner))
  (bind _returnvalue_2 (Components|GetOwner))
  (bind _returnvalue_3 (Actor|GetComponentbyClass _returnvalue "/Game/SRPG/Blueprints/AttributeSystem/HealthAttributes/BPC_PlayerHealthComponent.BPC_PlayerHealthComponent_C"))
  (bind _returnvalue_4 (Actor|GetComponentbyClass _returnvalue_2 "/Game/SRPG/Blueprints/AttributeSystem/StaminaAttributes/BPC_PlayerStaminaComponent.BPC_PlayerStaminaComponent_C"))
  (Utilities|IsValid _returnvalue_4
    (:Is%20Valid
      (Variables|Default|SetStamina%20Component _returnvalue_4)
      (Utilities|IsValid _returnvalue_3
        (:Is%20Valid
          (Variables|Default|SetHealth%20Component _returnvalue_3))
        (:Is%20Not%20Valid
          (Development|PrintString "No Valid Health  Component"))))
    (:Is%20Not%20Valid
      (Development|PrintString "No Valid Stamina Component"))))

(event EventAddEffecttoUI
  (params (IconTexutre :type Texture%202D%20Object%20Reference) (IconColor :type Color%20Structure) (BackgroundColor :type Color%20Structure) (EffectName :type Name :default "None") (Discription :type Text%20%28by%20ref%29))
  (bind _returnvalue (Math|Conversions|ToLinearColor(Color) IconColor))
  (bind _returnvalue_2 (Math|Conversions|ToLinearColor(Color) BackgroundColor))
  (bind _asbp_srpgcharacter (Utilities|Casting|CastToBP_SRPGCharacter (Components|GetOwner)))
  (Default|AddEffect (Variables|/Game/SRPG/Blueprints/CharacterAssets/BP_SRPGCharacter.BP_SRPGCharacter_C|GetPlayer%20HUD _asbp_srpgcharacter) _returnvalue_2 _returnvalue IconTexutre EffectName Discription)
  (Default|AddEffect (Variables|/Game/SRPG/Blueprints/MenuSystem/CharacterMenu/WBP_PlayerMenuContainer.WBP_PlayerMenuContainer_C|GetWBP_CharacterMenuContainer (Variables|/Game/SRPG/Blueprints/CharacterAssets/BP_SRPGCharacter.BP_SRPGCharacter_C|GetPlayer%20Menu%20Widget _asbp_srpgcharacter)) _returnvalue_2 _returnvalue IconTexutre EffectName Discription))