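; Player stamina component for the SRPG character that shows and clears stamina-related effects in the player's UI.
; Its add and remove events cast the owner to BP_SRPGCharacter, then forward to both the HUD and the character menu container.
; Added effects carry an icon, colors, name and description, while removal uses only the effect name.
; The component holds no stamina logic in its event graph, only this UI bridge.
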(event EventRemoveEffectfromUI
  (params (EffectName :type Name :default "None"))
  (bind _asbp_srpgcharacter (Utilities|Casting|CastToBP_SRPGCharacter (Components|GetOwner)))
  (Default|RemoveEffect (Variables|/Game/SRPG/Blueprints/CharacterAssets/BP_SRPGCharacter.BP_SRPGCharacter_C|GetPlayer%20HUD _asbp_srpgcharacter) EffectName)
  (Default|RemoveEffect (Variables|/Game/SRPG/Blueprints/MenuSystem/CharacterMenu/WBP_PlayerMenuContainer.WBP_PlayerMenuContainer_C|GetWBP_CharacterMenuContainer (Variables|/Game/SRPG/Blueprints/CharacterAssets/BP_SRPGCharacter.BP_SRPGCharacter_C|GetPlayer%20Menu%20Widget _asbp_srpgcharacter)) EffectName))

(event EventAddEffecttoUI
  (params (IconTexutre :type Texture%202D%20Object%20Reference) (IconColor :type Color%20Structure) (BackgroundColor :type Color%20Structure) (EffectName :type Name :default "None") (Discription :type Text%20%28by%20ref%29))
  (bind _returnvalue (Math|Conversions|ToLinearColor(Color) IconColor))
  (bind _returnvalue_2 (Math|Conversions|ToLinearColor(Color) BackgroundColor))
  (bind _asbp_srpgcharacter (Utilities|Casting|CastToBP_SRPGCharacter (Components|GetOwner)))
  (Default|AddEffect (Variables|/Game/SRPG/Blueprints/CharacterAssets/BP_SRPGCharacter.BP_SRPGCharacter_C|GetPlayer%20HUD _asbp_srpgcharacter) _returnvalue_2 _returnvalue IconTexutre EffectName Discription)
  (Default|AddEffect (Variables|/Game/SRPG/Blueprints/MenuSystem/CharacterMenu/WBP_PlayerMenuContainer.WBP_PlayerMenuContainer_C|GetWBP_CharacterMenuContainer (Variables|/Game/SRPG/Blueprints/CharacterAssets/BP_SRPGCharacter.BP_SRPGCharacter_C|GetPlayer%20Menu%20Widget _asbp_srpgcharacter)) _returnvalue_2 _returnvalue IconTexutre EffectName Discription))