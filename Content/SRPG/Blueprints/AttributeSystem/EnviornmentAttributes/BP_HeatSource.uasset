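; BP_HeatSource is a placeable environmental heat emitter that adds warmth to SRPG characters within its range.
; A sphere zone, sized to EmissionRange in the construction script, registers or unregisters the source with each overlapping character's environmental component.
; GetHeat scales MaxHeatAdded by a falloff curve sampled at distance normalized by the emission range.
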(event OnComponentBeginOverlap(MaxEmissionZone)
  (params (OverlappedComponent :type Primitive%20Component%20Object%20Reference) (OtherActor :type Actor%20Object%20Reference) (OtherComp :type Primitive%20Component%20Object%20Reference) (OtherBodyIndex :type Integer) (bFromSweep :type Boolean) (SweepResult :type Hit%20Result%20Structure%20%28by%20ref%29))
  (bind _asbp_srpgcharacter (Utilities|Casting|CastToBP_SRPGCharacter OtherActor))
  (Default|CheckinHeatSource (Variables|/Game/SRPG/Blueprints/CharacterAssets/BP_SRPGCharacter.BP_SRPGCharacter_C|GetBPC_PlayerEnviornmentalComponent _asbp_srpgcharacter) self))

(event OnComponentEndOverlap(MaxEmissionZone)
  (params (OverlappedComponent :type Primitive%20Component%20Object%20Reference) (OtherActor :type Actor%20Object%20Reference) (OtherComp :type Primitive%20Component%20Object%20Reference) (OtherBodyIndex :type Integer))
  (bind _asbp_srpgcharacter (Utilities|Casting|CastToBP_SRPGCharacter OtherActor))
  (Default|CheckOutHeatSource (Variables|/Game/SRPG/Blueprints/CharacterAssets/BP_SRPGCharacter.BP_SRPGCharacter_C|GetBPC_PlayerEnviornmentalComponent _asbp_srpgcharacter) self))

(fn ConstructionScript
  (Components|Sphere|SetSphereRadius (Variables|Default|GetMaxEmissionZone) (Variables|Congif|GetEmissionRange) true))

(fn GetHeat
  (params (Distance :type Float%20%28single-precision%29))
  (return (* (Math|Curves|GetFloatValue (Variables|Congif|GetHeat%20Falloff%20Curve) (/ Distance (Variables|Congif|GetEmissionRange))) (Variables|Congif|GetMax%20Heat%20Added))))