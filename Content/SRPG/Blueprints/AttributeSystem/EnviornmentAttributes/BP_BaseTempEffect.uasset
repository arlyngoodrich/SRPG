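; Base attribute effect for temperature states from the player environmental component, with empty start and end functions as hooks for child effects.
; On trigger it casts the spawning attribute component to that component, starts the effect, and binds to temperature state changes after a short timer delay.
; The next state change ends the effect, checks it out of the target attribute component and unbinds the listener.
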(event Custom|Bind%20to%20Temp%20State%20Change
  (EventDispatchers|BindEventtoTemponStateChange (Variables|Default|GetEnviornmental%20Component) (delegate Custom|On%20Temp%20State%20Change)))

(event Custom|On%20Temp%20State%20Change
  (params (NewTempState :type ETemperatureState%20Enum :default "ETS_Freezing"))
  (CallFunction|EndEffect)
  (Class|BaseAttributeComponent|CheckOutEffect (Variables|Default|GetTargetAttributeComponent) self)
  (EventDispatchers|UnbindEventfromTemponStateChange (Variables|Default|GetEnviornmental%20Component) (delegate Custom|On%20Temp%20State%20Change)))

(event EventOnEffectTriggered
  (bind _asbpc_player_enviornmental_component (Utilities|Casting|CastToBPC_PlayerEnviornmentalComponent (Variables|Default|GetSpawningAttributeComponent)))
  (Variables|Default|SetEnviornmental%20Component _asbpc_player_enviornmental_component)
  (Utilities|Time|SetTimerbyEvent (delegate Custom|Bind%20to%20Temp%20State%20Change) 0.1)
  (CallFunction|StartInitalEffect))

(fn StartInitalEffect)

(fn EndEffect)