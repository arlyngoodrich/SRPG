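; BP_HotEffect is an environment attribute effect that alters water decay in the player's metabolism while it is active.
; On start, it runs the parent logic, casts the target attribute component to BPC_PlayerMetabolismComponent and passes WaterDecayMod to ModifyDecayAmounts.
; On end, it makes the same call with the negated value to undo the change.
; Targets without that metabolism component receive only the parent behavior.
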(fn StartInitalEffect
  (|CallParentFunction)
  (bind _asbpc_player_metabolism_component (Utilities|Casting|CastToBPC_PlayerMetabolismComponent (Variables|Default|GetTargetAttributeComponent)))
  (Class|MetabolismAttribute|ModifyDecayAmounts _asbpc_player_metabolism_component 0.0 0.0 0.0 (Variables|MetabolismEffect|GetWater%20Decay%20Mod)))

(fn EndEffect
  (|CallParentFunction)
  (bind _asbpc_player_metabolism_component (Utilities|Casting|CastToBPC_PlayerMetabolismComponent (Variables|Default|GetTargetAttributeComponent)))
  (Class|MetabolismAttribute|ModifyDecayAmounts _asbpc_player_metabolism_component 0.0 0.0 0.0 (* -1 (Variables|MetabolismEffect|GetWater%20Decay%20Mod))))