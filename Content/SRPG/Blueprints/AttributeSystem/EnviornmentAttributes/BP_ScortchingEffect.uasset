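; BP_ScortchingEffect is an environment attribute effect that alters a character's stamina regeneration while it is active.
; On start, it casts the spawning attribute component's owner to BP_SRPGCharacter, caches its stamina component and applies ModifyAmount to regen.
; On end, it applies the negated amount to undo the change.
; Both overrides call their parent implementations first.
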(fn StartInitalEffect
  (|CallParentFunction)
  (bind _asbp_srpgcharacter (Utilities|Casting|CastToBP_SRPGCharacter (Components|GetOwner (Variables|Default|GetSpawningAttributeComponent))))
  (bind _output_get (Variables|Default|SetStamina%20Component (Variables|/Game/SRPG/Blueprints/CharacterAssets/BP_SRPGCharacter.BP_SRPGCharacter_C|GetBPC_StaminaComponent _asbp_srpgcharacter)))
  (Class|StaminaAttribute|ModifyStaminaReGen _output_get (Variables|Default|GetModify%20Amount)))

(fn EndEffect
  (|CallParentFunction)
  (Class|StaminaAttribute|ModifyStaminaReGen (Variables|Default|GetStamina%20Component) (* -1 (Variables|Default|GetModify%20Amount))))