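; BP_ShelterEffect is an attribute-system effect that responds to changes in the player's shelter state.
; When triggered, it casts its spawning attribute component to BPC_PlayerEnviornmentalComponent and caches it, then waits on a short one-shot timer before binding to that component's shelter update.
; Each update passes the effect to CheckOutEffect on the target attribute component, without reading the new shelter value itself.
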(event Custom|Bind%20to%20Shelter%20Update
  (EventDispatchers|BindEventtoOnShelterUpdate (Variables|Default|GetAs%20BPC%20Player%20Enviornmental%20Component) (delegate Custom|On%20Shelter%20Update)))

(event Custom|On%20Shelter%20Update
  (params (New%20In%20Shelter :type Boolean))
  (Class|BaseAttributeComponent|CheckOutEffect (Variables|Default|GetTargetAttributeComponent) self))

(event EventOnEffectTriggered
  (bind _asbpc_player_enviornmental_component (Utilities|Casting|CastToBPC_PlayerEnviornmentalComponent (Variables|Default|GetSpawningAttributeComponent)))
  (Variables|Default|SetAs%20BPC%20Player%20Enviornmental%20Component _asbpc_player_enviornmental_component)
  (Utilities|Time|SetTimerbyEvent (delegate Custom|Bind%20to%20Shelter%20Update) 0.1))