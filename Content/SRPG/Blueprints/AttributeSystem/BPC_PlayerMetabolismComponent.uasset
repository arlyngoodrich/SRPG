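; Player metabolism component that turns changes in metabolic balance into effects on other player attributes.
; On BeginPlay it caches the owner's stamina and health components, printing an error if one is missing.
; When the balance updates, the authority constructs an effect object: carb-heavy targets stamina, vitamin-heavy targets health.
; Each effect is initialized with this component as its source.
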(event EventOnMetabolicBalanceUpdate
  (params (NewBalance :type EMetabolicBalanceType%20Enum :default "EMBT_None"))
  (bind _self self)
  (bind _self_2 self)
  (if (Ability|HasAuthority (Components|GetOwner))
    (switch Utilities|FlowControl|Switch|SwitchonEMetabolicBalanceType NewBalance
      (:EMBT_Carbs
        (bind _returnvalue (Game|ConstructObjectfromClass "/Game/SRPG/Blueprints/AttributeSystem/BP_CarbHeavyEffect.BP_CarbHeavyEffect_C" _self_2))
        (Class|AttributeEffect|InitalizeEffect _returnvalue _self_2 (Variables|Default|GetStamina%20Component)))
      (:EMBT_Vitamins
        (bind _returnvalue_2 (Game|ConstructObjectfromClass "/Game/SRPG/Blueprints/AttributeSystem/BP_VitaminHeavyEffect.BP_VitaminHeavyEffect_C" _self))
        (Class|AttributeEffect|InitalizeEffect _returnvalue_2 _self (Variables|Default|GetHealth%20Component))))))

(event EventBeginPlay
  (bind _returnvalue (Components|GetOwner))
  (bind _returnvalue_2 (Components|GetOwner))
  (bind _returnvalue_3 (Actor|GetComponentbyClass _returnvalue "/Game/SRPG/Blueprints/AttributeSystem/BPC_PlayerHealthComponent.BPC_PlayerHealthComponent_C"))
  (bind _returnvalue_4 (Actor|GetComponentbyClass _returnvalue_2 "/Game/SRPG/Blueprints/AttributeSystem/BPC_PlayerStaminaComponent.BPC_PlayerStaminaComponent_C"))
  (Utilities|IsValid _returnvalue_4
    (:Is%20Valid
      (Variables|Default|SetStamina%20Component _returnvalue_4)
      (Utilities|IsValid _returnvalue_3
        (:Is%20Valid
          (Variables|Default|SetHealth%20Component _returnvalue_3))
        (:Is%20Not%20Valid
          (Development|PrintString "No Valid Health  Component"))))
    (:Is%20Not%20Valid
      (Development|PrintString "No Valid Stamina Component"))))