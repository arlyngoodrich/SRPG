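; Player environmental component that, on the server, feeds temperature and wetness samples from Ultra Dynamic Weather into SampleEnviornment.
; A looping timer, plus swim status changes, triggers sampling; wetness comes from weather type plus swimming, or drying values under cover.
; A second timer traces up from the head for a BuildingPiece ceiling, then four horizontal directions, counting three wall hits as shelter.
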(event Custom|Call%20Regular%20Enviornmental%20Sample
  (bind (_celsius _current_weather_type) (Default|GetCurrentWeatherData (Variables|Refrences|GetWeather%20Actor)))
  (Class|EnvironmentalAttributes|SampleEnviornment _celsius (select (Variables|Config|GetUnder%20Ceiling) (select (Variables|Config|GetIn%20Shelter) -2e+01 -1e+01) (+ (CallFunction|CalcualteWetness _current_weather_type) (Math|Float|SelectFloat (Variables|Config|GetSwiming%20Wetness) 0.0 (Variables|Config|GetIs%20Swiming)))))
  (if (Variables|Debug|GetPrint%20State%20Info)
    (CallFunction|PrintEnviornmentData)))

(event Custom|On%20is%20Swiming
  (params (Is%20Swiming :type Boolean))
  (Variables|Config|SetIs%20Swiming Is%20Swiming)
  (CallFunction|CallRegularEnviornmentalSample))

(event Custom|Shelter%20Check
  (CallFunction|CheckforShelter))

(event EventBeginPlay
  (bind _output_get (Variables|Refrences|SetHas%20Authority (Ability|HasAuthority (Components|GetOwner))))
  (if _output_get
    (CallFunction|Initalize)
    (bind _returnvalue (Utilities|Time|SetTimerbyEvent (delegate Custom|Call%20Regular%20Enviornmental%20Sample) (Variables|Config|GetSample%20Frequency) true 0.0 0.1))
    (Variables|Refrences|SetRegulat%20Sample%20Timer%20Handle _returnvalue)
    (EventDispatchers|BindEventtoSwimStatus (Variables|Refrences|GetOwning%20Player%20Character) (delegate Custom|On%20is%20Swiming))
    (Utilities|Time|SetTimerbyEvent (delegate Custom|Shelter%20Check) (Variables|Config|GetShelter%20Check%20Frequency) true)))

(fn Initalize
  (bind _outactors (Actor|GetAllActorsOfClass "/Game/Homestead/Environment/UltraDynamicSky/Blueprints/Ultra_Dynamic_Weather.Ultra_Dynamic_Weather_C"))
  (Utilities|IsValid (Utilities|Array|Get(acopy) _outactors)
    (:Is%20Valid
      (Variables|Refrences|SetWeather%20Actor (Utilities|Array|Get(acopy) _outactors))
      (bind _asbp_srpgcharacter (Utilities|Casting|CastToBP_SRPGCharacter (Components|GetOwner))
        (:then
          (Variables|Refrences|SetOwning%20Player%20Character _asbp_srpgcharacter))
        (:CastFailed
          (Development|PrintString "Player enviornmental attribute could not set owning player"))))
    (:Is%20Not%20Valid
      (Development|PrintString "Player enviornmental attribute could not get weather actor"))))

(fn CalcualteWetness
  (params (Selection :type UDS_WeatherTypes%20Enum :default "NewEnumerator0"))
  (return (Utilities|Select :Index Selection :NewEnumerator0 -5.0 :NewEnumerator1 -2.0 :NewEnumerator2 -2.0 :NewEnumerator3 -1.0 :NewEnumerator11 -1.0 :NewEnumerator4 (Variables|Config|GetLight%20Rain%20Wetness) :NewEnumerator5 (Variables|Config|GetRain%20Wetness) :NewEnumerator6 (Variables|Config|GetThunderstrom%20Wetness) :NewEnumerator7 (Variables|Config|GetLightsnow%20Wetness) :NewEnumerator8 (Variables|Config|GetSnow%20Wetness) :NewEnumerator9 (Variables|Config|GetBlizzart%20Wetness) :NewEnumerator10 -1.0)))

(fn PrintEnviornmentData
  (Development|PrintString (Utilities|String|Append "Current Temp:" (Utilities|String|ToString(Float) (Variables|Default|GetCurrentTemperature))) true true "(R=0.000000,G=0.660000,B=1.000000,A=1.000000)" (Variables|Config|GetSample%20Frequency))
  (Development|PrintString (Utilities|String|Append "Current Wetness:" (Utilities|String|ToString(Float) (Variables|Default|GetCurrentWetness))) true true "(R=0.000000,G=0.660000,B=1.000000,A=1.000000)" (Variables|Config|GetSample%20Frequency))
  (Development|PrintString (Utilities|String|Append "Current Temp State:" (Utilities|String|EnumtoString (Variables|Default|GetCurrentTempState))) true true "(R=0.000000,G=0.660000,B=1.000000,A=1.000000)" (Variables|Config|GetSample%20Frequency))
  (Development|PrintString (Utilities|String|Append "Current Wetness State:" (Utilities|String|EnumtoString (Variables|Default|GetCurrentWetnessState))) true true "(R=0.000000,G=0.660000,B=1.000000,A=1.000000)" (Variables|Config|GetSample%20Frequency))
  (bind _current_weather_type (Default|GetCurrentWeatherType (Variables|Refrences|GetWeather%20Actor)))
  (Development|PrintString (Utilities|String|Append "Current Weather: " (Utilities|String|EnumtoString _current_weather_type)) true true "(R=0.000000,G=0.660000,B=1.000000,A=1.000000)" (Variables|Config|GetSample%20Frequency))
  (Development|PrintString (Utilities|String|Append "Is Swiming: : " (Utilities|String|ToString(Boolean) (Variables|Config|GetIs%20Swiming))) true true "(R=0.000000,G=0.660000,B=1.000000,A=1.000000)" (Variables|Config|GetSample%20Frequency)))

(fn CheckforShelter
  (bind _owning_player_character (Variables|Refrences|GetOwning%20Player%20Character))
  (bind _owning_player_character_2 (Variables|Refrences|GetOwning%20Player%20Character))
  (bind _owning_player_character_3 (Variables|Refrences|GetOwning%20Player%20Character))
  (bind _owning_player_character_4 (Variables|Refrences|GetOwning%20Player%20Character))
  (bind _owning_player_character_5 (Variables|Refrences|GetOwning%20Player%20Character))
  (bind _returnvalue (Transformation|GetActorLocation _owning_player_character))
  (bind _returnvalue_2 (Transformation|GetActorLocation _owning_player_character_2))
  (bind _returnvalue_3 (Transformation|GetActorLocation _owning_player_character_3))
  (bind _returnvalue_4 (Transformation|GetActorLocation _owning_player_character_4))
  (bind _head (Variables|/Game/SRPG/Blueprints/CharacterAssets/BP_SRPGCharacter.BP_SRPGCharacter_C|GetHead _owning_player_character_5))
  (bind _returnvalue_5 (Transformation|GetWorldLocation _head))
  (bind _outhit (Collision|LineTraceByChannel _returnvalue_5 (+ _returnvalue_5 (Math|Vector|MakeVector 0.0 0.0 (Variables|Config|GetShelter%20Check%20Distance))) "TraceTypeQuery1" false 0 (select (Variables|Debug|GetDebug%20Traces) "ForDuration" "None") true "(R=1.000000,G=0.000000,B=0.000000,A=1.000000)" "(R=0.000000,G=1.000000,B=0.000000,A=1.000000)" (Variables|Config|GetShelter%20Check%20Frequency)))
  (Utilities|Casting|CastToBuildingPiece (.hitactor _outhit)
    (:then
      (Variables|Config|SetUnder%20Ceiling true)
      (bind _outhit_2 (Collision|LineTraceByChannel _returnvalue_3 (+ _returnvalue_3 (* (Transformation|GetActorForwardVector _owning_player_character_3) (Variables|Config|GetShelter%20Check%20Distance))) "TraceTypeQuery1" false 0 (select (Variables|Debug|GetDebug%20Traces) "ForDuration" "None") true "(R=1.000000,G=0.000000,B=0.000000,A=1.000000)" "(R=0.000000,G=1.000000,B=0.000000,A=1.000000)" (Variables|Config|GetShelter%20Check%20Frequency)))
      (Utilities|Casting|CastToBuildingPiece (.hitactor _outhit_2)
        (:then
          (Math|Integer|IncrementInt (LocalVariables|GetShelterCheck)
            (:%20%20
              _)))
        (:CastFailed
          _))
      (bind _outhit_3 (Collision|LineTraceByChannel _returnvalue_4 (+ _returnvalue_4 (* (Transformation|GetActorRightVector _owning_player_character_4) (Variables|Config|GetShelter%20Check%20Distance))) "TraceTypeQuery1" false 0 (select (Variables|Debug|GetDebug%20Traces) "ForDuration" "None") true "(R=1.000000,G=0.000000,B=0.000000,A=1.000000)" "(R=0.000000,G=1.000000,B=0.000000,A=1.000000)" (Variables|Config|GetShelter%20Check%20Frequency)))
      (Utilities|Casting|CastToBuildingPiece (.hitactor _outhit_3)
        (:then
          (Math|Integer|IncrementInt (LocalVariables|GetShelterCheck)
            (:%20%20
              _)))
        (:CastFailed
          _))
      (bind _outhit_4 (Collision|LineTraceByChannel _returnvalue_2 (- _returnvalue_2 (* (Transformation|GetActorForwardVector _owning_player_character_2) (Variables|Config|GetShelter%20Check%20Distance))) "TraceTypeQuery1" false 0 (select (Variables|Debug|GetDebug%20Traces) "ForDuration" "None") true "(R=1.000000,G=0.000000,B=0.000000,A=1.000000)" "(R=0.000000,G=1.000000,B=0.000000,A=1.000000)" (Variables|Config|GetShelter%20Check%20Frequency)))
      (Utilities|Casting|CastToBuildingPiece (.hitactor _outhit_4)
        (:then
          (Math|Integer|IncrementInt (LocalVariables|GetShelterCheck)
            (:%20%20
              _)))
        (:CastFailed
          _))
      (bind _outhit_5 (Collision|LineTraceByChannel _returnvalue (- _returnvalue (* (Transformation|GetActorRightVector _owning_player_character) (Variables|Config|GetShelter%20Check%20Distance))) "TraceTypeQuery1" false 0 (select (Variables|Debug|GetDebug%20Traces) "ForDuration" "None") true "(R=1.000000,G=0.000000,B=0.000000,A=1.000000)" "(R=0.000000,G=1.000000,B=0.000000,A=1.000000)" (Variables|Config|GetShelter%20Check%20Frequency)))
      (Utilities|Casting|CastToBuildingPiece (.hitactor _outhit_5)
        (:then
          (Math|Integer|IncrementInt (LocalVariables|GetShelterCheck)
            (:%20%20
              _)))
        (:CastFailed
          _))
      (if (>= (LocalVariables|GetShelterCheck) 3)
        (Variables|Config|SetIn%20Shelter true)
        (Development|PrintString "In Shelter" (Variables|Debug|GetDebug%20Traces) true "(R=0.000000,G=0.660000,B=1.000000,A=1.000000)" (Variables|Config|GetShelter%20Check%20Frequency))
        (else
          (Variables|Config|SetIn%20Shelter false))))
    (:CastFailed
      (Variables|Config|SetUnder%20Ceiling false)
      (Variables|Config|SetIn%20Shelter false))))