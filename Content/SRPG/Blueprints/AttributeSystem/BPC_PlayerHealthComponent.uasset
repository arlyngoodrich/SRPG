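; Player health component that gives BP_SRPGCharacter its reactions to damage and death.
; It caches the owning character on BeginPlay for use in the health events.
; On death it ragdolls the mesh and, only for the locally controlled character, disables input.
; Negative health changes trigger the damage display on the player HUD, also only for the local player.
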(event EventOnDeath
  (bind _owningcharacter (Variables|References|GetOwningCharacter))
  (Physics|SetSimulatePhysics (Variables|/Script/Engine.Character|GetMesh _owningcharacter) true)
  (if (Pawn|IsLocallyControlled _owningcharacter)
    (Input|DisableInput _owningcharacter (Variables|/Game/SRPG/Blueprints/CharacterAssets/BP_SRPGCharacter.BP_SRPGCharacter_C|GetPlayer%20Controller _owningcharacter))))

(event EventBeginPlay
  (bind _asbp_srpgcharacter (Utilities|Casting|CastToBP_SRPGCharacter (Components|GetOwner)))
  (Variables|References|SetOwningCharacter _asbp_srpgcharacter))

(event EventOnHealthChange
  (params (ChangeAmount :type Float%20%28single-precision%29) (NewHealth :type Float%20%28single-precision%29))
  (bind _owningcharacter (Variables|References|GetOwningCharacter))
  (if (Pawn|IsLocallyControlled _owningcharacter)
    (if (< ChangeAmount 0.0)
      (Default|ShowDamage (Variables|/Game/SRPG/Blueprints/CharacterAssets/BP_SRPGCharacter.BP_SRPGCharacter_C|GetPlayer%20HUD _owningcharacter)))))