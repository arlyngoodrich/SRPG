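; Player health component for the SRPG character that handles death, damage feedback and status effect display.
; On death it ragdolls the owner's mesh and disables input for the locally controlled player.
; Health loss triggers a damage indicator on the local player's HUD.
; Effect add and remove events forward icon, colors and name to that HUD, without a local-control check.
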(event EventOnHealthChange
  (params (ChangeAmount :type Float%20%28single-precision%29) (NewHealth :type Float%20%28single-precision%29))
  (bind _owningcharacter (Variables|References|GetOwningCharacter))
  (if (Pawn|IsLocallyControlled _owningcharacter)
    (if (< ChangeAmount 0.0)
      (Default|ShowDamage (Variables|/Game/SRPG/Blueprints/CharacterAssets/BP_SRPGCharacter.BP_SRPGCharacter_C|GetPlayer%20HUD _owningcharacter)))))

(event EventRemoveEffectfromUI
  (params (EffectName :type Name :default "None"))
  (bind _asbp_srpgcharacter (Utilities|Casting|CastToBP_SRPGCharacter (Components|GetOwner)))
  (Default|RemoveEffect (Variables|/Game/SRPG/Blueprints/CharacterAssets/BP_SRPGCharacter.BP_SRPGCharacter_C|GetPlayer%20HUD _asbp_srpgcharacter) EffectName))

(event EventOnDeath
  (bind _owningcharacter (Variables|References|GetOwningCharacter))
  (bind _mesh (Variables|/Script/Engine.Character|GetMesh _owningcharacter))
  (Collision|SetCollisionProfileName _mesh "Ragdoll" false :!class /Script/Engine.PrimitiveComponent)
  (Physics|SetSimulatePhysics _mesh true)
  (if (Pawn|IsLocallyControlled _owningcharacter)
    (Input|DisableInput _owningcharacter (Variables|/Game/SRPG/Blueprints/CharacterAssets/BP_SRPGCharacter.BP_SRPGCharacter_C|GetPlayer%20Controller _owningcharacter))))

(event EventBeginPlay
  (bind _asbp_srpgcharacter (Utilities|Casting|CastToBP_SRPGCharacter (Components|GetOwner)))
  (Variables|References|SetOwningCharacter _asbp_srpgcharacter))

(event EventAddEffecttoUI
  (params (IconTexutre :type Texture%202D%20Object%20Reference) (IconColor :type Color%20Structure) (BackgroundColor :type Color%20Structure) (EffectName :type Name :default "None"))
  (bind _asbp_srpgcharacter (Utilities|Casting|CastToBP_SRPGCharacter (Components|GetOwner)))
  (Default|AddEffect (Variables|/Game/SRPG/Blueprints/CharacterAssets/BP_SRPGCharacter.BP_SRPGCharacter_C|GetPlayer%20HUD _asbp_srpgcharacter) (Math|Conversions|ToLinearColor(Color) BackgroundColor) (Math|Conversions|ToLinearColor(Color) IconColor) IconTexutre EffectName))