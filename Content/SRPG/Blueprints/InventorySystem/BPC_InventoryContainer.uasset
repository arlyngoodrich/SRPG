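; Inventory container component that serves characters and world storage, including crafting stations, in the SRPG inventory system.
; On character owners, inventory updates refresh the player inventory manager's weight.
; Opening storage claims an unowned actor via SetOwner and disables the user's movement; InteractingCharacter's RepNotify toggles a lazily created storage widget for the local player.
; Closing the menu restores walking and clears ownership.
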(event Custom|Toggle%20Storage%20UI
  (bind _interacting_character (Variables|Default|GetInteracting%20Character))
  (Utilities|IsValid _interacting_character
    (:Is%20Valid
      (if (Pawn|IsLocallyControlled _interacting_character)
        (Utilities|IsValid (Variables|Default|GetStorage%20UI)
          (:Is%20Valid
            (Default|MulticastToggleMenu (Variables|Default|GetInteracting%20Character) (Variables|Default|GetStorage%20UI)))
          (:Is%20Not%20Valid
            (bind _returnvalue (UserInterface|CreateWidget "/Game/SRPG/Blueprints/ItemSystem/WBP_CraftingStorageContainer.WBP_CraftingStorageContainer_C" 0 self (Variables|Default|GetInteracting%20Character) (Variables|Default|GetIs%20Part%20of%20Crafting%20Station) (Math|Integer|Absolute(Integer) (Variables|Default|GetInteraction%20Index))))
            (Variables|Default|SetStorage%20UI _returnvalue)
            (Default|MulticastToggleMenu (Variables|Default|GetInteracting%20Character) (Variables|Default|GetStorage%20UI))
            (EventDispatchers|BindEventtoMenuClosed (Variables|Default|GetInteracting%20Character) (delegate Custom|Storage%20Closed))))))))

(event Custom|Storage%20Closed
  (CallFunction|ReleaseStorage))

(event Custom|Release%20Storage
  (Pawn|Components|CharacterMovement|SetMovementMode (Variables|/Script/Engine.Character|GetCharacterMovement (Variables|Default|GetInteracting%20Character)) "MOVE_Walking" 0)
  (Actor|SetOwner (Components|GetOwner) 0))

(event Custom|Call%20Toggle%20Stroage
  (params (Interacting%20Actor :type Actor%20Object%20Reference) (Interaction%20Index :type Integer))
  (bind _returnvalue (Components|GetOwner))
  (bind _returnvalue_2 (Components|GetOwner _returnvalue))
  (Variables|Default|SetInteraction%20Index Interaction%20Index)
  (if (== 0 _returnvalue_2)
    (Actor|SetOwner (Components|GetOwner) Interacting%20Actor)
    (bind _asbp_srpgcharacter (Utilities|Casting|CastToBP_SRPGCharacter Interacting%20Actor)
      (:then
        (Variables|Default|SetInteracting%20Character _asbp_srpgcharacter)
        (Pawn|Components|CharacterMovement|DisableMovement (Variables|/Script/Engine.Character|GetCharacterMovement (Variables|Default|GetInteracting%20Character))))
      (:CastFailed
        (Development|PrintString "Trying to open inventory UI with non SRPG Character")))
    (elif (== Interacting%20Actor _returnvalue_2)
      (CallFunction|ToggleStorageUI))))

(event EventInventoryUpdated
  (bind _my_player_owner (Variables|Default|GetMy%20Player%20Owner))
  (bind _bpc_playerinventorymanager (Variables|/Game/SRPG/Blueprints/CharacterAssets/BP_SRPGCharacter.BP_SRPGCharacter_C|GetBPC_PlayerInventoryManager _my_player_owner))
  (if (Variables|Default|GetIs%20Character%20Owned)
    (Utilities|IsValid _bpc_playerinventorymanager
      (:Is%20Valid
        (Default|UpdateWeight _bpc_playerinventorymanager)))))

(event EventBeginPlay
  (bind _ascharacter (Utilities|Casting|CastToCharacter (Components|GetOwner))
    (:then
      (Variables|Default|SetIs%20Character%20Owned true)
      (bind _asbp_srpgcharacter (Utilities|Casting|CastToBP_SRPGCharacter _ascharacter))
      (Variables|Default|SetMy%20Player%20Owner _asbp_srpgcharacter))
    (:CastFailed
      (Variables|Default|SetIs%20Character%20Owned false))))

(fn ExternalDestroyComponent
  (Components|DestroyComponent))

(fn OnRepInteractingCharacter
  (CallFunction|ToggleStorageUI))