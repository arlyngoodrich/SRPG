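; Short-lived crop spawner for the field system that turns itself into a crop on a field's snap point.
; When spawning finishes, the server checks that the snap point belongs to a BP_Field, then spawns the configured crop class with random yaw.
; The crop receives the field and snap point, the snap point is force-snapped, and the spawner expires almost immediately via its lifespan.
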(event EventOnSpawnFinished
  (bind _returnvalue (Transformation|GetActorTransform))
  (bind _snap_point (Variables|Default|GetSnap%20Point))
  (Networking|SwitchHasAuthority
    (:Authority
      (Utilities|IsValid _snap_point
        (:Is%20Valid
          (bind _asbp_field (Utilities|Casting|CastToBP_Field (Variables|/Game/SRPG/Blueprints/BuildSystem/BP_SnapPointActor.BP_SnapPointActor_C|GetMy%20Parent _snap_point)))
          (Variables|Default|SetMy%20Field _asbp_field)
          (Game|SpawnActorfromClass (Variables|Default|GetCrop%20to%20Spawn) (Math|Transform|MakeTransform (.location _returnvalue) (Math|Rotator|MakeRotator (.roll (.rotation _returnvalue)) (.pitch (.rotation _returnvalue)) (Math|Random|RandomFloatinRange -1.8e+02 1.8e+02)) (.scale _returnvalue)) "Undefined" 0 (Variables|Default|GetMy%20Field) (Variables|Default|GetSnap%20Point) 0)
          (Default|ForceSnap (Variables|Default|GetSnap%20Point))
          (Actor|SetLifeSpan 0.1))))))

(fn ConstructionScript
  (|CallParentFunction))