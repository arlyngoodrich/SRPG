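; Base crop Blueprint for the field system that links crop growth and watering to Ultra Dynamic Sky and Weather.
; On BeginPlay it warns about missing growth-stage meshes, finds both actors and binds to their sunrise and weather events.
; Each sunrise calls AdvanceDay with the previous day's average temperature.
; Light rain, rain and thunderstorms start a looping timer that adds water by intensity, cleared on every weather change.
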(event Custom|On%20Weather%20Change
  (params (Temperature :type Float%20%28single-precision%29) (Weather%20Type :type UDS_WeatherTypes%20Enum :default "NewEnumerator0"))
  (CallFunction|HandleWeatherChange Temperature Weather%20Type))

(event Custom|On%20Sunrise
  (CallFunction|HandleNewDay))

(event Custom|On%20Rain%20Start
  (bind _returnvalue (Utilities|Time|SetTimerbyFunctionName self "Add Rain Water" (Variables|Rain|GetRain%20Water%20Add%20Frequency) true))
  (Variables|Rain|SetRain%20Timer%20Handle _returnvalue))

(event Custom|On%20Rain%20End
  (Utilities|Time|ClearandInvalidateTimerbyHandle (Variables|Rain|GetRain%20Timer%20Handle)))

(event EventBeginPlay
  (CallFunction|ValidateGrowthData)
  (CallFunction|InitalizeReferences)
  (EventDispatchers|BindEventtoSunrise (Variables|Refrences|GetSky) (delegate Custom|On%20Sunrise))
  (EventDispatchers|BindEventtoUpdateWeatherData (Variables|Refrences|GetWeather) (delegate Custom|On%20Weather%20Change))
  (bind (_celsius _current_weather_type) (Default|GetCurrentWeatherData (Variables|Refrences|GetWeather)))
  (CallFunction|HandleWeatherChange _celsius _current_weather_type))

(fn ConstructionScript
  (|CallParentFunction))

(fn ValidateGrowthData
  (if (not (Math|Boolean|ANDBoolean (Utilities|IsValid (.GrowthLevelMesh (Utilities|Struct|BreakCropGrowthData (Variables|Default|GetSeedlingGrowthData)))) (Utilities|IsValid (.GrowthLevelMesh (Utilities|Struct|BreakCropGrowthData (Variables|Default|GetMiddlingGrowthData)))) (Utilities|IsValid (.GrowthLevelMesh (Utilities|Struct|BreakCropGrowthData (Variables|Default|GetMatureGrowthData))))))
    (Development|PrintString (Utilities|String|Append (Utilities|GetDisplayName self) " is missing growth level meshes"))))

(fn HandleWeatherChange
  (params (New%20Temp :type Float%20%28single-precision%29) (New%20Weather%20Type :type UDS_WeatherTypes%20Enum :default "NewEnumerator0"))
  (CallFunction|OnRainEnd)
  (switch Utilities|FlowControl|Switch|SwitchonUDS_WeatherTypes New%20Weather%20Type
    (:NewEnumerator4
      (Variables|Rain|SetCurrentRainAmount (Variables|Rain|GetLight%20Rain%20Water%20Amount)))
    (:NewEnumerator5
      (Variables|Rain|SetCurrentRainAmount (Variables|Rain|GetRain%20Water%20Amount)))
    (:NewEnumerator6
      (Variables|Rain|SetCurrentRainAmount (Variables|Rain|GetHeavy%20Rain%20Water%20Amount))))
  (CallFunction|OnRainStart))

(fn HandleNewDay
  (Class|Crop|AdvanceDay (Variables|/Game/Homestead/Environment/UltraDynamicSky/Blueprints/Ultra_Dynamic_Weather.Ultra_Dynamic_Weather_C|GetAverage%20Temp%20for%20Previous%20Day (Variables|Refrences|GetWeather))))

(fn InitalizeReferences
  (bind _outactors (Actor|GetAllActorsOfClass "/Game/Homestead/Environment/UltraDynamicSky/Blueprints/Ultra_Dynamic_Weather.Ultra_Dynamic_Weather_C"))
  (Utilities|IsValid (Utilities|Array|Get(acopy) _outactors)
    (:Is%20Valid
      (Variables|Refrences|SetWeather (Utilities|Array|Get(acopy) _outactors)))
    (:Is%20Not%20Valid
      _))
  (bind _outactors_2 (Actor|GetAllActorsOfClass "/Game/Homestead/Environment/UltraDynamicSky/Blueprints/Ultra_Dynamic_Sky.Ultra_Dynamic_Sky_C"))
  (Variables|Refrences|SetSky (Utilities|Array|Get(acopy) _outactors_2)))

(fn AddRainWater
  (Class|Crop|AddWater (Variables|Rain|GetCurrentRainAmount)))