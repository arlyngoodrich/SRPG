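; Base crop actor for a farming system that grows with weather and days and can be inspected or harvested.
; On the server, Ultra Dynamic Sky sunrises advance days and weather drives rain-watering timers, though BeginPlay also forces Mature after a short delay.
; Interaction opens a plant info UI, using actor ownership as a single-user lock, or harvests seasonal yields.
; Harvest cross-breeds genes with a random overlapping same-class crop, registering seed data through ItemManager.
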(event InteractionTriggered(BPC_InteractableObjectComponent)
  (params (Player%20Interaction%20Sensor :type BPC%20Player%20Interaction%20Sensor%20Object%20Reference) (Interaction%20Index :type Integer))
  ;[1 1 1] Interaction
  (switch int Interaction%20Index
    (:0
      (CallFunction|CallToggleStroage (Components|GetOwner Player%20Interaction%20Sensor)))
    (:1
      (bind _asbp_srpgcharacter (Utilities|Casting|CastToBP_SRPGCharacter (Components|GetOwner Player%20Interaction%20Sensor)))
      (Harvest|HarvestCrop _asbp_srpgcharacter))))

(event Custom|On%20Weather%20Change
  (params (Temperature :type Float%20%28single-precision%29) (Weather%20Type :type UDS_WeatherTypes%20Enum :default "NewEnumerator0"))
  ;[1 1 1] Weather Bindings
  (Enviornment|HandleWeatherChange Temperature Weather%20Type))

(event Custom|Client%20Update%20UI
  ;[1 1 1] Client Updates
  (Default|CallUpdateUI))

(event Custom|Toggle%20Storage%20UI
  (bind _interacting_character_ui (Variables|UI|GetInteracting%20Character%20UI))
  ;[1 1 1] UI Management
  (Utilities|IsValid _interacting_character_ui
    (:Is%20Valid
      (if (Pawn|IsLocallyControlled _interacting_character_ui)
        (Utilities|IsValid (Variables|UI|GetPlantUI)
          (:Is%20Valid
            (Default|MulticastToggleMenu (Variables|UI|GetInteracting%20Character%20UI) (Variables|UI|GetPlantUI)))
          (:Is%20Not%20Valid
            (bind _returnvalue (UserInterface|CreateWidget "/Game/SRPG/Blueprints/CropSystem/WBP_PlantInfoUI.WBP_PlantInfoUI_C" 0 self))
            (Variables|UI|SetPlantUI _returnvalue)
            (Default|MulticastToggleMenu (Variables|UI|GetInteracting%20Character%20UI) (Variables|UI|GetPlantUI))
            (EventDispatchers|BindEventtoMenuClosed (Variables|UI|GetInteracting%20Character%20UI) (delegate Custom|Storage%20Closed))))))))

(event Custom|Release%20Storage
  ;[1 1 1] UI Management
  (Pawn|Components|CharacterMovement|SetMovementMode (Variables|/Script/Engine.Character|GetCharacterMovement (Variables|UI|GetInteracting%20Character%20UI)) "MOVE_Walking" 0)
  (Actor|SetOwner 0)
  (Variables|UI|SetbIsUIOpen false))

(event Custom|Storage%20Closed
  ;[1 1 1] UI Management
  (CallFunction|ReleaseStorage))

(event Custom|On%20Rain%20End
  ;[1 1 1] Rain Controls
  (Utilities|Time|ClearandInvalidateTimerbyHandle (Variables|Rain|GetRain%20Timer%20Handle)))

(event Custom|Call%20Toggle%20Stroage
  (params (Interacting%20Actor :type Actor%20Object%20Reference))
  (bind _returnvalue (Components|GetOwner))
  ;[1 1 1] UI Management
  (if (== 0 _returnvalue)
    (Variables|UI|SetbIsUIOpen true)
    (Actor|SetOwner Interacting%20Actor)
    (bind _asbp_srpgcharacter (Utilities|Casting|CastToBP_SRPGCharacter Interacting%20Actor)
      (:then
        (Variables|UI|SetInteracting%20Character%20UI _asbp_srpgcharacter)
        (Pawn|Components|CharacterMovement|DisableMovement (Variables|/Script/Engine.Character|GetCharacterMovement (Variables|UI|GetInteracting%20Character%20UI))))
      (:CastFailed
        (Development|PrintString "Trying to open Plant UI with non SRPG Character")))
    (elif (== Interacting%20Actor _returnvalue)
      (CallFunction|ToggleStorageUI))))

(event Custom|On%20Rain%20Start
  ;[1 1 1] Rain Controls
  (bind _returnvalue (Utilities|Time|SetTimerbyFunctionName self "Add Rain Water" (Variables|Rain|GetRain%20Water%20Add%20Frequency) true))
  (Variables|Rain|SetRain%20Timer%20Handle _returnvalue))

(event Custom|On%20Sunrise
  ;[1 1 1] Weather Bindings
  (Enviornment|HandleNewDay))

(event EventOnCropDataUpdate
  ;[1 1 1] Client Updates
  (Networking|SwitchHasAuthority
    (:Authority
      (CallFunction|ClientUpdateUI))))

(event EventOnFertilizerUpdate
  ;[1 1 1] Client Updates
  (Networking|SwitchHasAuthority
    (:Authority
      (if (Variables|UI|GetbIsUIOpen)
        (CallFunction|ClientUpdateUI)))))

(event EventOnWaterUpdate
  ;[1 1 1] Client Updates
  (Networking|SwitchHasAuthority
    (:Authority
      (if (Variables|UI|GetbIsUIOpen)
        (CallFunction|ClientUpdateUI)))))

(event EventBeginPlay
  ;[1 1 1] Initalization
  (Networking|SwitchHasAuthority
    (:Authority
      (Initalize|ValidateGrowthData)
      (Initalize|InitalizeReferences)
      (EventDispatchers|BindEventtoSunrise (Variables|Refrences|GetSky) (delegate Custom|On%20Sunrise))
      (EventDispatchers|BindEventtoUpdateWeatherData (Variables|Refrences|GetWeather) (delegate Custom|On%20Weather%20Change))
      (bind (_celsius _current_weather_type) (Default|GetCurrentWeatherData (Variables|Refrences|GetWeather)))
      (Enviornment|HandleWeatherChange _celsius _current_weather_type)
      (Utilities|FlowControl|Delay 5.0)
      (Class|Crop|SetGrowhtStage "EGS_Mature"))))

(fn ConstructionScript
  (|CallParentFunction)
  (Components|Sphere|SetSphereRadius (Variables|Default|GetCrossBreedCheck) (Variables|Harvest|GetCross%20Breed%20Radius) true))

(fn ValidateGrowthData
  (if (not (Math|Boolean|ANDBoolean (Utilities|IsValid (Utilities|Struct|BreakCropGrowthData (Variables|Default|GetSeedlingGrowthData))) (Utilities|IsValid (Utilities|Struct|BreakCropGrowthData (Variables|Default|GetMiddlingGrowthData))) (Utilities|IsValid (Utilities|Struct|BreakCropGrowthData (Variables|Default|GetMatureGrowthData)))))
    (Development|PrintString (Utilities|String|Append (Utilities|GetDisplayName self) " is missing growth level meshes"))))

(fn HandleWeatherChange
  (params (New%20Temp :type Float%20%28single-precision%29) (New%20Weather%20Type :type UDS_WeatherTypes%20Enum :default "NewEnumerator0"))
  (CallFunction|OnRainEnd)
  (switch Utilities|FlowControl|Switch|SwitchonUDS_WeatherTypes New%20Weather%20Type
    (:NewEnumerator4
      (Variables|Rain|SetCurrentRainAmount (Variables|Rain|GetLight%20Rain%20Water%20Amount)))
    (:NewEnumerator5
      (Variables|Rain|SetCurrentRainAmount (Variables|Rain|GetRain%20Water%20Amount)))
    (:NewEnumerator6
      (Variables|Rain|SetCurrentRainAmount (Variables|Rain|GetHeavy%20Rain%20Water%20Amount))))
  (CallFunction|OnRainStart))

(fn HandleNewDay
  (Class|Crop|AdvanceDay (Variables|/Game/Homestead/Environment/UltraDynamicSky/Blueprints/Ultra_Dynamic_Weather.Ultra_Dynamic_Weather_C|GetAverage%20Temp%20for%20Previous%20Day (Variables|Refrences|GetWeather))))

(fn InitalizeReferences
  (bind _outactors (Actor|GetAllActorsOfClass "/Game/Homestead/Environment/UltraDynamicSky/Blueprints/Ultra_Dynamic_Weather.Ultra_Dynamic_Weather_C"))
  (Utilities|IsValid (Utilities|Array|Get(acopy) _outactors)
    (:Is%20Valid
      (Variables|Refrences|SetWeather (Utilities|Array|Get(acopy) _outactors)))
    (:Is%20Not%20Valid
      _))
  (bind _outactors_2 (Actor|GetAllActorsOfClass "/Game/Homestead/Environment/UltraDynamicSky/Blueprints/Ultra_Dynamic_Sky.Ultra_Dynamic_Sky_C"))
  (Utilities|IsValid (Utilities|Array|Get(acopy) _outactors_2)
    (:Is%20Valid
      (Variables|Refrences|SetSky (Utilities|Array|Get(acopy) _outactors_2)))
    (:Is%20Not%20Valid
      _))
  (bind _outactors_3 (Actor|GetAllActorsOfClass "/Game/SRPG/Blueprints/ItemSystem/BP_ItemManager.BP_ItemManager_C"))
  (Utilities|IsValid (Utilities|Array|Get(acopy) _outactors_3)
    (:Is%20Valid
      (Variables|Refrences|SetItem%20Manager (Utilities|Array|Get(acopy) _outactors_3)))))

(fn AddRainWater
  (Class|Crop|AddWater (Variables|Rain|GetCurrentRainAmount)))

(fn OnRepInteractingCharacter
  (CallFunction|ToggleStorageUI))

(fn HarvestCrop
  (params (Player%20Character :type BP%20SRPG%20Character%20Object%20Reference))
  (bind _currentgrowthdata (Variables|Default|GetCurrentGrowthData))
  (bind (_winteryield _springyield _summeryield _fallyield _seedyield) (Utilities|Struct|BreakCropGrowthData _currentgrowthdata))
  (bind _cross_bredgene_data (Harvest|CrossBreed))
  (Variables|Harvest|SetCross%20Bred%20Gene%20Data _cross_bredgene_data)
  (switch Utilities|FlowControl|Switch|SwitchonUDS_Season (Variables|/Game/Homestead/Environment/UltraDynamicSky/Blueprints/Ultra_Dynamic_Weather.Ultra_Dynamic_Weather_C|GetSeason (Variables|Refrences|GetWeather))
    (:NewEnumerator0
      (LocalVariables|SetCurrent%20Yield%20Data _summeryield))
    (:NewEnumerator1
      (LocalVariables|SetCurrent%20Yield%20Data _fallyield))
    (:NewEnumerator2
      (LocalVariables|SetCurrent%20Yield%20Data _winteryield))
    (:NewEnumerator3
      (LocalVariables|SetCurrent%20Yield%20Data _springyield)))
  (bind _output_get (LocalVariables|SetSeed%20Yield%20Data _seedyield))
  (for _array_element _output_get
    (if (Utilities|IsValidClass (.HarvestedItem (Utilities|Struct|BreakCropYieldData _array_element)))
      (bind _seed_id (Default|CheckinSeedData (Variables|Refrences|GetItem%20Manager) (Variables|Harvest|GetCross%20Bred%20Gene%20Data)))
      (bind _structout (Utilities|Struct|SetmembersinItemData (Utilities|GetClassDefaults (.HarvestedItem (Utilities|Struct|BreakCropYieldData _array_element))) (Math|Random|RandomIntegerinRange (.MinYield (Utilities|Struct|BreakCropYieldData _array_element)) (.MaxYield (Utilities|Struct|BreakCropYieldData _array_element))) _seed_id))
      (Default|AutoAddItem (Variables|/Game/SRPG/Blueprints/CharacterAssets/BP_SRPGCharacter.BP_SRPGCharacter_C|GetBPC_PlayerInventoryManager Player%20Character) _structout)
      (else
        (Development|PrintString "Not valid seed class"))))
  (for _array_element_2 (LocalVariables|GetCurrent%20Yield%20Data)
    (if (Utilities|IsValidClass (.HarvestedItem (Utilities|Struct|BreakCropYieldData _array_element_2)))
      (bind _structout_2 (Utilities|Struct|SetmembersinItemData (Utilities|GetClassDefaults (.HarvestedItem (Utilities|Struct|BreakCropYieldData _array_element_2))) (Math|Random|RandomIntegerinRange (.MinYield (Utilities|Struct|BreakCropYieldData _array_element_2)) (.MaxYield (Utilities|Struct|BreakCropYieldData _array_element_2)))))
      (Default|AutoAddItem (Variables|/Game/SRPG/Blueprints/CharacterAssets/BP_SRPGCharacter.BP_SRPGCharacter_C|GetBPC_PlayerInventoryManager Player%20Character) _structout_2)
      (else
        (Development|PrintString "Not valid class"))))
  (Actor|SetLifeSpan 0.1))

(fn CrossBreed
  (bind _self self)
  (bind _crossbreedcheck (Variables|Default|GetCrossBreedCheck))
  (bind _returnvalue (Utilities|GetClass _self))
  (bind _overlappingactors (Collision|GetOverlappingActors _crossbreedcheck _returnvalue :!class /Script/Engine.PrimitiveComponent))
  (Collision|SetCollisionEnabled (Variables|Default|GetCrossBreedCheck) "QueryOnly")
  (LocalVariables|SetCrossBreedCandidates _overlappingactors)
  (LocalVariables|SetNumCrossBreedCandidates (Utilities|Array|Length _overlappingactors))
  (if (> (LocalVariables|GetNumCrossBreedCandidates) 0)
    (bind _asbp_base_crop (Utilities|Casting|CastToBP_BaseCrop (Utilities|Array|Get(acopy) (LocalVariables|GetCrossBreedCandidates) (Math|Random|RandomIntegerinRange 0 (- (LocalVariables|GetNumCrossBreedCandidates) 1))))
      (:then
        (Collision|SetCollisionEnabled (Variables|Default|GetCrossBreedCheck) "NoCollision")
        (return (Class|Crop|GetCrossBredGeneData (Class|Crop|GetGeneData _asbp_base_crop))))
      (:CastFailed
        (Development|PrintString "attemped to cross breed with invalid crop")))
    (else
      (Collision|SetCollisionEnabled (Variables|Default|GetCrossBreedCheck) "NoCollision")
      (return (Class|Crop|GetCrossBredGeneData (Class|Crop|GetGeneData))))))