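; BP_FieldCrop is a crop actor in the crop system that belongs to a parent field and occupies a snap point.
; On BeginPlay it checks in with the field, then after a brief delay takes the first snap point overlapping its sphere and forces a snap.
; When destroyed with a valid snap point, it has that point recheck snaps and checks out of the field.
; If the field is destroyed, the crop expires shortly after.
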(event OnDestroyed(ParentField)
  (params (DestroyedActor :type Actor%20Object%20Reference))
  (Actor|SetLifeSpan 0.1))

(event EventBeginPlay
  (|CallParentFunction)
  (Default|CheckinCrop (Variables|Default|GetParent%20Field) self)
  (Utilities|FlowControl|Delay 0.1)
  (bind _asbp_snap_point_actor (Utilities|Casting|CastToBP_SnapPointActor (Utilities|Array|Get(acopy) (Collision|GetOverlappingActors (Variables|Default|GetSphere_0) "/Game/SRPG/Blueprints/BuildSystem/BP_SnapPointActor.BP_SnapPointActor_C" :!class /Script/Engine.PrimitiveComponent))))
  (bind _output_get (Variables|Default|SetSnap%20Point _asbp_snap_point_actor))
  (Default|ForceSnap _output_get))

(event EventDestroyed
  (bind _snap_point (Variables|Default|GetSnap%20Point))
  (Utilities|IsValid _snap_point
    (:Is%20Valid
      (Default|CheckforSnaps _snap_point)
      (Default|CheckOutCrop (Variables|Default|GetParent%20Field) self))))

(fn ConstructionScript)