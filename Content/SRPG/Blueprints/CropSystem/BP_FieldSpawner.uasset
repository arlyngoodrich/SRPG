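; BP_FieldSpawner is a crop system build placeholder that swaps itself for a BP_Field actor when its build status changes to set.
; On that event it removes foliage via a multicast, then spawns the field at a fixed local XY offset, rotated by its yaw using manual sine and cosine math.
; It passes the foliage transforms and components to the field through SetGrassRemoved, then destroys itself.
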(event EventOnBuildStatusChangetoSet
  (bind _returnvalue (Transformation|GetActorRotation))
  (bind (_x _y) (Math|Vector|BreakVector "-360.000000,-500.000000, 0"))
  (bind _returnvalue_2 (Math|Trig|Cos(Degrees) (.yaw _returnvalue)))
  (bind _returnvalue_3 (Math|Trig|Sin(Degrees) (.yaw _returnvalue)))
  (CallFunction|RemoveFoliageMulticast)
  (bind _returnvalue_4 (Game|SpawnActorfromClass "/Game/SRPG/Blueprints/CropSystem/BP_Field.BP_Field_C" (Math|Transform|MakeTransform (+ (Transformation|GetActorLocation) (Math|Vector|MakeVector (- (* _x _returnvalue_2) (* _y _returnvalue_3)) (+ (* _y _returnvalue_2) (* _x _returnvalue_3)) 0.0)) (Transformation|GetActorRotation) "1,1,1") "Undefined" 0 0))
  (Default|SetGrassRemoved _returnvalue_4 (Variables|Default|GetFoliage%20Transforms) (Variables|Default|GetFoliage%20Components))
  (Actor|DestroyActor))

(fn ConstructionScript
  (|CallParentFunction))