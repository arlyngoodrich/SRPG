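; BP_Field is a crop field actor that builds a terrain-conforming procedural soil mesh and a grid of crop snap points.
; Construction line-traces each vertex and snap point onto the ground, sinking the mesh edges.
; Registered crops save class, transform, growth and gene data, and respawn on the authority after load.
; Grass near snap points is hidden on load, with transforms cached to re-add when the field is destroyed, including by interaction.
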(event InteractionTriggered(BPC_InteractableObjectComponent)
  (params (Player%20Interaction%20Sensor :type BPC%20Player%20Interaction%20Sensor%20Object%20Reference) (Interaction%20Index :type Integer))
  (Actor|SetLifeSpan 0.1))

(event Custom|Initalization%20Finished_Event
  (Networking|SwitchHasAuthority
    (:Authority
      (SaveData|LoadCrops)
      (EventDispatchers|UnbindEventfromInitalizationFinished (delegate Custom|Initalization%20Finished_Event)))))

(event Custom|Multicast%20Remove%20Grass%20on%20Load
  (GrassManagement|RemoveGrassonLoad))

(event EventDestroyed
  (GrassManagement|ReturnGrass))

(event EventBeginPlay
  (for _array_element (Actor|GetComponentsByClass "/Game/SRPG/Blueprints/BuildSystem/BPC_SnapPointSpawn.BPC_SnapPointSpawn_C")
    (Default|OnSpawnFinished _array_element)
    (Utilities|FlowControl|Delay 0.2)
    (bind _asbp_snap_point_actor (Utilities|Casting|CastToBP_SnapPointActor (Utilities|Array|Get(acopy) (Collision|GetOverlappingActors (Variables|Default|GetBox) "/Game/SRPG/Blueprints/BuildSystem/BP_SnapPointActor.BP_SnapPointActor_C" :!class /Script/Engine.PrimitiveComponent))))
    (Default|CheckforSnaps _asbp_snap_point_actor)
    (Default|CallInitalizationFinished)))

(event EventActorLoaded
  (CallFunction|MulticastRemoveGrassonLoad)
  (EventDispatchers|BindEventtoInitalizationFinished (delegate Custom|Initalization%20Finished_Event)))

(event EventActorPreSave
  (SaveData|SaveCropData))

(fn ConstructionScript
  (MeshSettings|CreateQuad)
  (Class|ProceduralMeshComponent|CreateMeshSectionLinearColor (Variables|Default|GetProceduralMesh) 0 (Variables|MeshSettings|GetVertexLocations) (Variables|MeshSettings|GetTriangles) (Variables|MeshSettings|GetNormals) (Variables|MeshSettings|GetUVs) 0 0 0 0 (Variables|MeshSettings|GetTangents) true)
  (Rendering|Material|SetMaterial (Variables|Default|GetProceduralMesh) 0 "/Game/Homestead/Environment/FieldSystem/MI_Field.MI_Field")
  (CropManagement|AddCropSnapPoints))

(fn SetMeshHeight
  (params (Location :type Vector) (X :type Integer) (Y :type Integer))
  (bind _returnvalue (Transformation|GetActorLocation))
  (bind (_x _y) (Math|Vector|BreakVector Location))
  (bind _self self)
  (bind _returnvalue_2 (Transformation|GetActorRotation _self))
  (bind _returnvalue_3 (Math|Trig|Cos(Degrees) (.yaw _returnvalue_2)))
  (bind _returnvalue_4 (Math|Trig|Sin(Degrees) (.yaw _returnvalue_2)))
  (bind _returnvalue_5 (* _y _returnvalue_3))
  (bind _returnvalue_6 (* _x _returnvalue_4))
  (bind _returnvalue_7 (* _x _returnvalue_3))
  (bind _returnvalue_8 (* _y _returnvalue_4))
  (bind _returnvalue_9 (- _returnvalue_7 _returnvalue_8))
  (bind _returnvalue_10 (+ _returnvalue_5 _returnvalue_6))
  (bind _returnvalue_11 (+ (Math|Vector|MakeVector _returnvalue_9 _returnvalue_10 0.0) _returnvalue))
  (bind (_outhit _returnvalue_12) (Collision|LineTraceForObjects (+ _returnvalue_11 (Math|Vector|MakeVector 0.0 0.0 5e+02)) (+ _returnvalue_11 (Math|Vector|MakeVector 0.0 0.0 -5e+02)) (Utilities|Array|MakeArray "ObjectTypeQuery1") true (Utilities|Array|MakeArray self) "None" true "(R=1.000000,G=0.000000,B=0.000000,A=1.000000)" "(R=0.000000,G=1.000000,B=0.000000,A=1.000000)" 1.0))
  (if _returnvalue_12
    (return (+ (Math|Transform|InverseTransformLocation (Transformation|GetActorTransform) (.location _outhit)) (Math|Vector|MakeVector 0.0 0.0 (MeshSettings|SelectHeightOffset X Y))))
    (else
      (return Location))))

(fn CreateQuad
  (bind _point_spread (Variables|MeshSettings|GetPoint%20Spread))
  (Utilities|Array|Clear (Variables|MeshSettings|GetNormals))
  (Utilities|Array|Clear (Variables|MeshSettings|GetVertexLocations))
  (Utilities|Array|Clear (Variables|MeshSettings|GetTriangles))
  (Utilities|Array|Clear (Variables|MeshSettings|GetUVs))
  (for _index (range 0 (Variables|MeshSettings|GetXPoints))
    (LocalVariables|SetX _index)
    (for _index_2 (range 0 (Variables|MeshSettings|GetYPoints))
      (LocalVariables|SetY _index_2)
      (Utilities|FlowControl|Sequence
        (:then_0
          ;[1 1 1] Make Vertex Locations
          (bind _hit_location__local_ (MeshSettings|SetMeshHeight (Math|Vector|MakeVector (* (LocalVariables|GetX) _point_spread) (* (LocalVariables|GetY) _point_spread) 0.0) (LocalVariables|GetX) (LocalVariables|GetY)))
          (Utilities|Array|Add (Variables|MeshSettings|GetVertexLocations) _hit_location__local_))
        (:then_1
          ;[1 1 1] Make UV Locations
          (Utilities|Array|Add (Variables|MeshSettings|GetUVs) (Math|Vector2D|MakeVector2D (/ (Math|Conversions|ToFloat(Integer) (LocalVariables|GetX)) (Math|Conversions|ToFloat(Integer) (Variables|MeshSettings|GetXPoints))) (/ (Math|Conversions|ToFloat(Integer) (LocalVariables|GetY)) (Math|Conversions|ToFloat(Integer) (Variables|MeshSettings|GetYPoints)))))))))
  (Utilities|FlowControl|Sequence
    (:then_0
      ;[1 1 1] Create Triangles
      (bind _triangles (Class|KismetProceduralMeshLibrary|CreateGridMeshTriangles (+ (Variables|MeshSettings|GetXPoints) 1) (+ (Variables|MeshSettings|GetYPoints) 1) true))
      (Variables|MeshSettings|SetTriangles _triangles))
    (:then_1
      ;[1 1 1] Create Tangents and Normals
      (Utilities|Array|Reverse (Variables|MeshSettings|GetTriangles))
      (bind (_normals _tangents) (Class|KismetProceduralMeshLibrary|CalculateTangentsforMesh (Variables|MeshSettings|GetVertexLocations) (Variables|MeshSettings|GetTriangles) (Variables|MeshSettings|GetUVs)))
      (Variables|MeshSettings|SetNormals _normals)
      (Variables|MeshSettings|SetTangents _tangents))))

(fn SelectHeightOffset
  (params (X :type Integer) (Y :type Integer))
  (return (select (or (or (== X 0) (== Y 0)) (or (== X (Variables|MeshSettings|GetXPoints)) (== Y (Variables|MeshSettings|GetYPoints)))) -2.0 (select (or (or (== X 1) (== Y 1)) (or (== Y (- (Variables|MeshSettings|GetXPoints) 1)) (== Y (- (Variables|MeshSettings|GetYPoints) 1)))) 1e+01 (select (or (or (== X 2) (== Y 2)) (or (== X (- (Variables|MeshSettings|GetXPoints) 2)) (== Y (- (Variables|MeshSettings|GetYPoints) 2)))) 1e+01 (select (or (or (== X 3) (== Y 3)) (or (== X (- (Variables|MeshSettings|GetXPoints) 3)) (== Y (- (Variables|MeshSettings|GetYPoints) 3)))) 1e+01 1e+01))))))

(fn SetGrassRemoved
  (params (Foliage%20Transforms :type Array%20of%20Transforms) (Foliage%20Components :type Array%20of%20Foliage%20Instanced%20Static%20Mesh%20Component%20Object%20References))
  (Variables|GrassManagement|SetFoliage%20Transforms Foliage%20Transforms)
  (Variables|GrassManagement|SetFoliage%20Components Foliage%20Components))

(fn ReturnGrass
  (for (_array_element _array_index) (Variables|GrassManagement|GetFoliage%20Components)
    (Class|InstancedStaticMeshComponent|AddInstanceWorldSpace _array_element (Utilities|Array|Get(acopy) (Variables|GrassManagement|GetFoliage%20Transforms) _array_index))))

(fn AddCropSnapPoints
  (bind _crop_spread (Variables|CropManagement|GetCrop%20Spread))
  (for _array_element (Variables|CropManagement|GetCop%20Snap%20Points)
    (Components|DestroyComponent _array_element))
  (Utilities|Array|Clear (Variables|CropManagement|GetCop%20Snap%20Points))
  (for _index (range 0 (Variables|CropManagement|GetCrop%20X%20Points))
    (LocalVariables|SetX _index)
    (for _index_2 (range 0 (Variables|CropManagement|GetCrop%20Y%20Points))
      (LocalVariables|SetY _index_2)
      (if (not (Math|Boolean|ORBoolean (== (LocalVariables|GetX) 0) (== (LocalVariables|GetX) (Variables|CropManagement|GetCrop%20X%20Points)) (== (LocalVariables|GetY) 0) (== (LocalVariables|GetY) (Variables|CropManagement|GetCrop%20Y%20Points))))
        (bind _hit_location__local_ (CropManagement|SetCropHeight (+ (Math|Vector|MakeVector (* (LocalVariables|GetX) _crop_spread) (* (LocalVariables|GetY) _crop_spread) 0.0) "0.000000,10.000000, 0")))
        (bind _returnvalue (Game|AddComponentbyClass "/Game/SRPG/Blueprints/BuildSystem/BPC_SnapPointSpawn.BPC_SnapPointSpawn_C" false (Math|Transform|MakeTransform _hit_location__local_ "0, 0, 0" "1,1,1") (Utilities|Array|MakeArray "BTE_Crop")))
        (Utilities|Array|Add (Variables|CropManagement|GetCop%20Snap%20Points) _returnvalue)))))

(fn SetCropHeight
  (params (Location :type Vector))
  (bind _returnvalue (Transformation|GetActorLocation))
  (bind (_x _y) (Math|Vector|BreakVector Location))
  (bind _self self)
  (bind _returnvalue_2 (Transformation|GetActorRotation _self))
  (bind _returnvalue_3 (Math|Trig|Cos(Degrees) (.yaw _returnvalue_2)))
  (bind _returnvalue_4 (Math|Trig|Sin(Degrees) (.yaw _returnvalue_2)))
  (bind _returnvalue_5 (* _y _returnvalue_3))
  (bind _returnvalue_6 (* _x _returnvalue_4))
  (bind _returnvalue_7 (* _x _returnvalue_3))
  (bind _returnvalue_8 (* _y _returnvalue_4))
  (bind _returnvalue_9 (- _returnvalue_7 _returnvalue_8))
  (bind _returnvalue_10 (+ _returnvalue_5 _returnvalue_6))
  (bind _returnvalue_11 (+ (Math|Vector|MakeVector _returnvalue_9 _returnvalue_10 0.0) _returnvalue))
  (bind (_outhit _returnvalue_12) (Collision|LineTraceForObjects (+ _returnvalue_11 (Math|Vector|MakeVector 0.0 0.0 5e+02)) (+ _returnvalue_11 (Math|Vector|MakeVector 0.0 0.0 -5e+02)) (Utilities|Array|MakeArray "ObjectTypeQuery1") true 0 "None" false "(R=1.000000,G=0.000000,B=0.000000,A=1.000000)" "(R=0.000000,G=1.000000,B=0.000000,A=1.000000)" 1.0))
  (if _returnvalue_12
    (return (Math|Transform|InverseTransformLocation (Transformation|GetActorTransform) (.location _outhit)))
    (else
      (return Location))))

(fn RemoveGrassonLoad
  (bind _outactors (Actor|GetAllActorsOfClass "/Script/Foliage.InstancedFoliageActor"))
  (for _array_element (Actor|GetComponentsByClass (Utilities|Array|Get(acopy) _outactors) "/Game/Homestead/Blueprints/FoliageSpawners/TemperateGrass/BPC_GrassFoliage.BPC_GrassFoliage_C")
    (for _array_element_2 (Variables|CropManagement|GetCop%20Snap%20Points)
      (LocalVariables|SetInstances (Class|InstancedStaticMeshComponent|GetInstancesOverlappingSphere _array_element (Transformation|GetWorldLocation _array_element_2) 1e+02 true))
      (for _array_element_3 (LocalVariables|GetInstances)
        (Utilities|Array|Add (Variables|GrassManagement|GetFoliage%20Components) _array_element)
        (Utilities|Array|Add (Variables|GrassManagement|GetFoliage%20Transforms) (.OutInstanceTransform (Components|InstancedStaticMesh|GetInstanceTransform _array_element _array_element_3 true))))
      (for _array_element_4 (LocalVariables|GetInstances)
        (Components|InstancedStaticMesh|UpdateInstanceTransform _array_element _array_element_4 (Math|Transform|MakeTransform "0, 0,-7000.000000" "0, 0, 0" "0.000000,0.000000,0.000000") false false false)))))

(fn CheckinCrop
  (params (New%20Crop :type BP%20Field%20Crop%20Object%20Reference))
  (Utilities|Array|AddUnique (Variables|CropManagement|GetMy%20Crops) New%20Crop))

(fn CheckOutCrop
  (params (Deleted%20Crop :type BP%20Field%20Crop%20Object%20Reference))
  (Utilities|Array|RemoveItem (Variables|CropManagement|GetMy%20Crops) Deleted%20Crop))

(fn SaveCropData
  (Utilities|Array|Clear (Variables|SaveData|GetCrop%20Class%20Save%20Data))
  (Utilities|Array|Clear (Variables|SaveData|GetCrop%20Transform%20Save%20Data))
  (Utilities|Array|Clear (Variables|SaveData|GetCrop%20Data))
  (Utilities|Array|Clear (Variables|SaveData|GetCrop%20Gene%20Data))
  (for _array_element (Variables|CropManagement|GetMy%20Crops)
    (Utilities|Array|Add (Variables|SaveData|GetCrop%20Class%20Save%20Data) (Utilities|GetClass _array_element))
    (Utilities|Array|Add (Variables|SaveData|GetCrop%20Transform%20Save%20Data) (Transformation|GetActorTransform _array_element))
    (bind _returnvalue (Class|Crop|GetCropSaveData _array_element))
    (Utilities|Array|Add (Variables|SaveData|GetCrop%20Data) _returnvalue)
    (Utilities|Array|Add (Variables|SaveData|GetCrop%20Gene%20Data) (Class|Crop|GetGeneData _array_element))))

(fn LoadCrops
  (for (_array_element _array_index) (Variables|SaveData|GetCrop%20Class%20Save%20Data)
    (bind _returnvalue (Game|SpawnActorfromClass _array_element (Utilities|Array|Get(acopy) (Variables|SaveData|GetCrop%20Transform%20Save%20Data) _array_index) "Undefined" 0 self 0))
    (Class|Crop|LoadCropSaveData _returnvalue (Utilities|Array|Get(acopy) (Variables|SaveData|GetCrop%20Data) _array_index) (Utilities|Array|Get(acopy) (Variables|SaveData|GetCrop%20Gene%20Data) _array_index))))

(fn ComponentstoSave
  (return 0))