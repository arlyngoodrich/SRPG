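; Crop spawner that acts as a short-lived, server-authoritative stand-in for planting a seed on a field.
; When its spawn finishes, it registers with BP_ItemManager, which calls back PlantSeed with the plant's genetic data.
; PlantSeed resolves the parent BP_Field from its snap point, spawns the configured crop there with random yaw, passes on field and genes, then expires.
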(event Custom|Plant%20Seed
  (params (Plant%20Genetic%20Data :type Crop%20Gene%20Data%20Structure))
  (bind _returnvalue (Transformation|GetActorTransform))
  (bind _snap_point (Variables|Default|GetSnap%20Point))
  (Networking|SwitchHasAuthority
    (:Authority
      (Utilities|IsValid _snap_point
        (:Is%20Valid
          (bind _asbp_field (Utilities|Casting|CastToBP_Field (Variables|/Game/SRPG/Blueprints/BuildSystem/BP_SnapPointActor.BP_SnapPointActor_C|GetMy%20Parent _snap_point)))
          (Variables|Default|SetMy%20Field _asbp_field)
          (bind _returnvalue_2 (Game|SpawnActorfromClass (Variables|Default|GetCrop%20to%20Spawn) (Math|Transform|MakeTransform (.location _returnvalue) (Math|Rotator|MakeRotator (.roll (.rotation _returnvalue)) (.pitch (.rotation _returnvalue)) (Math|Random|RandomFloatinRange -1.8e+02 1.8e+02)) (.scale _returnvalue)) "Undefined" 0 (Variables|Default|GetMy%20Field) 0))
          (Class|Crop|SetGenes _returnvalue_2 Plant%20Genetic%20Data)
          (Actor|SetLifeSpan 0.1))))))

(event EventOnSpawnFinished
  (Networking|SwitchHasAuthority
    (:Authority
      (bind _outactors (Actor|GetAllActorsOfClass "/Game/SRPG/Blueprints/ItemSystem/BP_ItemManager.BP_ItemManager_C"))
      (Utilities|IsValid (Utilities|Array|Get(acopy) _outactors)
        (:Is%20Valid
          (bind _output_get (Variables|Default|SetItem%20Manager (Utilities|Array|Get(acopy) _outactors)))
          (Default|OnCropSpawnerSet _output_get self))
        (:Is%20Not%20Valid
          (Development|PrintString "No Valid Item Manager"))))))

(fn ConstructionScript
  (|CallParentFunction))