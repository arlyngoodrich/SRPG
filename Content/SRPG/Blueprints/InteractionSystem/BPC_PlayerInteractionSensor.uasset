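; Player interaction sensor component that finds the interactable object the player's camera is looking at.
; A looping timer runs a Visibility line trace from the camera manager along its forward vector, with optional debug drawing.
; It tracks the hit actor that has an interactable object component, firing start and end focus calls as the target changes or is lost.
; Interact triggers the interaction on the currently focused object's component.
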(event EventBeginPlay
  (CallFunction|Initalize)
  (Utilities|Time|SetTimerbyFunctionName self "Check for Interactable" (Variables|Configuration|GetCheck%20Frequency) true))

(fn Initalize
  (bind _ascharacter (Utilities|Casting|CastToCharacter (Components|GetOwner)))
  (bind _output_get (Variables|References|SetOwningCharacter _ascharacter))
  (bind _asplayer_controller (Utilities|Casting|CastToPlayerController (Pawn|GetController _output_get)))
  (Variables|References|SetPlayerCameraManager (Variables|/Script/Engine.PlayerController|GetPlayerCameraManager _asplayer_controller)))

(fn CheckforInteractable
  (bind _playercameramanager (Variables|References|GetPlayerCameraManager))
  (bind _returnvalue (Camera|GetCameraLocation _playercameramanager))
  (Utilities|IsValid _playercameramanager
    (:Is%20Valid
      (bind _outhit (Collision|LineTraceByChannel _returnvalue (+ _returnvalue (* (Transformation|GetActorForwardVector _playercameramanager) (Variables|Configuration|GetView%20Distance))) "TraceTypeQuery1" true 0 (select (Variables|Configuration|GetDebug) "ForDuration" "None") true "(R=1.000000,G=0.000000,B=0.000000,A=1.000000)" "(R=0.000000,G=1.000000,B=0.000000,A=1.000000)" (Variables|Configuration|GetCheck%20Frequency)))
      (if (.bBlockingHit (Collision|BreakHitResult _outhit))
        (bind _output_get (LocalVariables|SetHit%20Actor (.HitActor (Collision|BreakHitResult _outhit))))
        (if (.Valid%20Interactable (Utilities|GetActorInteractableComponent _output_get))
          (if (not (== (Variables|References|GetInteractable%20In%20View) (LocalVariables|GetHit%20Actor)))
            (Utilities|IsValid (Variables|References|GetInteractable%20In%20View)
              (:Is%20Valid
                (Default|OnEndFocus (.Output (Utilities|GetActorInteractableComponent (Variables|References|GetInteractable%20In%20View)))))
              (:Is%20Not%20Valid
                _))
            (bind _output_get_2 (Variables|References|SetInteractable%20In%20View (LocalVariables|GetHit%20Actor)))
            (Default|OnStartFocus (.Output (Utilities|GetActorInteractableComponent _output_get_2))))
          (else
            ;[1 1 1] If view gets no hit, interacatble set to null
            (Utilities|IsValid (Variables|References|GetInteractable%20In%20View) :!label _label
              (:Is%20Valid
                (Default|OnEndFocus (.Output (Utilities|GetActorInteractableComponent (Variables|References|GetInteractable%20In%20View))))
                (Variables|References|SetInteractable%20In%20View 0)))))
        (else
          (goto _label))))))

(fn Interact
  (bind _interactable_in_view (Variables|References|GetInteractable%20In%20View)
    (:then
      (if (.Valid%20Interactable (Utilities|GetActorInteractableComponent _interactable_in_view))
        (Class|PlayerInteractionSensor|TriggerInteraction (.Output (Utilities|GetActorInteractableComponent _interactable_in_view)))))
    (:else)))