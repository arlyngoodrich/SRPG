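; Component that makes its owning actor interactable, showing a prompt and optional outline while in focus.
; Focus start adds a WBP_InteractionText widget and, if ShouldOutline, sets custom depth stencil on the owner's static meshes cached at BeginPlay.
; Focus end clears the outline but removes the prompt only when Debug is set; EndPlay also removes it.
; InteractionTriggered passes on calls from a BPC_PlayerInteractionSensor through CallInteractionTriggered.
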(event EventBeginPlay
  (CallFunction|Initalize))

(event EventInteractionTriggered
  (params (InstigatingComponent :type Player%20Interaction%20Sensor%20Object%20Reference))
  (bind _asbpc_player_interaction_sensor (Utilities|Casting|CastToBPC_PlayerInteractionSensor InstigatingComponent))
  (Default|CallInteractionTriggered _asbpc_player_interaction_sensor))

(event EventEndPlay
  (params (EndPlayReason :type EEndPlayReason%20Enum :default "Destroyed"))
  (bind _interactionui (Variables|Referecnes|GetInteractionUI))
  (Utilities|IsValid _interactionui
    (:Is%20Valid
      (Widget|RemovefromParent _interactionui))))

(fn OnStartFocus
  (Development|PrintString (Utilities|String|Append (Utilities|GetDisplayName (Components|GetOwner)) " is in focus") false true "(R=0.000000,G=0.660000,B=1.000000,A=1.000000)" 1.0)
  (if (Variables|InteractionConfig|GetShould%20Outline)
    (CallFunction|StartOutline))
  (if true
    (bind _returnvalue (UserInterface|CreateWidget "/Game/SRPG/Blueprints/InteractionSystem/WBP_InteractionText.WBP_InteractionText_C" 0 (Variables|InteractionConfig|GetInteraction%20Prompt)))
    (bind _output_get (Variables|Referecnes|SetInteractionUI _returnvalue))
    (UserInterface|Viewport|AddtoViewport _output_get 0)))

(fn OnEndFocus
  (bind _interactionui (Variables|Referecnes|GetInteractionUI))
  (Development|PrintString (Utilities|String|Append (Utilities|GetDisplayName (Components|GetOwner)) " is not in focus") false true "(R=0.000000,G=0.660000,B=1.000000,A=1.000000)" 1.0)
  (if (Variables|InteractionConfig|GetDebug)
    (Utilities|IsValid _interactionui
      (:Is%20Valid
        (Widget|RemovefromParent _interactionui))
      (:Is%20Not%20Valid
        _)))
  (if (Variables|InteractionConfig|GetShould%20Outline)
    (CallFunction|EndOutline)))

(fn StartOutline
  (for _array_element (Variables|InteractionConfig|GetOwner%20Static%20Meshes)
    (Rendering|SetRenderCustomDepth _array_element true)
    (Rendering|SetCustomDepthStencilValue _array_element (Variables|InteractionConfig|GetOutline%20Stencil))))

(fn Initalize
  (bind _output_get (Variables|Referecnes|SetOwner (Components|GetOwner)))
  (Variables|InteractionConfig|SetOwner%20Static%20Meshes (Actor|GetComponentsByClass _output_get "/Script/Engine.StaticMeshComponent")))

(fn EndOutline
  (for _array_element (Variables|InteractionConfig|GetOwner%20Static%20Meshes)
    (Rendering|SetRenderCustomDepth _array_element false)
    (Rendering|SetCustomDepthStencilValue _array_element 1)))