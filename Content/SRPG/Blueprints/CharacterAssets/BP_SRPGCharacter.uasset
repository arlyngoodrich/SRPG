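; Player character for an SRPG with modular body meshes following the main mesh pose, interaction, and inventory and build menus.
; Input events forward to components and dispatchers, while menu toggles manage widgets and cursor.
; On authority, save hooks flatten inventory containers into parallel arrays by equipment slot, and loading rebuilds nested abstract inventories by pair ID.
; The pair ID generator is a stub returning zero; K and L trigger save and load.
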(event EventActorPreSave
  (Networking|SwitchHasAuthority
    (:Authority
      (SaveData|SaveData))))

(event EventActorLoaded
  (Networking|SwitchHasAuthority
    (:Authority
      (Utilities|FlowControl|Delay 0.2)
      (SaveData|LoadInventoryData))))

(event EventBeginPlay
  ;[1 1 1] Initalization
  (CallFunction|Initalize))

(event Input|KeyboardEvents|K
  (params (Key :type Key%20Structure :default "None"))
  (:Pressed
    (|AsyncSaveActors 3
      (:OnCompleted
        (Development|PrintString "Saved")))))

(event Input|KeyboardEvents|L
  (params (Key :type Key%20Structure :default "None"))
  (:Pressed
    (Utilities|Platform|CollectGarbage)
    (|AsyncLoadActors 3 true
      (:OnCompleted
        (Development|PrintString "Loaded")))))

(event Custom|Multicast_Toggle%20Menu
  (params (Menu :type User%20Widget%20Object%20Reference))
  (bind _player_controller (Variables|Components|GetPlayer%20Controller))
  (bind _player_controller_2 (Variables|Components|GetPlayer%20Controller))
  ;[1 1 1] Toggle Inventory Menu
  (Utilities|IsValid (Variables|UI|GetActive%20Widget)
    (:Is%20Valid
      (if (== Menu (Variables|UI|GetActive%20Widget))
        (Variables|UI|SetActive%20Widget Menu :!label _label)
        (Utilities|FlowControl|FlipFlop
          (:A
            (Default|CallMenuOpen)
            (Utilities|IsValid (Variables|UI|GetActive%20Widget)
              (:Is%20Valid
                (UserInterface|Viewport|AddtoViewport (Variables|UI|GetActive%20Widget) 0)
                (Input|SetInputModeGameandUI _player_controller_2 (Variables|UI|GetActive%20Widget) "DoNotLock" true)
                (Variables|/Script/Engine.PlayerController|SetbShowMouseCursor _player_controller_2 true))))
          (:B
            (Default|CallMenuClosed)
            (Utilities|IsValid (Variables|UI|GetActive%20Widget)
              (:Is%20Valid
                (Widget|RemovefromParent (Variables|UI|GetActive%20Widget))
                (Input|SetInputModeGameOnly _player_controller)
                (Variables|/Script/Engine.PlayerController|SetbShowMouseCursor _player_controller false)
                (Variables|UI|SetActive%20Widget 0)))))))
    (:Is%20Not%20Valid
      (goto _label))))

(event Custom|Toggle%20Player%20Menu
  (bind _player_controller (Variables|Components|GetPlayer%20Controller))
  (bind _player_controller_2 (Variables|Components|GetPlayer%20Controller))
  ;[1 1 1] Toggle Inventory Menu
  (Utilities|IsValid (Variables|UI|GetActive%20Widget)
    (:Is%20Valid
      _)
    (:Is%20Not%20Valid
      (Variables|UI|SetActive%20Widget (Variables|UI|GetPlayer%20Menu%20Widget))))
  (Utilities|FlowControl|FlipFlop
    (:A
      (Default|CallMenuOpen)
      (Utilities|IsValid (Variables|UI|GetActive%20Widget)
        (:Is%20Valid
          (UserInterface|Viewport|AddtoViewport (Variables|UI|GetActive%20Widget) 0)
          (Input|SetInputModeGameandUI _player_controller_2 (Variables|UI|GetActive%20Widget) "DoNotLock" true)
          (Variables|/Script/Engine.PlayerController|SetbShowMouseCursor _player_controller_2 true))))
    (:B
      (Default|CallMenuClosed)
      (Utilities|IsValid (Variables|UI|GetActive%20Widget)
        (:Is%20Valid
          (Widget|RemovefromParent (Variables|UI|GetActive%20Widget))
          (Input|SetInputModeGameOnly _player_controller)
          (Variables|/Script/Engine.PlayerController|SetbShowMouseCursor _player_controller false)
          (Variables|UI|SetActive%20Widget 0))))))

(event Input|ActionEvents|InputActionToggleInventory
  (params (Key :type Key%20Structure))
  (bind _player_controller (Variables|Components|GetPlayer%20Controller))
  (bind _player_controller_2 (Variables|Components|GetPlayer%20Controller))
  ;[1 1 1] Toggle Inventory Menu
  (:Pressed
    (Utilities|IsValid (Variables|UI|GetActive%20Widget)
      (:Is%20Valid
        _)
      (:Is%20Not%20Valid
        (Variables|UI|SetActive%20Widget (Variables|UI|GetPlayer%20Menu%20Widget))))
    (Utilities|FlowControl|FlipFlop
      (:A
        (Default|CallMenuOpen)
        (Utilities|IsValid (Variables|UI|GetActive%20Widget)
          (:Is%20Valid
            (UserInterface|Viewport|AddtoViewport (Variables|UI|GetActive%20Widget) 0)
            (Input|SetInputModeGameandUI _player_controller_2 (Variables|UI|GetActive%20Widget) "DoNotLock" true)
            (Variables|/Script/Engine.PlayerController|SetbShowMouseCursor _player_controller_2 true))))
      (:B
        (Default|CallMenuClosed)
        (Utilities|IsValid (Variables|UI|GetActive%20Widget)
          (:Is%20Valid
            (Widget|RemovefromParent (Variables|UI|GetActive%20Widget))
            (Input|SetInputModeGameOnly _player_controller)
            (Variables|/Script/Engine.PlayerController|SetbShowMouseCursor _player_controller false)
            (Variables|UI|SetActive%20Widget 0)))))))

(event Input|ActionEvents|InputActionUseSlot2
  (params (Key :type Key%20Structure))
  ;[1 1 1] Slots
  (:Pressed
    (Default|CallSlot2)))

(event Input|ActionEvents|InputActionInteract
  (params (Key :type Key%20Structure))
  ;[1 1 1] Interaction
  (:Pressed
    (Default|Interact (Variables|Default|GetBPC_PlayerInteractionSensor) (Variables|UI|GetInteractionIndex))))

(event Input|ActionEvents|InputActionPrimary
  (params (Key :type Key%20Structure))
  ;[1 1 1] RMD and LMB
  (:Pressed
    (Default|CallPrimaryPressed)))

(event Input|ActionEvents|InputActionSecondary
  (params (Key :type Key%20Structure))
  ;[1 1 1] RMD and LMB
  (:Pressed
    (Default|CallSecondaryPressed)))

(event Input|ActionEvents|InputActionUseSlot1
  (params (Key :type Key%20Structure))
  ;[1 1 1] Slots
  (:Pressed
    (Default|CallSlot1)))

(event Input|ActionEvents|InputActionRotateItem
  (params (Key :type Key%20Structure))
  ;[1 1 1] Rotate Pressed
  (:Pressed
    (Default|PlayerPressedRotate (Variables|Default|GetBPC_PlayerInventoryManager))
    (Default|CallRotatePressed)))

(event Input|ActionEvents|InputActionUseSlot3
  (params (Key :type Key%20Structure))
  ;[1 1 1] Slots
  (:Pressed
    (Default|CallSlot3)))

(event Input|KeyboardEvents|B
  (params (Key :type Key%20Structure))
  (bind _player_controller (Variables|Components|GetPlayer%20Controller))
  ;[1 1 1] Build Menu
  (:Pressed
    (Utilities|FlowControl|FlipFlop
      (:A
        (UserInterface|Viewport|AddtoViewport (Variables|UI|GetBuild%20Menu%20Widget) 0)
        (Variables|/Script/Engine.PlayerController|SetbShowMouseCursor _player_controller true)
        (Default|CallMenuOpen))
      (:B
        (Widget|RemovefromParent (Variables|UI|GetBuild%20Menu%20Widget))
        (Variables|/Script/Engine.PlayerController|SetbShowMouseCursor _player_controller false)
        (Default|CallMenuClosed)))))

(event Input|KeyboardEvents|LeftShift
  (params (Key :type Key%20Structure))
  ;[1 1 1] Left Shit
  (:Pressed
    (Default|CallShiftDown))
  (:Released
    (Default|CallShiftUp)))

(event Input|MouseEvents|MouseWheelUp
  (params (Key :type Key%20Structure))
  ;[1 1 1] Mouse Wheel
  (:Pressed
    (Default|CallMouseWheelUp)))

(event Input|MouseEvents|MouseWheelDown
  (params (Key :type Key%20Structure))
  ;[1 1 1] Mouse Wheel
  (:Pressed
    (Default|CallMouseWheelDown)))

(fn ConstructionScript
  (Class|SkinnedMeshComponent|SetMasterPoseComponent (Variables|Default|GetHead) (Variables|Character|GetMesh) false))

(fn Initalize
  (bind _asplayer_controller (Utilities|Casting|CastToPlayerController (Pawn|GetController)))
  (bind _output_get (Variables|Components|SetPlayer%20Controller _asplayer_controller))
  (bind _returnvalue (UserInterface|CreateWidget "/Game/SRPG/Blueprints/MenuSystem/CharacterMenu/WBP_PlayerMenuContainer.WBP_PlayerMenuContainer_C" _output_get))
  (Variables|UI|SetPlayer%20Menu%20Widget _returnvalue)
  (bind _returnvalue_2 (UserInterface|CreateWidget "/Game/SRPG/Blueprints/BuildSystem/WBP_BuildingMenu.WBP_BuildingMenu_C" 0 self (Variables|Default|GetBPC_PlayerBuildManager)))
  (Variables|UI|SetBuild%20Menu%20Widget _returnvalue_2))

(fn SetInteractionIndex
  (params (Interaction%20Menu :type WBP%20Interaction%20Menu%20Object%20Reference) (Index :type Integer))
  (Variables|UI|SetInteraction%20Menu Interaction%20Menu)
  (Variables|UI|SetInteractionIndex Index))

(fn SaveData
  ;[1 1 1] Clear Previously Saved Data
  (Utilities|Array|Clear (Variables|SaveData|Inventory|GetSaved%20Abstract%20Inventory%20Data))
  (Utilities|Array|Clear (Variables|SaveData|Inventory|GetSaved%20Inventory%20Data))
  (Utilities|Array|Clear (Variables|SaveData|Inventory|GetAbstract%20Inventory%20Data%20Pair%20ID))
  (Utilities|Array|Clear (Variables|SaveData|Inventory|GetHas%20Abstract%20Inventory))
  (Utilities|Array|Clear (Variables|SaveData|Inventory|GetEquipment%20Slot))
  (for _array_element (Actor|GetComponentsByClass "/Game/SRPG/Blueprints/InventorySystem/BPC_InventoryContainer.BPC_InventoryContainer_C")
    (bind _outinventorydata (Class|InventoryContainer|GetInventoryforAbstract _array_element))
    (for _array_element_2 _outinventorydata
      (Utilities|IsValid (Utilities|Struct|BreakItemData (.ItemData (Utilities|Struct|BreakInventoryItemData _array_element_2))) ; Save Abstract Inventory IF VALID
        (:Is%20Valid
          ;[1 1 1] Save Inventory Data with abstract inventory
          (LocalVariables|SetAbstract%20Pair%20ID (SaveData|CreateUniquePairID))
          (bind _outinventory (Class|AbstractInventoryContainer|GetInventory (Utilities|Struct|BreakItemData (.ItemData (Utilities|Struct|BreakInventoryItemData _array_element_2)))))
          (for _array_element_3 _outinventory
            (Utilities|Array|Add (Variables|SaveData|Inventory|GetAbstract%20Inventory%20Data%20Pair%20ID) (LocalVariables|GetAbstract%20Pair%20ID))
            (Utilities|Array|Add (Variables|SaveData|Inventory|GetSaved%20Abstract%20Inventory%20Data) _array_element_3))
          (bind _structout (Utilities|Struct|SetmembersinItemData (.ItemData (Utilities|Struct|BreakInventoryItemData _array_element_2)) (LocalVariables|GetAbstract%20Pair%20ID)))
          (Utilities|Array|Add (Variables|SaveData|Inventory|GetHas%20Abstract%20Inventory) true)
          (Utilities|Array|Add (Variables|SaveData|Inventory|GetSaved%20Inventory%20Data) (Utilities|Struct|MakeInventoryItemData _structout (.Position (Utilities|Struct|BreakInventoryItemData _array_element_2))))
          (Utilities|Array|Add (Variables|SaveData|Inventory|GetEquipment%20Slot) (Variables|/Script/SRPG.InventoryContainer|GetEquippedSlot _array_element)))
        (:Is%20Not%20Valid
          ;[1 1 1] Save Inventory data for no abstract Inventory
          (Utilities|Array|Add (Variables|SaveData|Inventory|GetHas%20Abstract%20Inventory) false)
          (Utilities|Array|Add (Variables|SaveData|Inventory|GetSaved%20Inventory%20Data) _array_element_2)
          (Utilities|Array|Add (Variables|SaveData|Inventory|GetEquipment%20Slot) (Variables|/Script/SRPG.InventoryContainer|GetEquippedSlot _array_element))
          (Development|PrintString (Utilities|String|Append (Utilities|String|ToString(Name) (.DisplayName (Utilities|Struct|BreakItemData (.ItemData (Utilities|Struct|BreakInventoryItemData _array_element_2))))) " saved")))))))

(fn LoadInventoryData
  (for _array_element (Actor|GetComponentsByClass "/Game/SRPG/Blueprints/InventorySystem/BPC_InventoryContainer.BPC_InventoryContainer_C")
    (Utilities|Array|Clear (LocalVariables|GetTemp%20Inventory%20Data))
    (for (_array_element_2 _array_index) (Variables|SaveData|Inventory|GetEquipment%20Slot)
      (if (Utilities|Enum|Equal(Enum) _array_element_2 (Variables|/Script/SRPG.InventoryContainer|GetEquippedSlot _array_element))
        (if (Utilities|Array|Get(acopy) (Variables|SaveData|Inventory|GetHas%20Abstract%20Inventory) _array_index)
          ;[1 1 1] Create abstract inventories and add back to items
          (Utilities|Array|Clear (LocalVariables|GetTemp%20Abstract%20Inventory%20Data))
          (for (_array_element_3 _array_index_2) (Variables|SaveData|Inventory|GetAbstract%20Inventory%20Data%20Pair%20ID)
            (if (== (Utilities|Struct|BreakItemData (.ItemData (Utilities|Struct|BreakInventoryItemData (Utilities|Array|Get(acopy) (Variables|SaveData|Inventory|GetSaved%20Inventory%20Data) _array_index)))) _array_element_3)
              (Utilities|Array|Add (LocalVariables|GetTemp%20Abstract%20Inventory%20Data) (Utilities|Array|Get(acopy) (Variables|SaveData|Inventory|GetSaved%20Abstract%20Inventory%20Data) _array_index_2))))
          (bind _returnvalue (Game|ConstructObjectfromClass "/Game/SRPG/Blueprints/InventorySystem/BP_AbstractInventoryContainer.BP_AbstractInventoryContainer_C" self))
          (bind _output_get (LocalVariables|SetAbstract%20Inventory _returnvalue))
          (Class|AbstractInventoryContainer|SetInventory _output_get (LocalVariables|GetTemp%20Abstract%20Inventory%20Data))
          (bind _structout (Utilities|Struct|SetmembersinItemData (.ItemData (Utilities|Struct|BreakInventoryItemData (Utilities|Array|Get(acopy) (Variables|SaveData|Inventory|GetSaved%20Inventory%20Data) _array_index))) (LocalVariables|GetAbstract%20Inventory)))
          (Utilities|Array|Add (LocalVariables|GetTemp%20Inventory%20Data) (Utilities|Struct|MakeInventoryItemData _structout (.Position (Utilities|Struct|BreakInventoryItemData (Utilities|Array|Get(acopy) (Variables|SaveData|Inventory|GetSaved%20Inventory%20Data) _array_index)))))
          (else
            (Utilities|Array|Add (LocalVariables|GetTemp%20Inventory%20Data) (Utilities|Array|Get(acopy) (Variables|SaveData|Inventory|GetSaved%20Inventory%20Data) _array_index))))))
    (Class|InventoryContainer|SetInventoryfromAbstract _array_element (LocalVariables|GetTemp%20Inventory%20Data))))

(fn CreateUniquePairID
  (return 0))

(fn ComponentstoSave
  (return 0))