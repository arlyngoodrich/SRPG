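; BP_StorageBase is a base interactable storage actor that lets one character at a time open its inventory container.
; Interaction claims the actor by setting its owner and disables that character's movement; further interactions from the owner toggle storage.
; The InteractingCharacter RepNotify binds the local player's menu open/close events to create or remove WBP_StorageUI.
; Closing clears the owner and restores walking.
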(event Custom|Interaction%20Triggered
  (params (Player%20Interaction%20Sensor :type BPC%20Player%20Interaction%20Sensor%20Object%20Reference))
  (bind _returnvalue (Components|GetOwner))
  (bind _owningcharacter (Variables|/Game/SRPG/Blueprints/InteractionSystem/BPC_PlayerInteractionSensor.BPC_PlayerInteractionSensor_C|GetOwningCharacter Player%20Interaction%20Sensor))
  (if (== _returnvalue 0)
    (Actor|SetOwner _owningcharacter)
    (bind _asbp_srpgcharacter (Utilities|Casting|CastToBP_SRPGCharacter _owningcharacter))
    (Variables|References|SetInteracting%20Character _asbp_srpgcharacter)
    (Pawn|Components|CharacterMovement|DisableMovement (Variables|/Script/Engine.Character|GetCharacterMovement (Variables|References|GetInteracting%20Character)))
    (elif (== _owningcharacter _returnvalue)
      (Default|ToggleStorage (Variables|References|GetInteracting%20Character)))))

(event Custom|Client%20Add%20Storage%20UI
  (bind _interacting_character (Variables|References|GetInteracting%20Character))
  (bind _interacting_character_2 (Variables|References|GetInteracting%20Character))
  (Utilities|IsValid _interacting_character
    (:Is%20Valid
      (if (Pawn|IsLocallyControlled _interacting_character)
        (EventDispatchers|BindEventtoMenuOpen _interacting_character_2 (delegate Custom|Open%20Storage%20UI))
        (EventDispatchers|BindEventtoMenuClosed _interacting_character_2 (delegate Custom|Remove%20Stroage%20UI))
        (Default|ToggleStorage _interacting_character_2)))))

(event Custom|Open%20Storage%20UI
  (bind _returnvalue (UserInterface|CreateWidget "/Game/SRPG/Blueprints/ItemSystem/WBP_StorageUI.WBP_StorageUI_C" 0 (Variables|Default|GetBPC_InventoryContainer)))
  (bind _output_get (Variables|References|SetStorage%20UI _returnvalue))
  (Default|Initalize _output_get)
  (UserInterface|Viewport|AddtoViewport (Variables|References|GetStorage%20UI) 0))

(event Custom|Remove%20Stroage%20UI
  (bind _interacting_character (Variables|References|GetInteracting%20Character))
  (if (Pawn|IsLocallyControlled _interacting_character)
    (Widget|RemovefromParent (Variables|References|GetStorage%20UI))
    (CallFunction|ClearOwner)
    (EventDispatchers|UnbindallEventsfromMenuClosed _interacting_character)
    (EventDispatchers|UnbindallEventsfromMenuOpen _interacting_character)))

(event Custom|Clear%20Owner
  (Actor|SetOwner 0)
  (Pawn|Components|CharacterMovement|SetMovementMode (Variables|/Script/Engine.Character|GetCharacterMovement (Variables|References|GetInteracting%20Character)) "MOVE_Walking" 0))

(event EventBeginPlay
  (EventDispatchers|BindEventtoInteractionTriggered (Variables|Default|GetBPC_InteractableObjectComponent) (delegate Custom|Interaction%20Triggered)))

(fn ConstructionScript)

(fn OnRepInteractingCharacter
  (CallFunction|ClientAddStorageUI))