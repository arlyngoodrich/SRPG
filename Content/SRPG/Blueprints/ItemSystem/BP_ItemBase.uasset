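; BP_ItemBase is a base world item that characters pick up into their inventory.
; Sphere overlap or the interactable component's trigger event both call PickupTriggered with the instigating actor.
; That function auto-adds ItemData to the actor's InventoryContainer, if present.
; The item destroys itself when the leftover flag is true and otherwise updates to the remaining item, which looks inverted given the flag's name.
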(event OnComponentBeginOverlap(Sphere)
  (params (OverlappedComponent :type Primitive%20Component%20Object%20Reference) (OtherActor :type Actor%20Object%20Reference) (OtherComp :type Primitive%20Component%20Object%20Reference) (OtherBodyIndex :type Integer) (bFromSweep :type Boolean) (SweepResult :type Hit%20Result%20Structure%20%28by%20ref%29))
  (CallFunction|PickupTriggered OtherActor))

(event Custom|On%20Interaction%20Triggered
  (params (Player%20Interaction%20Sensor :type BPC%20Player%20Interaction%20Sensor%20Object%20Reference))
  (CallFunction|PickupTriggered (Variables|/Game/SRPG/Blueprints/InteractionSystem/BPC_PlayerInteractionSensor.BPC_PlayerInteractionSensor_C|GetOwningCharacter Player%20Interaction%20Sensor)))

(event EventBeginPlay
  (EventDispatchers|BindEventtoInteractionTriggered (Variables|Default|GetBPC_InteractableObjectComponent) (delegate Custom|On%20Interaction%20Triggered)))

(fn ConstructionScript)

(fn PickupTriggered
  (params (Instigating%20Actor :type Actor%20Object%20Reference))
  (bind _returnvalue (Actor|GetComponentbyClass Instigating%20Actor "/Script/SRPG.InventoryContainer"))
  (Utilities|IsValid _returnvalue
    (:Is%20Valid
      (bind (_outbhasleftover _outremainingitem) (Class|InventoryContainer|AutoAddItem _returnvalue (Variables|Default|GetItemData)))
      (if _outbhasleftover
        (Actor|DestroyActor)
        (else
          (Class|ItemBase|UpdateItemInformation _outremainingitem))))))