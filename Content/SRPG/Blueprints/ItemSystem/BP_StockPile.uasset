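; BP_StockPile is a stockpile that tracks how much of a single resource its inventory container holds.
; Initialization takes the resource class and display name from the container's whitelist, printing an error unless it has exactly one filter class.
; On inventory updates, the authority recalculates the stockpile quantity by summing every item's stack quantity.
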(event InventoryUpdatedOnupdate(BPC_InventoryContainer)
  (Networking|SwitchHasAuthority
    (:Authority
      (CallFunction|UpdateStockPileQuantity))))

(fn ConstructionScript
  (|CallParentFunction))

(fn UpdateStockPileQuantity
  (for _array_element (.OutItems (Class|InventoryContainer|GetInventoryData (Variables|Default|GetBPC_InventoryContainer)))
    (LocalVariables|SetLocal%20Stock%20Pile%20Incrament (+ (LocalVariables|GetLocal%20Stock%20Pile%20Incrament) (Utilities|Struct|BreakItemData _array_element))))
  (Variables|StockPileData|SetStock%20Pile%20Quantity (LocalVariables|GetLocal%20Stock%20Pile%20Incrament)))

(fn Initalize
  (bind _bpc_inventorycontainer (Variables|Default|GetBPC_InventoryContainer))
  (bind _filterclasses (Variables|/Script/SRPG.InventoryContainer|GetFilterClasses _bpc_inventorycontainer))
  (|CallParentFunction)
  (if (and (== (Utilities|Array|Length _filterclasses) 1) (Utilities|Enum|Equal(Enum) (Variables|/Script/SRPG.InventoryContainer|GetFilterType _bpc_inventorycontainer) "EIT_WhiteList"))
    (bind _output_get (Variables|Default|SetStock%20Pile%20Resrouce (Utilities|Array|Get(acopy) _filterclasses)))
    (Variables|Default|SetResource%20Display%20Nane (Utilities|Struct|BreakItemData (Utilities|GetClassDefaults _output_get)))
    (else
      (Development|PrintString (Utilities|String|ToString(Text) (Utilities|Text|FormatText "{Actor} stock pile is set up incorrrectly. " (Utilities|GetDisplayName self)))))))