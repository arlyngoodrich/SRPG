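; BP_ItemManager tracks world pickup items through check-in/check-out and persists them, including their inventories, across save and load.
; On pre-save, the authority flattens class, transform, item data and container contents into parallel arrays.
; Random unique pair IDs link items to their inventories and to one level of nested abstract inventories.
; On load, it destroys all pickups, respawns saved items and rebuilds both inventory levels from those IDs.
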(event EventActorPreSave
  (SavedData|SaveItemData))

(event EventActorLoaded
  (bind _outactors (Actor|GetAllActorsOfClass "/Game/SRPG/Blueprints/ItemSystem/BP_PickupBase.BP_PickupBase_C"))
  (for _array_element _outactors
    (Actor|DestroyActor _array_element))
  (SavedData|LoadItems))

(fn ConstructionScript)

(fn CheckItemin
  (params (New%20Item :type BP%20Pickup%20Base%20Object%20Reference))
  (Utilities|Array|AddUnique (Variables|ItemManagement|GetTracked%20Items) New%20Item))

(fn CheckItemOut
  (params (Item :type BP%20Pickup%20Base%20Object%20Reference%20%28by%20ref%29))
  (bind _returnvalue (Utilities|Array|RemoveItem (Variables|ItemManagement|GetTracked%20Items) Item))
  (if (not _returnvalue)
    (Development|PrintString (Utilities|String|Append "Item Manager failed to check out : " (Utilities|GetDisplayName Item)))))

(fn SaveItemData
  (Utilities|Array|Clear (Variables|SavedData|GetSaved%20Actor%20Classes))
  (Utilities|Array|Clear (Variables|SavedData|GetSaved%20Actor%20Locations))
  (Utilities|Array|Clear (Variables|SavedData|GetSaved%20Item%20Data))
  (Utilities|Array|Clear (Variables|SavedData|GetUnique%20Item%20ID))
  (Utilities|Array|Clear (Variables|SavedData|GetSaved%20Invetory%20Pair%20IDs))
  (Utilities|Array|Clear (Variables|SavedData|GetSaved%20Inventory%20Data))
  (Utilities|Array|Clear (Variables|SavedData|GetAdd%20Abstract%20Inventory))
  (Utilities|Array|Clear (Variables|SavedData|GetSaved%20Abstract%20Inventory%20Data))
  (Utilities|Array|Clear (Variables|SavedData|GetSaved%20Abstract%20Pair%20ID))
  (Utilities|Array|Clear (Variables|UniqueID|GetUnique%20ID%20List))
  (Networking|SwitchHasAuthority
    (:Authority
      (for _array_element (Variables|ItemManagement|GetTracked%20Items)
        (Utilities|Array|Add (Variables|SavedData|GetSaved%20Actor%20Classes) (Utilities|GetClass _array_element))
        (Utilities|Array|Add (Variables|SavedData|GetSaved%20Actor%20Locations) (Transformation|GetActorTransform _array_element))
        (Utilities|Array|Add (Variables|SavedData|GetSaved%20Item%20Data) (Variables|/Script/SRPG.ItemBase|GetItemData _array_element))
        (bind _output_get (LocalVariables|SetPair%20ID (UniqueID|CreateUniquePairID)))
        (Utilities|Array|Add (Variables|SavedData|GetUnique%20Item%20ID) _output_get)
        (Utilities|IsValid (Actor|GetComponentbyClass _array_element "/Game/SRPG/Blueprints/InventorySystem/BPC_InventoryContainer.BPC_InventoryContainer_C")
          (:Is%20Valid
            ;[1 1 1] Save inventories from pickup items
            (bind _outinventorydata (Class|InventoryContainer|GetInventoryforAbstract (Actor|GetComponentbyClass _array_element "/Game/SRPG/Blueprints/InventorySystem/BPC_InventoryContainer.BPC_InventoryContainer_C")))
            (for _array_element_2 _outinventorydata
              (Utilities|IsValid (Utilities|Struct|BreakItemData (.ItemData (Utilities|Struct|BreakInventoryItemData _array_element_2)))
                (:Is%20Valid
                  ;[1 1 1] Save Items with Abstract Inventories
                  (Utilities|Array|Add (Variables|SavedData|GetAdd%20Abstract%20Inventory) true)
                  (bind _outinventory (Class|AbstractInventoryContainer|GetInventory (Utilities|Struct|BreakItemData (.ItemData (Utilities|Struct|BreakInventoryItemData _array_element_2)))))
                  (LocalVariables|SetAbstract%20Pair%20ID (UniqueID|CreateUniquePairID))
                  (for _array_element_3 _outinventory
                    (Utilities|Array|Add (Variables|SavedData|GetSaved%20Abstract%20Inventory%20Data) _array_element_3)
                    (Utilities|Array|Add (Variables|SavedData|GetSaved%20Abstract%20Pair%20ID) (LocalVariables|GetAbstract%20Pair%20ID)))
                  (bind _structout (Utilities|Struct|SetmembersinItemData (.ItemData (Utilities|Struct|BreakInventoryItemData _array_element_2)) (LocalVariables|GetAbstract%20Pair%20ID)))
                  (Utilities|Array|Add (Variables|SavedData|GetSaved%20Inventory%20Data) (Utilities|Struct|MakeInventoryItemData _structout (.Position (Utilities|Struct|BreakInventoryItemData _array_element_2))))
                  (Utilities|Array|Add (Variables|SavedData|GetSaved%20Invetory%20Pair%20IDs) (LocalVariables|GetPair%20ID)))
                (:Is%20Not%20Valid
                  ;[1 1 1] Save Invetory Without adding Items with Abstract
                  (Utilities|Array|Add (Variables|SavedData|GetAdd%20Abstract%20Inventory) false)
                  (Utilities|Array|Add (Variables|SavedData|GetSaved%20Inventory%20Data) _array_element_2)
                  (Utilities|Array|Add (Variables|SavedData|GetSaved%20Invetory%20Pair%20IDs) (LocalVariables|GetPair%20ID)))))))))))

(fn LoadItems
  (for (_array_element _array_index) (Variables|SavedData|GetSaved%20Actor%20Classes)
    (bind _returnvalue (Game|SpawnActorfromClass _array_element (Utilities|Array|Get(acopy) (Variables|SavedData|GetSaved%20Actor%20Locations) _array_index) "Undefined" 0 (Utilities|GetClassDefaults _array_element) false (Utilities|Array|Get(acopy) (Variables|SavedData|GetSaved%20Item%20Data) _array_index) 0))
    (bind _output_get (LocalVariables|SetSpawned%20Actor _returnvalue))
    (Utilities|IsValid _output_get
      (:Is%20Valid
        (if (Utilities|Struct|BreakItemData (Utilities|Array|Get(acopy) (Variables|SavedData|GetSaved%20Item%20Data) _array_index))
          ;[1 1 1] Add Inventory back to pickup items
          (Utilities|Array|Clear (LocalVariables|GetTemp%20Inventory))
          (for (_array_element_2 _array_index_2) (Variables|SavedData|GetSaved%20Invetory%20Pair%20IDs)
            (if (== _array_element_2 (Utilities|Array|Get(acopy) (Variables|SavedData|GetUnique%20Item%20ID) _array_index))
              (if (Utilities|Array|Get(acopy) (Variables|SavedData|GetAdd%20Abstract%20Inventory) _array_index_2)
                ;;[1 1 1] Add abstract inventory items back
                (Utilities|Array|Clear (LocalVariables|GetTemp%20Abstract%20Inventory))
                (for (_array_element_3 _array_index_3) (Variables|SavedData|GetSaved%20Abstract%20Pair%20ID)
                  (if (== _array_element_3 (Utilities|Struct|BreakItemData (.ItemData (Utilities|Struct|BreakInventoryItemData (Utilities|Array|Get(acopy) (Variables|SavedData|GetSaved%20Inventory%20Data) _array_index_2)))))
                    (Utilities|Array|Add (LocalVariables|GetTemp%20Abstract%20Inventory) (Utilities|Array|Get(acopy) (Variables|SavedData|GetSaved%20Abstract%20Inventory%20Data) _array_index_3))))
                (bind _returnvalue_2 (Game|ConstructObjectfromClass "/Game/SRPG/Blueprints/InventorySystem/BP_AbstractInventoryContainer.BP_AbstractInventoryContainer_C" (LocalVariables|GetSpawned%20Actor)))
                (bind _output_get_2 (LocalVariables|SetSpawned%20Abstract%20Inventory _returnvalue_2))
                (Class|AbstractInventoryContainer|SetInventory _output_get_2 (LocalVariables|GetTemp%20Abstract%20Inventory))
                (bind _structout (Utilities|Struct|SetmembersinItemData (.ItemData (Utilities|Struct|BreakInventoryItemData (Utilities|Array|Get(acopy) (Variables|SavedData|GetSaved%20Inventory%20Data) _array_index_2))) (LocalVariables|GetSpawned%20Abstract%20Inventory)))
                (Utilities|Array|Add (LocalVariables|GetTemp%20Inventory) (Utilities|Struct|MakeInventoryItemData _structout (.Position (Utilities|Struct|BreakInventoryItemData (Utilities|Array|Get(acopy) (Variables|SavedData|GetSaved%20Inventory%20Data) _array_index_2)))))
                (else
                  (Utilities|Array|Add (LocalVariables|GetTemp%20Inventory) (Utilities|Array|Get(acopy) (Variables|SavedData|GetSaved%20Inventory%20Data) _array_index_2))))))
          (Utilities|IsValid (Actor|GetComponentbyClass (LocalVariables|GetSpawned%20Actor) "/Game/SRPG/Blueprints/InventorySystem/BPC_InventoryContainer.BPC_InventoryContainer_C")
            (:Is%20Valid
              (Class|InventoryContainer|SetInventoryfromAbstract (Actor|GetComponentbyClass (LocalVariables|GetSpawned%20Actor) "/Game/SRPG/Blueprints/InventorySystem/BPC_InventoryContainer.BPC_InventoryContainer_C") (LocalVariables|GetTemp%20Inventory)))))))))

(fn CreateUniquePairID
  (LocalVariables|SetNew%20ID (Math|Random|RandomInteger 10000000) :!label _label)
  (if (not (Utilities|Array|ContainsItem (Variables|UniqueID|GetUnique%20ID%20List) (LocalVariables|GetNew%20ID)))
    (return (LocalVariables|GetNew%20ID))
    (else
      (goto _label))))

(fn ComponentstoSave
  (return 0))