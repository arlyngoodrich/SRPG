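; Base stockpile buildable that holds one whitelisted resource type and makes it known to nearby players' build managers.
; Once fully built, its sphere checks characters' build managers in and out on overlap, also scanning existing overlaps on build completion or load.
; Inventory updates notify tracked managers on server and clients, then recompute total quantity and a fill percentage based on occupied item entries versus grid capacity.
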(event InventoryUpdatedOnupdate(BPC_InventoryContainer)
  (CallFunction|OnInventoryUpdate)
  (Development|PrintString "Stockpile Inventory Updated"))

(event OnComponentBeginOverlap(Sphere)
  (params (OverlappedComponent :type Primitive%20Component%20Object%20Reference) (OtherActor :type Actor%20Object%20Reference) (OtherComp :type Primitive%20Component%20Object%20Reference) (OtherBodyIndex :type Integer) (bFromSweep :type Boolean) (SweepResult :type Hit%20Result%20Structure%20%28by%20ref%29))
  (if (Utilities|Enum|Equal(Enum) (Variables|Default|GetBuildStatus) "BPSE_FullyBuilt")
    (bind _asbp_srpgcharacter (Utilities|Casting|CastToBP_SRPGCharacter OtherActor))
    (Default|CheckinStockPile (Variables|/Game/SRPG/Blueprints/CharacterAssets/BP_SRPGCharacter.BP_SRPGCharacter_C|GetBPC_PlayerBuildManager _asbp_srpgcharacter) self)
    (Utilities|Array|Add (Variables|Default|GetTracking%20Build%20Managers) (Variables|/Game/SRPG/Blueprints/CharacterAssets/BP_SRPGCharacter.BP_SRPGCharacter_C|GetBPC_PlayerBuildManager _asbp_srpgcharacter))))

(event OnComponentEndOverlap(Sphere)
  (params (OverlappedComponent :type Primitive%20Component%20Object%20Reference) (OtherActor :type Actor%20Object%20Reference) (OtherComp :type Primitive%20Component%20Object%20Reference) (OtherBodyIndex :type Integer))
  (if (Utilities|Enum|Equal(Enum) (Variables|Default|GetBuildStatus) "BPSE_FullyBuilt")
    (bind _asbp_srpgcharacter (Utilities|Casting|CastToBP_SRPGCharacter OtherActor))
    (Default|CheckOutStockPile (Variables|/Game/SRPG/Blueprints/CharacterAssets/BP_SRPGCharacter.BP_SRPGCharacter_C|GetBPC_PlayerBuildManager _asbp_srpgcharacter) self)
    (Utilities|Array|RemoveItem (Variables|Default|GetTracking%20Build%20Managers) (Variables|/Game/SRPG/Blueprints/CharacterAssets/BP_SRPGCharacter.BP_SRPGCharacter_C|GetBPC_PlayerBuildManager _asbp_srpgcharacter))))

(event Custom|On%20Inventory%20Update
  (Networking|SwitchHasAuthority
    (:Authority
      (for _array_element (Variables|Default|GetTracking%20Build%20Managers)
        (Default|StockPileUpdate _array_element))
      (CallFunction|UpdateStockPileQuantity)
      (CallFunction|UpdateStockPilePercentage))
    (:Remote
      (for _array_element_2 (Variables|Default|GetTracking%20Build%20Managers)
        (Default|StockPileUpdate _array_element_2))
      (CallFunction|UpdateStockPileQuantity)
      (CallFunction|UpdateStockPilePercentage))))

(event EventOnBuildStatusChangetoBuilt
  (|CallParentFunction)
  (for _array_element (Collision|GetOverlappingActors (Variables|Default|GetSphere) "/Game/SRPG/Blueprints/CharacterAssets/BP_SRPGCharacter.BP_SRPGCharacter_C" :!class /Script/Engine.PrimitiveComponent)
    (bind _asbp_srpgcharacter (Utilities|Casting|CastToBP_SRPGCharacter _array_element))
    (Default|CheckinStockPile (Variables|/Game/SRPG/Blueprints/CharacterAssets/BP_SRPGCharacter.BP_SRPGCharacter_C|GetBPC_PlayerBuildManager _asbp_srpgcharacter) self)
    (Utilities|Array|Add (Variables|Default|GetTracking%20Build%20Managers) (Variables|/Game/SRPG/Blueprints/CharacterAssets/BP_SRPGCharacter.BP_SRPGCharacter_C|GetBPC_PlayerBuildManager _asbp_srpgcharacter))))

(event EventActorLoaded
  (|CallParentFunction)
  (Networking|SwitchHasAuthority
    (:Authority
      (for _array_element (Collision|GetOverlappingActors (Variables|Default|GetSphere) "/Game/SRPG/Blueprints/CharacterAssets/BP_SRPGCharacter.BP_SRPGCharacter_C" :!class /Script/Engine.PrimitiveComponent)
        (bind _asbp_srpgcharacter (Utilities|Casting|CastToBP_SRPGCharacter _array_element))
        (Default|CheckinStockPile (Variables|/Game/SRPG/Blueprints/CharacterAssets/BP_SRPGCharacter.BP_SRPGCharacter_C|GetBPC_PlayerBuildManager _asbp_srpgcharacter) self)
        (Utilities|Array|Add (Variables|Default|GetTracking%20Build%20Managers) (Variables|/Game/SRPG/Blueprints/CharacterAssets/BP_SRPGCharacter.BP_SRPGCharacter_C|GetBPC_PlayerBuildManager _asbp_srpgcharacter))))))

(event EventBeginPlay
  (|CallParentFunction)
  (Development|PrintString (Utilities|String|EnumtoString (Networking|GetLocalRole))))

(fn ConstructionScript
  (|CallParentFunction)
  (Variables|Default|SetRange (Variables|/Script/Engine.SphereComponent|GetSphereRadius (Variables|Default|GetSphere))))

(fn UpdateStockPileQuantity
  (for _array_element (.OutItems (Class|InventoryContainer|GetInventoryData (Variables|Default|GetBPC_InventoryContainer)))
    (LocalVariables|SetLocal%20Stock%20Pile%20Incrament (+ (LocalVariables|GetLocal%20Stock%20Pile%20Incrament) (Utilities|Struct|BreakItemData _array_element))))
  (Variables|StockPileData|SetStock%20Pile%20Quantity (LocalVariables|GetLocal%20Stock%20Pile%20Incrament)))

(fn Initalize
  (bind _bpc_inventorycontainer (Variables|Default|GetBPC_InventoryContainer))
  (bind _filterclasses (Variables|/Script/SRPG.InventoryContainer|GetFilterClasses _bpc_inventorycontainer))
  (|CallParentFunction)
  (if (and (== (Utilities|Array|Length _filterclasses) 1) (Utilities|Enum|Equal(Enum) (Variables|/Script/SRPG.InventoryContainer|GetFilterType _bpc_inventorycontainer) "EIT_WhiteList"))
    (bind _output_get (Variables|Default|SetStock%20Pile%20Resrouce (Utilities|Array|Get(acopy) _filterclasses)))
    (Variables|Default|SetResource%20Display%20Nane (Utilities|Struct|BreakItemData (Utilities|GetClassDefaults _output_get)))
    (else
      (Development|PrintString (Utilities|String|ToString(Text) (Utilities|Text|FormatText "{Actor} stock pile is set up incorrrectly. " (Utilities|GetDisplayName self)))))))

(fn UpdateStockPilePercentage
  (bind _stock_pile_resrouce (Variables|Default|GetStock%20Pile%20Resrouce))
  (bind _bpc_inventorycontainer (Variables|Default|GetBPC_InventoryContainer))
  (bind _itemdata (Utilities|GetClassDefaults _stock_pile_resrouce))
  (bind (_sizex _sizey) (Utilities|Struct|BreakItemData _itemdata))
  (Variables|StockPileData|SetStock%20Pile%20Percentage (/ (Math|Conversions|ToFloat(Integer) (Utilities|Array|Length (.OutItems (Class|InventoryContainer|GetInventoryData (Variables|Default|GetBPC_InventoryContainer))))) (Math|Conversions|ToFloat(Integer) (/ (* (Variables|/Script/SRPG.InventoryContainer|GetInventorySizeX _bpc_inventorycontainer) (Variables|/Script/SRPG.InventoryContainer|GetInventorySizeY _bpc_inventorycontainer)) (* _sizex _sizey)))))
  (return))