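; BP_TestFoliageTree is a test tree that turns into wood pickups when fully depleted by something other than an interaction.
; It extends the parent's depletion event, then swaps its static mesh to a low-poly trunk when FromInteraction is false.
; After a short delay it deactivates the actor and spawns a BP_TestWoodPickup at each scene component tagged "Log Spawner".
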(event EventOnFullyDepleated
  (params (From%20Interaction :type Boolean))
  (|CallParentFunction From%20Interaction)
  (if (not From%20Interaction)
    (Components|StaticMesh|SetStaticMesh (Variables|Default|GetStaticMesh) "/Game/TestContent/Meshes/SM_Trunk_LP.SM_Trunk_LP")
    (Utilities|FlowControl|Delay 2.0)
    (CallFunction|DeactivateActor)
    (for _array_element (Actor|GetComponentsbyTag "/Script/Engine.SceneComponent" "Log Spawner")
      (Game|SpawnActorfromClass :Class "/Game/TestContent/Blueprints/BP_TestWoodPickup.BP_TestWoodPickup_C" :SpawnTransform (Transformation|GetWorldTransform _array_element) :CollisionHandlingOverride "Undefined" :Instigator 0))))

(fn ConstructionScript
  (|CallParentFunction))