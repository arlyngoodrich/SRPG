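; BP_FoliageTestTree is a test foliage tree that turns into wood pickups when depleted.
; On the depletion event, the authority swaps the mesh to a low-poly trunk and waits briefly.
; It then gathers transforms from scene components tagged "Spawner", clears the mesh and spawns a BP_TestWoodPickup at each transform.
; A very short lifespan then removes the tree actor.
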(event EventBPEonFoliageDepleted
  (Networking|SwitchHasAuthority
    (:Authority
      (Components|StaticMesh|SetStaticMesh (Variables|Default|GetFoliageMeshComponent) "/Game/TestContent/Meshes/SM_Trunk_LP.SM_Trunk_LP")
      (Utilities|FlowControl|Delay 2.0)
      (for _array_element (Actor|GetComponentsbyTag "/Script/Engine.SceneComponent" "Spawner")
        (Utilities|Array|Add (Variables|Default|GetSpawn%20Transforms) (Transformation|GetWorldTransform _array_element)))
      (Components|StaticMesh|SetStaticMesh (Variables|Default|GetFoliageMeshComponent) 0)
      (for _array_element_2 (Variables|Default|GetSpawn%20Transforms)
        (Game|SpawnActorfromClass "/Game/TestContent/Blueprints/BP_TestWoodPickup.BP_TestWoodPickup_C" _array_element_2 "Undefined" 0 0))
      (Actor|SetLifeSpan 0.01))))

(fn ConstructionScript)